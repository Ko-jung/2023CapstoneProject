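; BP_ClientCharacter is a character Blueprint that tracks whether a player controls it and how fast it moves.
; Possession sets IsPossessed only when the controller's class is exactly PlayerController, and unpossession clears it, each printing a debug message.
; Tick calls the parent, then stores velocity length in Speed while possessed.
; The IA_Move event is empty, and the camera-relative movement and mapping-context nodes are disconnected, so never run.
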(event `self.ReceivePossessed`
  (params (NewController :type "Controller Object Reference"))
  (if (== (`GameplayStatics.GetObjectClass` NewController) "/Script/Engine.PlayerController")
    (set `self.IsPossessed?` true)
    (`KismetSystemLibrary.PrintString` "On Possesed")))

(event `self.ReceiveUnpossessed`
  (params (OldController :type "Controller Object Reference"))
  (set `self.IsPossessed?` false)
  (`KismetSystemLibrary.PrintString` "Un Possessed"))

(event `self.ReceiveBeginPlay`
  (`parent.ReceiveBeginPlay`))

(event `self.ReceiveTick`
  (params (DeltaSeconds :type "Float (single-precision)"))
  (`parent.ReceiveTick` DeltaSeconds)
  (if (`self.IsPossessed?`)
    (set `self.Speed` (`KismetMathLibrary.VSize` (`MovementComponent.Velocity` (`self.CharacterMovement`))))))

(event `EnhancedInput|/Game/ThirdPerson/Input/Actions/IA_Move`
  (params (ActionValue :type "Vector2D Structure") (ElapsedSeconds :type "Float (double-precision)") (TriggeredSeconds :type "Float (double-precision)") (InputAction :type "InputAction Object Reference" :default "/Game/ThirdPerson/Input/Actions/IA_Move.IA_Move")))

(fn `UserConstructionScript`)