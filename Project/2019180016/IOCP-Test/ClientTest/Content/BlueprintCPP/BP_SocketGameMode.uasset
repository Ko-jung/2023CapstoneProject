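; BP_SocketGameMode is a game mode that syncs third-person characters by serial number, apparently for socket-based multiplayer.
; Each tick it applies ClientTransform entries to every player except the local SerialNum, then writes that player's own transform back.
; Events collect the character list, possess a player by serial, update remote positions, and recolor spawned players blue.
; The InitClientInfo call that fills the transform array is unwired here, noted as controlled on the level.
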(event `self.ReceiveTick`
  (params (DeltaSeconds :type "Float (single-precision)"))
  (`parent.ReceiveTick` DeltaSeconds)
  (`self.SetClientInfo`)
  (`self.SetOwnTransform`))

(event `self.ReceiveBeginPlay`
  (`parent.ReceiveBeginPlay`))

(event `self.SpawnPlayer`
  (params (serial :type Integer))
  (`KismetSystemLibrary.PrintString` (`KismetStringLibrary.Concat_StrStr` (`KismetStringLibrary.Conv_IntToString` serial) "Player Spawn"))
  (`PrimitiveComponent.SetMaterial` (`Character.Mesh` (`|GetArrayItem` (`self.Players`) serial)) 0 "/Game/LevelPrototyping/Materials/MI_Solid_Blue.MI_Solid_Blue"))

(event `self.TestPrintHelloUseNative`
  (`KismetSystemLibrary.PrintString` "Hello" true false (struct :`R` 1.0 :`G` 0.048928 :`A` 1.0) 5.0))

(event `self.BPGetAllActorsOfThirdPerson`
  (bind _outactors (`GameplayStatics.GetAllActorsOfClass` "/Game/BlueprintCPP/BP_ThirdPersonCharacterChild.BP_ThirdPersonCharacterChild_C"))
  (set `self.Players` _outactors))

(event `self.BPSetPlayerPosition`
  (params (serial :type Integer) (location :type "Vector Structure") (rotate :type "Rotator Structure"))
  (`KismetArrayLibrary.Array_Set` (`self.ClientTransform`) serial (`KismetMathLibrary.MakeTransform` location rotate)))

(event `self.BPPossess`
  (params (serial :type Integer))
  (`Controller.Possess` (`GameplayStatics.GetPlayerController` 0) (`|GetArrayItem` (`self.Players`) serial))
  (`KismetSystemLibrary.PrintString` "Possess"))

(fn `InitClientInfo`
  (for _array_element (`self.Players`)
    (`KismetArrayLibrary.Array_Add` (`self.ClientTransform`) (`KismetMathLibrary.MakeTransform` (`self.K2_GetActorLocation` _array_element) (`self.K2_GetActorRotation` _array_element)))))

(fn `SetClientInfo`
  (for (_array_element _array_index) (`self.Players`)
    (if (not (== (`self.SerialNum`) _array_index))
      (`self.K2_SetActorTransform` _array_element (`|GetArrayItem` (`self.ClientTransform`) _array_index) false false))))

(fn `SetOwnTransform`
  (bind _serialnum (`self.SerialNum`))
  (bind _output (`|GetArrayItem` (`self.Players`) _serialnum))
  (`KismetArrayLibrary.Array_Set` (`self.ClientTransform`) _serialnum (`KismetMathLibrary.MakeTransform` (`self.K2_GetActorLocation` _output) (`self.K2_GetActorRotation` _output) (`self.GetActorScale3D` _output))))

(fn `SpawnCharacter`)

(fn `UserConstructionScript`)