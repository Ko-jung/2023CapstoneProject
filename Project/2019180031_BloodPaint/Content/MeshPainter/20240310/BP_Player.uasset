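; BP_Player is the player Blueprint that paints study mannequins by shooting at them.
; While the Shoot axis is positive, it runs a debug-drawn Visibility line trace every frame from the actor's location along the control rotation.
; A hit on a MyStudyMannequin passes the hit location and a fixed brush radius to that mannequin's CaptureActor, whose PaintActor call handles the painting.
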(event `self.ReceiveBeginPlay`)

(event `InputAxis|Shoot`
  (params (AxisValue :type "Float (single-precision)"))
  (if (> AxisValue 0.0)
    (`self.Shoot`)))

(fn `Shoot`
  (bind _returnvalue (`self.K2_GetActorLocation`))
  (bind (_outhit _returnvalue_2) (`KismetSystemLibrary.LineTraceSingle` :`Start` _returnvalue :`End` (+ _returnvalue (* (`KismetMathLibrary.GetForwardVector` (`self.GetControlRotation`)) (`self.ShootDistance`))) :`TraceChannel` "TraceTypeQuery1" :`DrawDebugType` "ForDuration" :`DrawTime` 1.0))
  (if _returnvalue_2
    (bind (_bblockinghit _binitialoverlap _time _distance _location _impactpoint _normal _impactnormal _physmat _hitactor) (`GameplayStatics.BreakHitResult` _outhit))
    (bind _asmy_study_mannequin (cast `/Game/MeshPainter/20240310/MyStudyMannequin` _hitactor))
    (`/Game/MeshPainter/20240310/MyStudyCapture.PaintActor` (`/Game/MeshPainter/20240310/MyStudyMannequin.CaptureActor` _asmy_study_mannequin) _asmy_study_mannequin _location 10.0)))

(fn `UserConstructionScript`)