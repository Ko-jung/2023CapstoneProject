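; Mesh-painting capture actor that renders hit marks on BPCloth into a render target through an unwrap material, apparently work in progress.
; TestCollision stores hit locations and radii; a looping 0.1-second tick shrinks the radii and calls SetTexture.
; SetTexture encodes hits as colors in a one-pixel-high data texture, then moves and captures the cloth with the unwrap material.
; Material restoration and hit-count update are disconnected.
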(event `self.ReceiveBeginPlay`
  (bind _unwraplocation (`self.UnwrapLocation`))
  (bind _crt_hitlocations (`self.CRT_HitLocations`))
  (bind _unwrapmaterial (`self.UnwrapMaterial`))
  ;[1 1 1] Unwrap Material 설정
  (bind _returnvalue (`KismetMaterialLibrary.CreateDynamicMaterialInstance` "/Game/MeshPainter/Materials/M_MultiParamUnWrap.M_MultiParamUnWrap"))
  (set `self.UnwrapMaterial` _returnvalue)
  (`MaterialInstanceDynamic.SetScalarParameterValue` (`self.UnwrapMaterial`) "CaptureSize" (`SceneCaptureComponent2D.OrthoWidth` (`self.SceneCaptureComponent2D`)))
  (`MaterialInstanceDynamic.SetVectorParameterValue` (`self.UnwrapMaterial`) "UnwrapLocation" (`KismetMathLibrary.Conv_VectorToLinearColor` _unwraplocation))
  (`self.K2_SetActorLocation` _unwraplocation) ; 위치 Unwrap Location으로 이동
  ;[1 1 1] 렌더타겟 생성
  (bind _returnvalue_2 (`KismetRenderingLibrary.CreateRenderTarget2D` 1000 1))
  (set `self.CRT_HitLocations` _returnvalue_2)
  ;[1 1 1] 파라미터 설정
  (`MaterialInstanceDynamic.SetTextureParameterValue` _unwrapmaterial "Tex" _crt_hitlocations)
  (`MaterialInstanceDynamic.SetScalarParameterValue` _unwrapmaterial "XSize" (`KismetMathLibrary.Conv_IntToDouble` (`TextureRenderTarget2D.SizeX` _crt_hitlocations)))
  (`MaterialInstanceDynamic.SetScalarParameterValue` _unwrapmaterial "Range" (`self.Valid_Range`))
  ;[1 1 1] 옷 최종 CRT 생성 및 SceneCaptureComponent 연결
  (bind _returnvalue_3 (`KismetRenderingLibrary.CreateRenderTarget2D` 1024 1024))
  (set `SceneCaptureComponent2D.TextureTarget` _returnvalue_3 (`self.SceneCaptureComponent2D`))
  ;[1 1 1] 옷 Dynamic Material 생성 및 렌더타겟 파라미터 생성
  (for _array_element (`/Game/MeshPainter/Blueprints/BP_Cloth.StaticMeshComps` (`self.BP_Cloth`))
    (bind _returnvalue_4 (`PrimitiveComponent.CreateDynamicMaterialInstance` _array_element 0 (`self.Cloths_Source_Mat`) "None"))
    (`MaterialInstanceDynamic.SetTextureParameterValue` _returnvalue_4 "None" (`SceneCaptureComponent2D.TextureTarget` (`self.SceneCaptureComponent2D`))))
  (`self.BrushTickEvent`)
  (bind _outactors (`GameplayStatics.GetAllActorsOfClass` "/Game/MeshPainter/Blueprints/BP_Plane.BP_Plane_C"))
  (`|ExecutionSequence`
    (:`then_0`
      (bind _returnvalue_5 (`KismetMaterialLibrary.CreateDynamicMaterialInstance` "/Game/MeshPainter/Materials/m_test_Inst.m_test_Inst"))
      (`MaterialInstanceDynamic.SetTextureParameterValue` _returnvalue_5 "RenderTarget" (`SceneCaptureComponent2D.TextureTarget` (`self.SceneCaptureComponent2D`)))
      (`PrimitiveComponent.SetMaterial` (`/Game/MeshPainter/Blueprints/BP_Plane.Plane` (`|GetArrayItem` _outactors)) 0 _returnvalue_5))
    (:`then_1`
      (`PrimitiveComponent.SetMaterial` (`/Game/MeshPainter/Blueprints/BP_Plane.Plane` (`|GetArrayItem` _outactors 1)) 0 (`self.UnwrapMaterial`)))
    (:`then_3`
      (`SceneCaptureComponent2D.CaptureScene` (`self.SceneCaptureComponent2D`)))))

(event `/Game/MeshPainter/Interface/BPI_Paintable.Paint`
  (params (HitLocation :type "Vector Structure") (BrushRadius :type "Float (double-precision)") (HitActor :type "Actor Object Reference")))

(event `BrushTickEvent`
  (bind _hitradius (`self.HitRadius`))
  (`KismetSystemLibrary.Delay` 0.1)
  (`self.BrushTickEvent`)
  (if (!= (`KismetArrayLibrary.Array_Length` (`self.HitRadius`)) 0)
    (for (_array_element _array_index) _hitradius
      (`KismetArrayLibrary.Array_Set` _hitradius _array_index (- _array_element 0.1)))
    (`self.SetTexture`)))

(event `TestCollision`
  (params (HitLocation :type "Vector Structure (by ref)") (BrushRadius :type "Float (double-precision) (by ref)"))
  (bind _hitlocations (`self.HitLocations`))
  ;[1 1 1] 충돌 추가 / 페인팅 BPI
  (if (< (`KismetArrayLibrary.Array_Length` _hitlocations) (`self.HitCountSize`))
    (`KismetArrayLibrary.Array_Add` _hitlocations HitLocation)
    (`KismetArrayLibrary.Array_Add` (`self.HitRadius`) BrushRadius)))

(event `SetTexture`
  (bind _crt_hitlocations (`self.CRT_HitLocations`))
  (bind _valid_range (`self.Valid_Range`))
  ;[1 1 1] 액터 이동시키기
  (`KismetSystemLibrary.PrintString` "Hello")
  (set `self.ActorInitialLocation` (`self.K2_GetActorLocation` (`self.BP_Cloth`)))
  (`self.K2_SetActorLocation` (`self.BP_Cloth`) (+ (`self.UnwrapLocation`) (0.0 0.0 0.0)) false false)
  ;[1 1 1] 렌더타겟 초기화
  (`MaterialInstanceDynamic.SetScalarParameterValue` (`self.UnwrapMaterial`) "HitCounts" 0.0)
  (`KismetRenderingLibrary.ClearRenderTarget2D` _crt_hitlocations)
  (bind (_canvas _size _context) (`KismetRenderingLibrary.BeginDrawCanvasToRenderTarget` _crt_hitlocations))
  (`|ExecutionSequence`
    (:`then_0`
      ;[1 1 1] 1. 캔버스 렌더 타겟에 데이터 담기
      (for (_array_element _array_index) (`self.HitLocations`)
        (bind (_returnvalue_x _returnvalue_y _returnvalue_z) (`KismetMathLibrary.BreakVector` (/ (+ (+ (- _array_element (`self.ActorInitialLocation`)) (0.0 0.0 0.0) (`self.UnwrapLocation`)) _valid_range) (* _valid_range 2.0))))
        (`Canvas.K2_DrawTexture` _canvas null (`KismetMathLibrary.MakeVector2D` (`KismetMathLibrary.Conv_IntToDouble` (- (* _array_index 4) 2))) (4.0 1.0) (0.0 0.0) (1.0 1.0) (`KismetMathLibrary.MakeColor` _returnvalue_x _returnvalue_y _returnvalue_z) "BLEND_Translucent" 0.0 (0.5 0.5)))
      (`KismetRenderingLibrary.EndDrawCanvasToRenderTarget` _context))
    (:`then_1`
      ;[1 1 1] Comment
      (for _array_element_2 (`/Game/MeshPainter/Blueprints/BP_Cloth.StaticMeshComps` (`self.BP_Cloth`))
        (set `self.OriginalMaterial` (`PrimitiveComponent.GetMaterial` _array_element_2 0))
        (`PrimitiveComponent.SetMaterial` _array_element_2 0 (`self.UnwrapMaterial`)))
      (`SceneCaptureComponent2D.CaptureScene` (`self.SceneCaptureComponent2D`)))))

(fn `UserConstructionScript`)