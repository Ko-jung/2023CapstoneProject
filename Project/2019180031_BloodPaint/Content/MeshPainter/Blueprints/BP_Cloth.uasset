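; BP_Cloth is a mesh-painter clothing actor with inside shirt and outside jacket meshes, each registered in StaticMeshComps at BeginPlay.
; On BeginPlay it spawns a BP_CaptureForNewMat helper at a random, potentially distant XY location, handing it itself and M_ClothTest as source material.
; It keeps that helper as ChildCaptureActor.
; An older, unconnected chain spawning CaptureForCloth never runs, and the construction script is empty.
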(event `self.ReceiveBeginPlay`
  (bind _staticmeshcomps (`self.StaticMeshComps`))
  (bind _returnvalue (`|SpawnActorFromClass` "/Game/MeshPainter/Blueprints/BP_CaptureForNewMat.BP_CaptureForNewMat_C" (`KismetMathLibrary.MakeTransform` (`KismetMathLibrary.MakeVector` (* (`KismetMathLibrary.RandomFloatInRange` -1.0 1.0) 100000.0) (* (`KismetMathLibrary.RandomFloatInRange` -1.0 1.0) 100000.0))) "Undefined" "MultiplyWithRoot" null (0.0 0.0 0.0) self "/Game/MeshPainter/staticmesh/M_ClothTest.M_ClothTest" null))
  (`KismetArrayLibrary.Array_Add` _staticmeshcomps (`self.inside_shirt`))
  (`KismetArrayLibrary.Array_Add` _staticmeshcomps (`self.outside_jacket`))
  (set `self.childCaptureActor` _returnvalue))

(fn `UserConstructionScript`)