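; Player Blueprint that paints on meshes in the world by shooting line traces along the control rotation.
; BeginPlay caches the first MyStudyCapture actor after a short delay, and the Shoot axis fires a trace whenever its value is positive.
; Each hit sends the location and brush radius to every CaptureForCloth actor, then asks the cached capture actor to paint the hit actor.
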(event `self.ReceiveBeginPlay`
  (`KismetSystemLibrary.Delay` 0.1)
  (bind _outactors (`GameplayStatics.GetAllActorsOfClass` "/Game/MeshPainter/Blueprints/MyStudyCapture.MyStudyCapture_C"))
  (set `self.CaptureActor` (`|GetArrayItem` _outactors)))

(event `InputAxis|Shoot`
  (params (AxisValue :type "Float (single-precision)"))
  (if (> AxisValue 0.0)
    (`self.Shoot`)))

(fn `Shoot`
  (bind _returnvalue (`self.K2_GetActorLocation`))
  (bind _captureactor (`self.CaptureActor`))
  (bind (_outhit _returnvalue_2) (`KismetSystemLibrary.LineTraceSingle` _returnvalue (+ _returnvalue (* (`KismetMathLibrary.GetForwardVector` (`self.GetControlRotation`)) (`self.ShootDistance`))) "TraceTypeQuery1"))
  (if _returnvalue_2
    (bind _outactors (`GameplayStatics.GetAllActorsOfClass` "/Game/MeshPainter/Blueprints/CaptureForCloth.CaptureForCloth_C"))
    (for _array_element _outactors
      (bind (_bblockinghit _binitialoverlap _time _distance _location _impactpoint _normal _impactnormal _physmat _hitactor) (`GameplayStatics.BreakHitResult` _outhit))
      (message `/Game/MeshPainter/Interface/BPI_Paintable.Paint` _array_element _location 10.0))
    (`/Engine/EditorBlueprintResources/StandardMacros.IsValid` _captureactor
      (:`Is Valid`
        (`/Game/MeshPainter/Blueprints/MyStudyCapture.PaintActor` _captureactor _hitactor _location 10.0)))))

(fn `UserConstructionScript`)