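; Scene-capture actor that paints brush hits on BPCloth's shirt and jacket into a shared runtime render target.
; BeginPlay sets up the unwrap material, moves the actor to UnwrapLocation and feeds the target to both garments and a debug plane.
; Each paint moves the cloth there, captures each garment with the unwrap material, offset hit location and brush radius, then restores materials and position.
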(event `self.ReceiveBeginPlay`
  (bind _bp_cloth (`self.BP_Cloth`))
  (bind _unwraplocation (`self.UnwrapLocation`))
  ;[1 1 1] Unwrap Material 설정
  (bind _returnvalue (`KismetMaterialLibrary.CreateDynamicMaterialInstance` "/Game/MeshPainter/Materials/M_UnwrapForCloth.M_UnwrapForCloth"))
  (set `self.UnwrapMaterial` _returnvalue)
  (`MaterialInstanceDynamic.SetScalarParameterValue` (`self.UnwrapMaterial`) "CaptureSize" (`SceneCaptureComponent2D.OrthoWidth` (`self.SceneCapture`)))
  (`MaterialInstanceDynamic.SetVectorParameterValue` (`self.UnwrapMaterial`) "UnwrapLocation" (`KismetMathLibrary.Conv_VectorToLinearColor` _unwraplocation))
  (`self.K2_SetActorLocation` _unwraplocation) ; 위치 Unwrap Location으로 이동
  ;[1 1 1] 렌더타겟 생성
  (bind _returnvalue_2 (`KismetRenderingLibrary.CreateRenderTarget2D` 1024 1024))
  (set `SceneCaptureComponent2D.TextureTarget` _returnvalue_2 (`self.SceneCapture`))
  ;[1 1 1] 디버깅용 생성
  (bind _returnvalue_3 (`KismetMaterialLibrary.CreateDynamicMaterialInstance` "/Game/MeshPainter/Materials/m_test_Inst.m_test_Inst"))
  (`MaterialInstanceDynamic.SetTextureParameterValue` _returnvalue_3 "RenderTarget" (`SceneCaptureComponent2D.TextureTarget` (`self.SceneCapture`)))
  (bind _returnvalue_4 (`GameplayStatics.GetActorOfClass` "/Game/MeshPainter/Blueprints/BP_Plane.BP_Plane_C"))
  (`PrimitiveComponent.SetMaterial` (`/Game/MeshPainter/Blueprints/BP_Plane.Plane` _returnvalue_4) 0 _returnvalue_3)
  (bind _returnvalue_5 (`PrimitiveComponent.CreateDynamicMaterialInstance` (`/Game/MeshPainter/Blueprints/BP_Cloth.outside_jacket` _bp_cloth) 0 "/Game/MeshPainter/staticmesh/M_ClothTest.M_ClothTest" "None"))
  (`MaterialInstanceDynamic.SetTextureParameterValue` _returnvalue_5 "RenderTarget" (`SceneCaptureComponent2D.TextureTarget` (`self.SceneCapture`)))
  (bind _returnvalue_6 (`PrimitiveComponent.CreateDynamicMaterialInstance` (`/Game/MeshPainter/Blueprints/BP_Cloth.inside_shirt` _bp_cloth) 0 "/Game/MeshPainter/staticmesh/M_ClothTest.M_ClothTest" "None"))
  (`MaterialInstanceDynamic.SetTextureParameterValue` _returnvalue_6 "RenderTarget" (`SceneCaptureComponent2D.TextureTarget` (`self.SceneCapture`))))

(event `TestTestTest`
  (params (`Hit Location` :type "Vector Structure") (BrushRadius :type "Float (double-precision)"))
  (set `self.Hit Location` `Hit Location` :!label _label)
  (set `self.BrushRadius` BrushRadius)
  (set `self.ActorInitialLocation` (`self.K2_GetActorLocation` (`self.BP_Cloth`)))
  (`self.K2_SetActorLocation` (`self.BP_Cloth`) (+ (`self.UnwrapLocation`) (0.0 0.0 0.0)) false false)
  (`|ExecutionSequence`
    (:`then_0`
      (`|ExecutionSequence`
        (:`then_0`
          (set `self.OriginalMaterial` (`PrimitiveComponent.GetMaterial` (`/Game/MeshPainter/Blueprints/BP_Cloth.inside_shirt` (`self.BP_Cloth`)) 0))
          (`PrimitiveComponent.SetMaterial` (`/Game/MeshPainter/Blueprints/BP_Cloth.inside_shirt` (`self.BP_Cloth`)) 0 (`self.UnwrapMaterial`)))
        (:`then_1`
          (`MaterialInstanceDynamic.SetVectorParameterValue` (`self.UnwrapMaterial`) "HitLocation" (`KismetMathLibrary.Conv_VectorToLinearColor` (+ (- (`self.Hit Location`) (`self.ActorInitialLocation`)) (0.0 0.0 0.0) (`self.UnwrapLocation`))))
          (`MaterialInstanceDynamic.SetScalarParameterValue` (`self.UnwrapMaterial`) "BrushRadius" (`self.BrushRadius`)))
        (:`then_2`
          (`SceneCaptureComponent2D.CaptureScene` (`self.SceneCapture`))
          (`PrimitiveComponent.SetMaterial` (`/Game/MeshPainter/Blueprints/BP_Cloth.inside_shirt` (`self.BP_Cloth`)) 0 (`self.OriginalMaterial`)))))
    (:`then_1`
      (set `self.OriginalMaterial` (`PrimitiveComponent.GetMaterial` (`/Game/MeshPainter/Blueprints/BP_Cloth.outside_jacket` (`self.BP_Cloth`)) 0))
      (`PrimitiveComponent.SetMaterial` (`/Game/MeshPainter/Blueprints/BP_Cloth.outside_jacket` (`self.BP_Cloth`)) 0 (`self.UnwrapMaterial`)))
    (:`then_2`
      (`MaterialInstanceDynamic.SetVectorParameterValue` (`self.UnwrapMaterial`) "HitLocation" (`KismetMathLibrary.Conv_VectorToLinearColor` (+ (- (`self.Hit Location`) (`self.ActorInitialLocation`)) (0.0 0.0 0.0) (`self.UnwrapLocation`))))
      (`MaterialInstanceDynamic.SetScalarParameterValue` (`self.UnwrapMaterial`) "BrushRadius" (`self.BrushRadius`)))
    (:`then_3`
      (`SceneCaptureComponent2D.CaptureScene` (`self.SceneCapture`))
      (`PrimitiveComponent.SetMaterial` (`/Game/MeshPainter/Blueprints/BP_Cloth.outside_jacket` (`self.BP_Cloth`)) 0 (`self.OriginalMaterial`))
      (`self.K2_SetActorLocation` (`self.BP_Cloth`) (`self.ActorInitialLocation`) false false))))

(event `/Game/MeshPainter/Interface/BPI_Paintable.Paint`
  (params (HitLocation :type "Vector Structure") (BrushRadius :type "Float (double-precision)") (HitActor :type "Actor Object Reference"))
  (goto _label))

(fn `UserConstructionScript`)