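; Mesh-painting capture actor that paints brush hits on characters into a render target through a UV-unwrap material and an orthographic scene capture.
; BeginPlay sets shared unwrap parameters, creates the render target and feeds it to materials for a display plane and the mannequin.
; PaintActor briefly moves the character to the unwrap location, swaps in the unwrap material with hit position and radius, captures, then restores both.
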(event `self.ReceiveBeginPlay`
  (`self.InitializeParameters`
    (:`Out`
      (bind _returnvalue (`KismetMaterialLibrary.CreateDynamicMaterialInstance` "/Game/MeshPainter/Materials/M_Unwrap.M_Unwrap"))
      (set `self.UnwrapMaterial` _returnvalue)
      (bind _returnvalue_2 (`KismetRenderingLibrary.CreateRenderTarget2D` 1024 1024))
      (set `SceneCaptureComponent2D.TextureTarget` _returnvalue_2 (`self.SceneCapture`))
      (bind _returnvalue_3 (`KismetMaterialLibrary.CreateDynamicMaterialInstance` "/Game/MeshPainter/Materials/m_test_Inst.m_test_Inst"))
      (`MaterialInstanceDynamic.SetTextureParameterValue` _returnvalue_3 "RenderTarget" (`SceneCaptureComponent2D.TextureTarget` (`self.SceneCapture`)))
      (bind _returnvalue_4 (`GameplayStatics.GetActorOfClass` "/Game/MeshPainter/Blueprints/BP_Plane.BP_Plane_C"))
      (`PrimitiveComponent.SetMaterial` (`/Game/MeshPainter/Blueprints/BP_Plane.Plane` _returnvalue_4) 0 _returnvalue_3)
      (bind _returnvalue_5 (`GameplayStatics.GetActorOfClass` "/Game/MeshPainter/Characters/Mannequin/MyStudyMannequin.MyStudyMannequin_C"))
      (bind _returnvalue_6 (`PrimitiveComponent.CreateDynamicMaterialInstance` (`Character.Mesh` _returnvalue_5) 0 "/Game/MeshPainter/Characters/Mannequin/Materials/M_Mannequin_Inst.M_Mannequin_Inst" "None"))
      (`MaterialInstanceDynamic.SetTextureParameterValue` _returnvalue_6 "RenderTarget" (`SceneCaptureComponent2D.TextureTarget` (`self.SceneCapture`))))))

(fn `PaintActor`
  (params (ActorToPaint :type "Actor Object Reference") (HitLocation :type "Vector Structure") (BrushRadius :type "Float (double-precision)"))
  (locals (MeshComponent :type "SkeletalMeshComponent Object Reference") (OriginalMaterial :type "MaterialInterface Object Reference") (ActorInitialLocation :type "Vector Structure" :default (0.0 0.0 0.0)))
  (bind _ascharacter (cast `Character` ActorToPaint))
  (set `self.TargetActor` _ascharacter)
  (set `local.MeshComponent` (`Character.Mesh` _ascharacter))
  (set `local.ActorInitialLocation` (`self.K2_GetActorLocation` (`self.TargetActor`)))
  (`self.K2_SetActorLocation` (`self.TargetActor`) (+ (`self.UnwrapLocation`) (0.0 0.0 90.0)) false false)
  (`|ExecutionSequence`
    (:`then_0`
      (set `local.OriginalMaterial` (`PrimitiveComponent.GetMaterial` (`local.MeshComponent`) 0))
      (`PrimitiveComponent.SetMaterial` (`local.MeshComponent`) 0 (`self.UnwrapMaterial`)))
    (:`then_1`
      (`MaterialInstanceDynamic.SetVectorParameterValue` (`self.UnwrapMaterial`) "HitLocation" (`KismetMathLibrary.Conv_VectorToLinearColor` (+ (- (`local.HitLocation`) (`local.ActorInitialLocation`)) (0.0 0.0 90.0) (`self.UnwrapLocation`))))
      (`MaterialInstanceDynamic.SetScalarParameterValue` (`self.UnwrapMaterial`) "BrushRadius" (`local.BrushRadius`)))
    (:`then_2`
      (`SceneCaptureComponent2D.CaptureScene` (`self.SceneCapture`))
      (`PrimitiveComponent.SetMaterial` (`local.MeshComponent`) 0 (`local.OriginalMaterial`))
      (`self.K2_SetActorLocation` (`self.TargetActor`) (`local.ActorInitialLocation`) false false))))

(fn `UserConstructionScript`)