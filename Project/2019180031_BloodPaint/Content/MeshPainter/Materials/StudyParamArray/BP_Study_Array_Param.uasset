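; Study actor for mesh painting that passes an array of paint hits to a material on its Plane through a render target.
; Paint stores hit locations and brush radii up to a fixed count, and Tick shrinks the radii without removing entries.
; Each tick redraws RT_Loc as a data strip, packing range-normalized XY into RG and radius into B.
; The dynamic material receives that texture, its width, Range and the hit count.
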(event `self.ReceiveBeginPlay`
  (bind _crt_hitlocation (`self.CRT_HitLocation`))
  (bind _material (`self.Material`))
  (bind _returnvalue (`PrimitiveComponent.CreateDynamicMaterialInstance` (`self.Plane`) 0 "/Game/MeshPainter/Materials/StudyParamArray/m_study_array_param.m_study_array_param" "None"))
  (set `self.Material` _returnvalue)
  ;[1 1 1] Create CRT Texture
  (`KismetRenderingLibrary.ClearRenderTarget2D` "/Game/MeshPainter/Materials/StudyParamArray/RT_Loc.RT_Loc")
  (set `self.CRT_HitLocation` "/Game/MeshPainter/Materials/StudyParamArray/RT_Loc.RT_Loc")
  (`MaterialInstanceDynamic.SetTextureParameterValue` _material "Tex" _crt_hitlocation)
  (`MaterialInstanceDynamic.SetScalarParameterValue` _material "XSize" (`KismetMathLibrary.Conv_IntToDouble` (`TextureRenderTarget2D.SizeX` _crt_hitlocation)))
  (`MaterialInstanceDynamic.SetScalarParameterValue` (`self.Material`) "Range" (`self.Range`)))

(event `/Game/MeshPainter/Interface/BPI_Paintable.Paint`
  (params (HitLocation :type "Vector Structure") (BrushRadius :type "Float (double-precision)"))
  (bind _hitlocations (`self.HitLocations`))
  ;[1 1 1] 페인팅 BPI
  (if (< (`KismetArrayLibrary.Array_Length` _hitlocations) (`self.HitCountSize`))
    (`KismetArrayLibrary.Array_Add` _hitlocations HitLocation)
    (`KismetArrayLibrary.Array_Add` (`self.HitRadius`) BrushRadius)))

(event `self.ReceiveTick`
  (params (DeltaSeconds :type "Float (single-precision)"))
  (bind _hitradius (`self.HitRadius`))
  (for (_array_element _array_index) _hitradius
    (`KismetArrayLibrary.Array_Set` _hitradius _array_index (- _array_element 0.1)))
  (`self.SetTexture`))

(event `SetTexture`
  (bind _crt_hitlocation (`self.CRT_HitLocation`))
  (bind _range (`self.Range`))
  (`MaterialInstanceDynamic.SetScalarParameterValue` (`self.Material`) "HitCounts" 0.0)
  (`KismetRenderingLibrary.ClearRenderTarget2D` _crt_hitlocation)
  (bind (_canvas _size _context) (`KismetRenderingLibrary.BeginDrawCanvasToRenderTarget` _crt_hitlocation))
  (for (_array_element _array_index) (`self.HitLocations`)
    (bind (_returnvalue_x _returnvalue_y) (`KismetMathLibrary.BreakVector` (/ (+ _array_element _range) (* _range 2.0))))
    (`Canvas.K2_DrawTexture` _canvas null (`KismetMathLibrary.MakeVector2D` (`KismetMathLibrary.Conv_IntToDouble` (- (* _array_index 4) 2))) (4.0 1.0) (0.0 0.0) (1.0 1.0) (`KismetMathLibrary.MakeColor` _returnvalue_x _returnvalue_y (/ (`|GetArrayItem` (`self.HitRadius`) _array_index) 50.0)) "BLEND_Translucent" 0.0 (0.5 0.5)))
  (`KismetRenderingLibrary.EndDrawCanvasToRenderTarget` _context)
  (`MaterialInstanceDynamic.SetScalarParameterValue` (`self.Material`) "HitCounts" (`KismetMathLibrary.Conv_IntToDouble` (`KismetArrayLibrary.Array_Length` (`self.HitLocations`)))))

(fn `UserConstructionScript`)