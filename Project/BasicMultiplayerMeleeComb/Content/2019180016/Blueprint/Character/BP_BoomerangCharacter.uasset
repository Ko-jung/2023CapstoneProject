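; Boomerang character Blueprint with two thrown grab abilities, bound directly to the Z and Q keys.
; Each press passes through an OnServer event to an OnClient event that spawns the actor, handing over the thrower and its first tag as team.
; Z spawns Boomerang_GrabCenter aimed along the forward vector.
; Q spawns Boomerang_Grab, whose EndLocation is the scaled forward vector without the actor's location added.
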(event `self.ReceiveBeginPlay`
  (`parent.ReceiveBeginPlay`))

(event `Key|Z`
  (params (Key :type "Key Structure"))
  (:`Pressed`
    (`self.Spawn Z Grab On Server` (`self.K2_GetActorLocation`) (`self.GetActorForwardVector`) self (`|GetArrayItem` (`self.Tags`)))))

(event `Spawn Z Grab On Server`
  (params (`Spawn Transform Location` :type "Vector Structure") (TargetVector :type "Vector Structure") (ThrowCharacter :type "Character Object Reference") (WhoSpawnTeam :type Name))
  (`self.Spawn Z Grab On Client` `Spawn Transform Location` TargetVector ThrowCharacter WhoSpawnTeam))

(event `Key|Q`
  (params (Key :type "Key Structure"))
  (:`Pressed`
    (`self.Spawn Bommerang Grab On Server` (`self.K2_GetActorLocation`) (* (`self.GetActorForwardVector`) 1000.0) self (`|GetArrayItem` (`self.Tags`)))))

(event `Spawn Z Grab On Client`
  (params (`Spawn Transform Location` :type "Vector Structure") (TargetVector :type "Vector Structure") (ThrowCharacter :type "Character Object Reference") (WhoSpawnTeam :type Name))
  (`|SpawnActorFromClass` "/Game/2019180016/Blueprint/SkillBP/Boomerang_GrabCenter.Boomerang_GrabCenter_C" (`KismetMathLibrary.MakeTransform` `Spawn Transform Location`) "Undefined" "MultiplyWithRoot" null TargetVector ThrowCharacter WhoSpawnTeam null))

(event `Spawn Bommerang Grab On Server`
  (params (`Start Location` :type "Vector Structure") (EndLocation :type "Vector Structure") (ThrowChar :type "Character Object Reference") (WhoSpawnTeam :type Name))
  (`self.Spawn Bommerang Grab On Client` `Start Location` EndLocation ThrowChar WhoSpawnTeam))

(event `Spawn Bommerang Grab On Client`
  (params (`Start Location` :type "Vector Structure") (EndLocation :type "Vector Structure") (ThrowChar :type "Character Object Reference") (WhoSpawnTeam :type Name))
  (`|SpawnActorFromClass` "/Game/2019180016/Blueprint/SkillBP/Boomerang_Grab.Boomerang_Grab_C" (`KismetMathLibrary.MakeTransform` `Start Location`) "Undefined" "MultiplyWithRoot" null `Start Location` EndLocation ThrowChar WhoSpawnTeam null))

(fn `UserConstructionScript`
  (`parent.UserConstructionScript`))