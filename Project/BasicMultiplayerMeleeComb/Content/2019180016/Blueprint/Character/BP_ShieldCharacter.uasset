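; Player character with a shield that is raised while the right mouse button is held and a throwable sphere on Z.
; Open and close events move, rescale and rotate the shield mesh between two spawn points, with opening gated on the shield being alive.
; Z passes a location ahead of the character and its team tag through server- and client-named events to spawn BP_ShieldSphereThrow.
; Shield hits only print a debug message.
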(event `self.ShieldMesh.OnComponentHit`
  (params (HitComponent :type "PrimitiveComponent Object Reference") (OtherActor :type "Actor Object Reference") (OtherComp :type "PrimitiveComponent Object Reference") (NormalImpulse :type "Vector Structure") (Hit :type "HitResult Structure (by ref)"))
  (`KismetSystemLibrary.PrintString` "Shield Damaged!"))

(event `Key|RightMouseButton`
  (params (Key :type "Key Structure"))
  (:`Pressed`
    (`self.OpenShield`))
  (:`Released`
    (`self.CloseShield`)))

(event `OpenShield`
  (bind _shieldmesh (`self.ShieldMesh`))
  (bind (_returnvalue_roll _returnvalue_pitch _returnvalue_yaw) (`KismetMathLibrary.BreakRotator` (`KismetMathLibrary.Conv_VectorToRotator` (`self.GetActorForwardVector`))))
  (`/Engine/EditorBlueprintResources/StandardMacros.IsValid` _shieldmesh
    (:`Is Valid`
      (if (`self.IsShieldAlive`)
        (`SceneComponent.K2_SetWorldLocation` _shieldmesh (`SceneComponent.K2_GetComponentLocation` (`self.RIghtClickShieldSpawnPoint`)) false false)
        (`SceneComponent.SetWorldScale3D` (`self.ShieldMesh`) (1.0 1.0 1.0))
        (`SceneComponent.K2_SetWorldRotation` (`self.ShieldMesh`) (`KismetMathLibrary.MakeRotator` 0.0 0.0 _returnvalue_yaw) false false)
        (set `self.IsClickingRight` true)))))

(event `CloseShield`
  (bind _shieldmesh (`self.ShieldMesh`))
  (`/Engine/EditorBlueprintResources/StandardMacros.IsValid` _shieldmesh
    (:`Is Valid`
      (`SceneComponent.K2_SetWorldLocation` _shieldmesh (`SceneComponent.K2_GetComponentLocation` (`self.ShieldSpawnPoint`)) false false)
      (`SceneComponent.SetWorldScale3D` (`self.ShieldMesh`) (0.15 0.15 0.15))
      (`SceneComponent.K2_SetWorldRotation` (`self.ShieldMesh`) (`KismetMathLibrary.Conv_VectorToRotator` (`SceneComponent.GetForwardVector` (`self.ShieldSpawnPoint`))) false false)
      (set `self.IsClickingRight` false))))

(event `Key|Z`
  (params (Key :type "Key Structure"))
  (:`Pressed`
    (`self.Spawn Sphere Throw On Server` (+ (`self.K2_GetActorLocation`) (* (`self.GetActorForwardVector`) 200.0)) (`|GetArrayItem` (`self.Tags`)))))

(event `Spawn Sphere Throw On Server`
  (params (`Spawn Transform Location` :type "Vector Structure") (WhoSpawnTeam :type Name))
  (`self.Spawn Sphere Throw On Client` `Spawn Transform Location` WhoSpawnTeam))

(event `Spawn Sphere Throw On Client`
  (params (`Spawn Transform Location` :type "Vector Structure") (WhoSpawnTeam :type Name))
  (`|SpawnActorFromClass` "/Game/2019180016/Blueprint/SkillBP/BP_ShieldSphereThrow.BP_ShieldSphereThrow_C" (`KismetMathLibrary.MakeTransform` `Spawn Transform Location`) "Undefined" "OverrideRootScale" null self WhoSpawnTeam null))

(fn `UserConstructionScript`
  (`parent.UserConstructionScript`))