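; BP_Bullet is a projectile actor in the SkillBP folder that flies straight along its forward vector.
; Tick adds to a Timer and moves the actor by Speed scaled by delta time, without sweep.
; The five-second timer check and the mesh overlap event lead to nothing.
; Cast, DestroyActor and debug print nodes are unreachable, so the bullet never destroys itself in this graph.
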(event `self.ReceiveTick`
  (params (DeltaSeconds :type "Float (single-precision)"))
  (set `self.Timer` (+ (`self.Timer`) DeltaSeconds))
  (`self.K2_SetActorLocation` (+ (`self.K2_GetActorLocation`) (* (`self.GetActorForwardVector`) (`self.Speed`) DeltaSeconds)))
  (if (>= (`self.Timer`) 5.0)
    _))

(event `self.StaticMeshComponent.OnComponentBeginOverlap`
  (params (OverlappedComponent :type "PrimitiveComponent Object Reference") (OtherActor :type "Actor Object Reference") (OtherComp :type "PrimitiveComponent Object Reference") (OtherBodyIndex :type Integer) (bFromSweep :type Boolean) (SweepResult :type "HitResult Structure (by ref)")))

(fn `UserConstructionScript`)