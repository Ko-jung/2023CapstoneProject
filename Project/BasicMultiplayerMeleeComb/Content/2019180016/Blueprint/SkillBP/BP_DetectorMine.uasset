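; BP_DetectorMine is a skill mine that emits expanding detection pulses to reveal non-allied characters.
; While IsSetting is true, Tick runs a five-second Delay, then shows the sphere, enables its query collision and scales it up through the BoomSphere timeline.
; Non-allied BP_ThirdPersonCharacters overlapping SphereCollision get Detecting(true).
; When the timeline finishes, it hides the sphere, disables collision and resets its time, letting Tick repeat the pulse.
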(event `self.ReceiveBeginPlay`
  (`parent.ReceiveBeginPlay`)
  (`self.SphereVisiable` false))

(event `self.ReceiveTick`
  (params (DeltaSeconds :type "Float (single-precision)"))
  (if (`self.IsSetting`)
    (`KismetSystemLibrary.Delay` 5.0)
    (`self.SphereVisiable` true)
    (bind (_direction _newtrack_0) (`Timeline|BoomSphere` :!label _label)
      (:`Update`
        (`SceneComponent.SetWorldScale3D` (`self.Sphere`) (`KismetMathLibrary.Conv_DoubleToVector` (`KismetMathLibrary.Lerp` 0.25 100.0 _newtrack_0))))
      (:`Finished`
        (`|ExecutionSequence`
          (:`then_0`
            (`self.SphereVisiable` false))
          (:`then_1`
            (goto _label :!via `SetNewTime`)))))))

(event `self.SphereCollision.OnComponentBeginOverlap`
  (params (OverlappedComponent :type "PrimitiveComponent Object Reference") (OtherActor :type "Actor Object Reference") (OtherComp :type "PrimitiveComponent Object Reference") (OtherBodyIndex :type Integer) (bFromSweep :type Boolean) (SweepResult :type "HitResult Structure (by ref)"))
  (bind _asbp_third_person_character (cast `/Game/DeleteLater_ThirdPerson/Blueprints/BP_ThirdPersonCharacter` OtherActor))
  (if (not (`self.IsAllience?` _asbp_third_person_character))
    (`/Game/DeleteLater_ThirdPerson/Blueprints/BP_ThirdPersonCharacter.Detecting` _asbp_third_person_character true)))

(fn `IsAllience?_0`)

(fn `SphereVisiable`
  (params (`IsVisible?` :type Boolean))
  (bind _spherecollision (`self.SphereCollision`))
  (bind _sphere (`self.Sphere`))
  (if `IsVisible?`
    (`SceneComponent.SetVisibility` _sphere true false)
    (`PrimitiveComponent.SetCollisionEnabled` _spherecollision "QueryOnly")
    (`SceneComponent.SetVisibility` _spherecollision true false)
    (else
      (`SceneComponent.SetVisibility` _sphere false false)
      (`PrimitiveComponent.SetCollisionEnabled` _spherecollision "NoCollision")
      (`SceneComponent.SetVisibility` _spherecollision false false))))

(fn `UserConstructionScript`)