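; BP_ShieldSphere is a skill actor with a sphere volume that speeds up allied third-person characters inside it.
; On begin overlap, it raises the walk speed of characters that pass the IsAllience check.
; On end overlap, it sets any third-person character to a fixed lower speed, without checking alliance or restoring the previous value.
; BeginPlay only calls the parent, and the file contains no shielding logic.
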(event `self.ReceiveBeginPlay`
  (`parent.ReceiveBeginPlay`))

(event `self.Sphere1.OnComponentBeginOverlap`
  (params (OverlappedComponent :type "PrimitiveComponent Object Reference") (OtherActor :type "Actor Object Reference") (OtherComp :type "PrimitiveComponent Object Reference") (OtherBodyIndex :type Integer) (bFromSweep :type Boolean) (SweepResult :type "HitResult Structure (by ref)"))
  (bind _asbp_third_person_character (cast `/Game/DeleteLater_ThirdPerson/Blueprints/BP_ThirdPersonCharacter` OtherActor))
  (if (`self.IsAllience?` _asbp_third_person_character)
    (set `CharacterMovementComponent.MaxWalkSpeed` 1200.0 (`Character.CharacterMovement` _asbp_third_person_character))))

(event `self.Sphere1.OnComponentEndOverlap`
  (params (OverlappedComponent :type "PrimitiveComponent Object Reference") (OtherActor :type "Actor Object Reference") (OtherComp :type "PrimitiveComponent Object Reference") (OtherBodyIndex :type Integer))
  (bind _asbp_third_person_character (cast `/Game/DeleteLater_ThirdPerson/Blueprints/BP_ThirdPersonCharacter` OtherActor))
  (set `CharacterMovementComponent.MaxWalkSpeed` 500.0 (`Character.CharacterMovement` _asbp_third_person_character)))

(fn `UserConstructionScript`)