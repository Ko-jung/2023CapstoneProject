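; BP_SkillActor is a skill actor, apparently a base for spawned skills, that carries the team of whoever spawned it.
; On BeginPlay it adds WhoSpawnTeam to its Tags and turns on replication of itself and its movement.
; IsAllience? identifies allies by comparing the other character's first tag with its own, so team checks depend on the team tag being at index zero.
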(event `self.ReceiveBeginPlay`
  (`KismetArrayLibrary.Array_Add` (`self.Tags`) (`self.WhoSpawnTeam`))
  (`self.SetReplicates` true)
  (`self.SetReplicateMovement` true))

(fn `IsAllience?`
  (params (OtherCharacter :type "Character Object Reference"))
  (returns (Return :type Boolean))
  (if (== (`|GetArrayItem` (`Actor.Tags` OtherCharacter)) (`|GetArrayItem` (`self.Tags`)))
    (return true)
    (else
      (return false))))

(fn `UserConstructionScript`)