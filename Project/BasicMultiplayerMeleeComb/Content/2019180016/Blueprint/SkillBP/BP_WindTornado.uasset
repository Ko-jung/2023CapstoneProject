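; Wind tornado skill actor that captures non-allied third-person characters, pulls them in and throws them out the top.
; Box overlap captures characters with a clear Visibility trace; blocked ones wait in a list retraced on Tick.
; Tick pulls captured characters toward TracePoint; Sphere overlap switches them to spinning and rising until TopPoint, then launches them in random directions.
; DisableKeyboardInput toggles mapping context and Flying/Walking movement on capture and release.
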(event `self.ReceiveTick`
  (params (DeltaSeconds :type "Float (single-precision)"))
  (bind _overlaplist (`self.OverlapList`))
  (bind (_returnvalue_x _returnvalue_y _returnvalue_z) (`KismetMathLibrary.BreakVector` (`SceneComponent.K2_GetComponentLocation` (`self.TopPoint`))))
  (`|ExecutionSequence`
    (:`then_0`
      (if (>= (`KismetArrayLibrary.Array_Length` _overlaplist) 1)
        (for _array_element _overlaplist
          (bind _returnvalue (`self.K2_GetActorLocation` _array_element))
          (`self.K2_SetActorLocation` _array_element (+ _returnvalue (* (`KismetMathLibrary.Normal` (- (`SceneComponent.K2_GetComponentLocation` (`self.TracePoint`)) _returnvalue)) 3.0)) false false))))
    (:`then_1`
      (for _array_element_2 (`self.CantOverlapList`)
        (bind (_outhit _returnvalue_2) (`KismetSystemLibrary.LineTraceSingle` :`Start` (`SceneComponent.K2_GetComponentLocation` (`self.TracePoint`)) :`End` (`self.K2_GetActorLocation` _array_element_2) :`TraceChannel` "TraceTypeQuery1" :`DrawDebugType` "ForOneFrame"))
        (if (not _returnvalue_2)
          (`self.DisableKeyboardInput` _array_element_2 true)
          (`KismetArrayLibrary.Array_Add` (`self.OverlapList`) _array_element_2)
          (`KismetArrayLibrary.Array_RemoveItem` (`self.CantOverlapList`) _array_element_2))))
    (:`then_2`
      (for _array_element_3 (`self.UpOverlapList`)
        (`self.K2_AddActorWorldRotation` _array_element_3 (struct :`Yaw` 5.0) false false)
        (bind _returnvalue_3 (`self.K2_GetActorLocation` _array_element_3))
        (`self.K2_SetActorLocation` _array_element_3 (+ _returnvalue_3 (0.0 0.0 3.0)) false false)
        (if (>= (`.Z` (`KismetMathLibrary.BreakVector3f` _returnvalue_3)) _returnvalue_z)
          (`self.DisableKeyboardInput` _array_element_3)
          (`Character.LaunchCharacter` _array_element_3 (* (+ (`KismetMathLibrary.Normal` (`KismetMathLibrary.MakeVector` (`KismetMathLibrary.RandomFloatInRange` -1.0 1.0) (`KismetMathLibrary.RandomFloatInRange` -1.0 1.0))) (0.0 0.0 0.75)) 1000.0) false false)
          (`KismetArrayLibrary.Array_RemoveItem` (`self.UpOverlapList`) _array_element_3))))))

(event `self.Box.OnComponentBeginOverlap`
  (params (OverlappedComponent :type "PrimitiveComponent Object Reference") (OtherActor :type "Actor Object Reference") (OtherComp :type "PrimitiveComponent Object Reference") (OtherBodyIndex :type Integer) (bFromSweep :type Boolean) (SweepResult :type "HitResult Structure (by ref)"))
  (bind _asbp_third_person_character (cast `/Game/DeleteLater_ThirdPerson/Blueprints/BP_ThirdPersonCharacter` OtherActor))
  (if (not (`self.IsAllience?` _asbp_third_person_character))
    (bind (_outhit _returnvalue) (`KismetSystemLibrary.LineTraceSingle` (`SceneComponent.K2_GetComponentLocation` (`self.TracePoint`)) (`self.K2_GetActorLocation` _asbp_third_person_character) "TraceTypeQuery1"))
    (if _returnvalue
      (`KismetArrayLibrary.Array_Add` (`self.CantOverlapList`) _asbp_third_person_character)
      (else
        (`self.DisableKeyboardInput` _asbp_third_person_character true)
        (`KismetArrayLibrary.Array_Add` (`self.OverlapList`) _asbp_third_person_character)))))

(event `self.Box.OnComponentEndOverlap`
  (params (OverlappedComponent :type "PrimitiveComponent Object Reference") (OtherActor :type "Actor Object Reference") (OtherComp :type "PrimitiveComponent Object Reference") (OtherBodyIndex :type Integer))
  (bind _asbp_third_person_character (cast `/Game/DeleteLater_ThirdPerson/Blueprints/BP_ThirdPersonCharacter` OtherActor))
  (if (not (`self.IsAllience?` _asbp_third_person_character))
    (`KismetArrayLibrary.Array_RemoveItem` (`self.CantOverlapList`) _asbp_third_person_character)))

(event `self.Sphere.OnComponentBeginOverlap`
  (params (OverlappedComponent :type "PrimitiveComponent Object Reference") (OtherActor :type "Actor Object Reference") (OtherComp :type "PrimitiveComponent Object Reference") (OtherBodyIndex :type Integer) (bFromSweep :type Boolean) (SweepResult :type "HitResult Structure (by ref)"))
  (bind _asbp_third_person_character (cast `/Game/DeleteLater_ThirdPerson/Blueprints/BP_ThirdPersonCharacter` OtherActor))
  (if (not (`self.IsAllience?` _asbp_third_person_character))
    (`KismetArrayLibrary.Array_Add` (`self.UpOverlapList`) _asbp_third_person_character)
    (`KismetArrayLibrary.Array_RemoveItem` (`self.OverlapList`) _asbp_third_person_character)))

(fn `DisableKeyboardInput`
  (params (Character :type "Character Object Reference") (`IsIntoTornado?` :type Boolean))
  (bind _charactermovement (`Character.CharacterMovement` Character))
  (if `IsIntoTornado?`
    (bind _asbp_third_person_character (cast `/Game/DeleteLater_ThirdPerson/Blueprints/BP_ThirdPersonCharacter` Character))
    (`/Game/DeleteLater_ThirdPerson/Blueprints/BP_ThirdPersonCharacter.ChangeMaapingContext` _asbp_third_person_character "NewEnumerator1")
    (`CharacterMovementComponent.SetMovementMode` _charactermovement "MOVE_Flying" 0)
    (set `CharacterMovementComponent.BrakingDecelerationFlying` 10000.0 _charactermovement)
    (else
      (bind _asbp_third_person_character_2 (cast `/Game/DeleteLater_ThirdPerson/Blueprints/BP_ThirdPersonCharacter` Character))
      (`/Game/DeleteLater_ThirdPerson/Blueprints/BP_ThirdPersonCharacter.ChangeMaapingContext` _asbp_third_person_character_2 "NewEnumerator0")
      (`CharacterMovementComponent.SetMovementMode` _charactermovement "MOVE_Walking" 0)
      (set `CharacterMovementComponent.BrakingDecelerationFlying` 0.0 _charactermovement)))
  (return))

(fn `UserConstructionScript`)