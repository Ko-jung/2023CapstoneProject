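; Boomerang_Grab is a skill projectile that catches a non-allied character and drags it along its path.
; On BeginPlay it gets a random spin, and a timeline moves it from StartLocation by a curve-scaled EndLocation offset, destroying it when finished.
; A sphere overlap stores the latest non-allied Character, which Tick then snaps to the projectile's location every frame.
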(event `self.ReceiveBeginPlay`
  (`parent.ReceiveBeginPlay`)
  (set `RotatingMovementComponent.RotationRate` (`KismetMathLibrary.MakeRotator` (`KismetMathLibrary.RandomFloatInRange` -360.0 360.0) (`KismetMathLibrary.RandomFloatInRange` -360.0 360.0) (`KismetMathLibrary.RandomFloatInRange` -360.0 360.0)) (`self.RotatingMovement`))
  (bind (_direction _newtrack_1) (`Timeline|Timeline` :!label _label)
    (:`Update`
      (`SceneComponent.K2_SetRelativeLocation` (`self.DefaultSceneRoot`) (+ (`self.StartLocation`) (* (`self.EndLocation`) _newtrack_1)) false false))
    (:`Finished`
      (`|ExecutionSequence`
        (:`then_0`
          (goto _label :!via `SetNewTime`))
        (:`then_1`
          (`self.K2_DestroyActor`))))))

(event `self.ReceiveTick`
  (params (DeltaSeconds :type "Float (single-precision)"))
  (if (`self.IsGrabbing`)
    (`self.K2_SetActorLocation` (`self.GrabbedCharacter`) (`self.K2_GetActorLocation`) false false)))

(event `self.Sphere.OnComponentBeginOverlap`
  (params (OverlappedComponent :type "PrimitiveComponent Object Reference") (OtherActor :type "Actor Object Reference") (OtherComp :type "PrimitiveComponent Object Reference") (OtherBodyIndex :type Integer) (bFromSweep :type Boolean) (SweepResult :type "HitResult Structure (by ref)"))
  (bind _ascharacter (cast `Character` OtherActor))
  (if (not (`self.IsAllience?` _ascharacter))
    (set `self.GrabbedCharacter` _ascharacter)
    (set `self.IsGrabbing` true)))

(fn `UserConstructionScript`)