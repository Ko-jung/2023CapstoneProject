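; Boomerang skill projectile that spins, chains between characters other than its thrower, then pulls those it hit together.
; Each new character hit is recorded, and a sphere trace steers the projectile toward a nearby unrecorded character, resetting its lifetime.
; When the trace finds no new target, Tick launches recorded characters toward their average location with upward lift, then destroys the actor.
; It also destroys itself on non-character overlap or timeout.
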(event `self.ReceiveBeginPlay`
  (set `RotatingMovementComponent.RotationRate` (`KismetMathLibrary.MakeRotator` (`KismetMathLibrary.RandomFloatInRange` -360.0 360.0) (`KismetMathLibrary.RandomFloatInRange` -360.0 360.0) (`KismetMathLibrary.RandomFloatInRange` -360.0 360.0)) (`self.RotatingMovement`)))

(event `self.ReceiveTick`
  (params (DeltaSeconds :type "Float (single-precision)"))
  (`|ExecutionSequence`
    (:`then_0`
      (if (`self.NoMoreAddToArray`)
        (bind _centerlocation (`self.Get Center Location To Grab And Set Location Array`))
        (for _array_element (`self.BlockCharacterArray`)
          (`Character.LaunchCharacter` _array_element (* (+ (`KismetMathLibrary.Normal` (- _centerlocation (`self.K2_GetActorLocation` _array_element))) (0.0 0.0 1.0)) 400.0) false false))
        (`self.K2_DestroyActor`)))
    (:`then_1`
      (bind _output_get (set `self.Timer` (+ DeltaSeconds (`self.Timer`))))
      (if (>= _output_get 5.0)
        (`self.K2_DestroyActor`)
        (else
          (`self.K2_SetActorLocation` (+ (`self.K2_GetActorLocation`) (* (`self.TargetVector`) (`self.Speed`) DeltaSeconds))))))))

(event `self.Sphere.OnComponentBeginOverlap`
  (params (OverlappedComponent :type "PrimitiveComponent Object Reference") (OtherActor :type "Actor Object Reference") (OtherComp :type "PrimitiveComponent Object Reference") (OtherBodyIndex :type Integer) (bFromSweep :type Boolean) (SweepResult :type "HitResult Structure (by ref)"))
  (bind _returnvalue (`self.K2_GetActorLocation`))
  (bind _blockcharacterarray (`self.BlockCharacterArray`))
  (bind _ascharacter (cast `Character` OtherActor)
    (:`then`
      (if (== _ascharacter (`self.ThrowCharacter`))
        _
        (elif (== (`KismetArrayLibrary.Array_Length` (`self.BlockCharacterArray`)) 0)
          (`KismetArrayLibrary.Array_Add` _blockcharacterarray _ascharacter)
          (bind (_outhits _returnvalue_2) (`KismetSystemLibrary.SphereTraceMulti` :`Start` _returnvalue :`End` _returnvalue :`Radius` 500.0 :`TraceChannel` "TraceTypeQuery3" :`DrawDebugType` "ForDuration" :!label _label))
          (if _returnvalue_2
            (set `self.NoMoreAddToArray` true)
            (for _array_element _outhits
              (bind (_bblockinghit _binitialoverlap _time _distance _location _impactpoint _normal _impactnormal _physmat _hitactor) (`GameplayStatics.BreakHitResult` _array_element))
              (`KismetSystemLibrary.PrintString` (`KismetSystemLibrary.GetDisplayName` _hitactor))
              (bind _ascharacter_2 (cast `Character` _hitactor))
              (if (== (`KismetArrayLibrary.Array_Find` (`self.BlockCharacterArray`) _ascharacter_2) -1)
                (set `self.Timer` 0.0)
                (set `self.TargetVector` (`KismetMathLibrary.Normal` (- (`self.K2_GetActorLocation` _ascharacter_2) (`self.K2_GetActorLocation`))))
                (set `self.NoMoreAddToArray` false)
                (break))))
          (else
            (bind _adddone (`self.Char Add to Array` _ascharacter _blockcharacterarray))
            (if _adddone
              (goto _label))))))
    (:`CastFailed`
      (`self.K2_DestroyActor`))))

(fn `Char Add to Array`
  (params (FindCharacter :type "Character Object Reference (by ref)") (BlockedCharArray :type "Array of Character Object Reference (by ref)"))
  (returns (AddDone :type Boolean))
  (if (== (`KismetArrayLibrary.Array_Find` BlockedCharArray FindCharacter) -1)
    (`KismetArrayLibrary.Array_Add` BlockedCharArray FindCharacter)
    (`KismetSystemLibrary.PrintString` (`KismetStringLibrary.Concat_StrStr` (`KismetSystemLibrary.GetDisplayName` FindCharacter) "Is Append!"))
    (return true)
    (else
      (return false))))

(fn `Get Center Location To Grab And Set Location Array`
  (returns (CenterLocation :type "Vector Structure"))
  (bind _blockcharacterarray (`self.BlockCharacterArray`))
  (for _array_element _blockcharacterarray
    (bind _returnvalue (`self.K2_GetActorLocation` _array_element))
    (set `self.GrabSumLocation` (+ _returnvalue (`self.GrabSumLocation`)))
    (`KismetArrayLibrary.Array_Add` (`self.BlockCharacterLocationArray`) _returnvalue))
  (bind _output_get (set `self.GrabToCenterLocation` (/ (`self.GrabSumLocation`) (`KismetArrayLibrary.Array_Length` _blockcharacterarray))))
  (return _output_get))

(fn `PrintAllCharacterArray`
  (bind _blockcharacterarray (`self.BlockCharacterArray`))
  (for _index (range (`KismetArrayLibrary.Array_Length` _blockcharacterarray))
    (`KismetSystemLibrary.PrintString` (`KismetSystemLibrary.GetDisplayName` (`|GetArrayItem` _blockcharacterarray _index)))))

(fn `UserConstructionScript`)