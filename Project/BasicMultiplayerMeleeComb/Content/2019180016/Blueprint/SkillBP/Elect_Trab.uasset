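; Elect_Trab is a thrown-style skill trap that falls under physics, sticks to the first non-character it hits, then homes in on nearby actors.
; On attach it stops simulating and aligns to the impact normal.
; Each tick while attached, it sphere-traces for a target and moves its mesh toward it unless a visibility trace is blocked.
; Hitting a character while attached spawns an explosion, launches the character upward and destroys the trap.
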(event `self.ReceiveBeginPlay`
  (set `self.IsAttach` false)
  (`PrimitiveComponent.SetSimulatePhysics` (`self.StaticMesh`) true))

(event `self.ReceiveTick`
  (params (DeltaSeconds :type "Float (single-precision)"))
  (bind _returnvalue (`self.K2_GetActorLocation`))
  (bind _returnvalue_2 (`self.K2_GetActorLocation`))
  (if (`self.IsAttach`)
    (bind (_outhit _returnvalue_3) (`KismetSystemLibrary.SphereTraceSingle` :`Start` _returnvalue :`End` _returnvalue :`Radius` 1000.0 :`TraceChannel` "TraceTypeQuery3" :`DrawDebugType` "ForOneFrame"))
    (if _returnvalue_3
      (bind _returnvalue_4 (`self.K2_GetActorLocation` (`.HitActor` (`GameplayStatics.BreakHitResult` _outhit))))
      (bind (_outhit_2 _returnvalue_5) (`KismetSystemLibrary.LineTraceSingle` _returnvalue_2 _returnvalue_4 "TraceTypeQuery1"))
      (if _returnvalue_5
        (`KismetSystemLibrary.PrintString` "Yesy")
        (else
          (`SceneComponent.K2_AddRelativeLocation` (`self.StaticMesh`) (* (`KismetMathLibrary.Normal` (- _returnvalue_4 _returnvalue_2)) 10.0) true true)
          (`KismetSystemLibrary.PrintString` "No"))))))

(event `self.StaticMesh.OnComponentHit`
  (params (HitComponent :type "PrimitiveComponent Object Reference") (OtherActor :type "Actor Object Reference") (OtherComp :type "PrimitiveComponent Object Reference") (NormalImpulse :type "Vector Structure") (Hit :type "HitResult Structure (by ref)"))
  (bind (_bblockinghit _binitialoverlap _time _distance _location _impactpoint _normal _impactnormal) (`GameplayStatics.BreakHitResult` Hit))
  (bind _ascharacter (cast `Character` OtherActor)
    (:`then`
      (if (`self.IsAttach`)
        (`GameplayStatics.SpawnEmitterAtLocation` "/Game/StarterContent/Particles/P_Explosion.P_Explosion" (`self.K2_GetActorLocation`))
        (`Character.LaunchCharacter` _ascharacter (0.0 0.0 1000.0) false false)
        (`self.K2_DestroyActor`)))
    (:`CastFailed`
      (set `self.IsAttach` true)
      (`PrimitiveComponent.SetSimulatePhysics` (`self.StaticMesh`) false)
      (`self.K2_SetActorRotation` (`KismetMathLibrary.MakeRotFromZX` _impactnormal (`self.GetActorUpVector`)))
      (`self.K2_SetActorLocation` (+ _location (* (`self.GetActorUpVector`) 5.0))))))

(fn `UserConstructionScript`)