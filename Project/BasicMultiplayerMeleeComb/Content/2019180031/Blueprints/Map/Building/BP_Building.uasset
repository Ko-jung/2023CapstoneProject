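; Multi-storey destructible building that collapses from a given floor upward.
; The construction script stacks static mesh components for each floor slab and four walls, stored in per-part arrays.
; DestructBuilding swaps those pieces, up to the current top, for Geometry Collection components at the same locations via SwapStaticToGeometry, then lowers CurrentFloor.
; Test events experiment with repeatedly applying upward velocity to a Geometry Collection.
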(event `self.ReceiveBeginPlay`
  (bind _output_get (set `self.CurrentFloor` (`self.Floor`))) ; 0~n-1층임
  (`KismetSystemLibrary.PrintString` (`KismetStringLibrary.Conv_IntToString` _output_get))
  (`KismetSystemLibrary.Delay` 1.0))

(event `Test`
  (`ActorComponent.K2_DestroyComponent` (`self.NewVar`))
  (bind _returnvalue (`AddComponent|NODE_AddGeometryCollectionComponent-10`))
  (`self.TestGravity` _returnvalue)
  (`KismetSystemLibrary.PrintString` "Hello"))

(event `DestructBuilding`
  (params (Floor :type Integer))
  (for _index (range Floor (+ (`self.CurrentFloor`) 1))
    (`KismetSystemLibrary.PrintString` (`KismetStringLibrary.Conv_IntToString` _index))
    (`|ExecutionSequence`
      (:`then_0`
        (`self.SwapStaticToGeometry` (`|GetArrayItem` (`self.Building_Floor`) _index) "/Game/2019180031/Blueprints/Map/Building/building_floor_building_floor/building_floor_GeometryCollection.building_floor_GeometryCollection"))
      (:`then_1`
        (`self.SwapStaticToGeometry` (`|GetArrayItem` (`self.Building_Wall1`) _index) "/Game/2019180031/Blueprints/Map/Building/building_wall001_building_wall001/building_wall001_GeometryCollection.building_wall001_GeometryCollection"))
      (:`then_2`
        (`self.SwapStaticToGeometry` (`|GetArrayItem` (`self.Building_Wall2`) _index) "/Game/2019180031/Blueprints/Map/Building/building_wall002_building_wall002/building_wall002_GeometryCollection.building_wall002_GeometryCollection"))
      (:`then_3`
        (`self.SwapStaticToGeometry` (`|GetArrayItem` (`self.Building_Wall3`) _index) "/Game/2019180031/Blueprints/Map/Building/building_wall003_building_wall003/building_wall003_GeometryCollection.building_wall003_GeometryCollection"))
      (:`then_4`
        (`self.SwapStaticToGeometry` (`|GetArrayItem` (`self.Building_Wall4`) _index) "/Game/2019180031/Blueprints/Map/Building/building_wall004_building_wall004/building_wall004_GeometryCollection.building_wall004_GeometryCollection"))))
  (set `self.CurrentFloor` (- Floor 1)))

(event `TestGravity`
  (params (NewVar_0 :type "GeometryCollectionComponent Object Reference"))
  ;[1 1 1] Comment
  (`GeometryCollectionComponent.ApplyLinearVelocity` NewVar_0 0 (0.0 0.0 140.0))
  (`KismetSystemLibrary.PrintString` "중력?")
  (`KismetSystemLibrary.Delay` 0.2)
  (`self.TestGravity` NewVar_0))

(event `Key|W`
  (params (Key :type "Key Structure")))

(fn `SwapStaticToGeometry`
  (params (Target :type "StaticMeshComponent Object Reference") (RestCollectionIn :type "GeometryCollection Object Reference"))
  (locals (RelativeLocation :type "Vector Structure"))
  (set `local.RelativeLocation` (`SceneComponent.RelativeLocation` Target))
  (`ActorComponent.K2_DestroyComponent` Target)
  (`|ExecutionSequence`
    (:`then_0`
      (if (== RestCollectionIn "/Game/2019180031/Blueprints/Map/Building/building_floor_building_floor/building_floor_GeometryCollection.building_floor_GeometryCollection")
        (`AddComponent|NODE_AddGeometryCollectionComponent-11` :`RelativeTransform` (`KismetMathLibrary.MakeTransform` (`local.RelativeLocation`)))))
    (:`then_1`
      (if (== RestCollectionIn "/Game/2019180031/Blueprints/Map/Building/building_wall001_building_wall001/building_wall001_GeometryCollection.building_wall001_GeometryCollection")
        (`AddComponent|NODE_AddGeometryCollectionComponent-12` :`RelativeTransform` (`KismetMathLibrary.MakeTransform` (`local.RelativeLocation`)))))
    (:`then_2`
      (if (== RestCollectionIn "/Game/2019180031/Blueprints/Map/Building/building_wall002_building_wall002/building_wall002_GeometryCollection.building_wall002_GeometryCollection")
        (`AddComponent|NODE_AddGeometryCollectionComponent-13` :`RelativeTransform` (`KismetMathLibrary.MakeTransform` (`local.RelativeLocation`)))))
    (:`then_3`
      (if (== RestCollectionIn "/Game/2019180031/Blueprints/Map/Building/building_wall003_building_wall003/building_wall003_GeometryCollection.building_wall003_GeometryCollection")
        (`AddComponent|NODE_AddGeometryCollectionComponent-14` :`RelativeTransform` (`KismetMathLibrary.MakeTransform` (`local.RelativeLocation`)))))
    (:`then_4`
      (if (== RestCollectionIn "/Game/2019180031/Blueprints/Map/Building/building_wall004_building_wall004/building_wall004_GeometryCollection.building_wall004_GeometryCollection")
        (`AddComponent|NODE_AddGeometryCollectionComponent-15` :`RelativeTransform` (`KismetMathLibrary.MakeTransform` (`local.RelativeLocation`)))))))

(fn `UserConstructionScript`
  (locals (ChaosObjectType :type "EObjectStateTypeEnum Enum" :default "Chaos_Object_Static"))
  ;[1 1 1] test-1
  (for _index (range (+ (`self.Floor`) 1))
    (`|ExecutionSequence`
      (:`then_0`
        (bind _returnvalue (* _index (`self.FloorDistance`)))
        (bind _returnvalue_2 (`AddComponent|NODE_AddStaticMeshComponent-5` :`RelativeTransform` (`KismetMathLibrary.MakeTransform` (`KismetMathLibrary.MakeVector` 0.0 0.0 (- _returnvalue 500.0)))))
        (`KismetArrayLibrary.Array_Add` (`self.Building_Floor`) _returnvalue_2))
      (:`then_1`
        (bind _returnvalue_3 (`AddComponent|NODE_AddStaticMeshComponent-6` :`RelativeTransform` (`KismetMathLibrary.MakeTransform` (`KismetMathLibrary.MakeVector` 0.0 (`self.Wall1Offset`) _returnvalue))))
        (`KismetArrayLibrary.Array_Add` (`self.Building_Wall1`) _returnvalue_3))
      (:`then_2`
        (bind _returnvalue_4 (`AddComponent|NODE_AddStaticMeshComponent-7` :`RelativeTransform` (`KismetMathLibrary.MakeTransform` (`KismetMathLibrary.MakeVector` (`self.wall2Offset`) 0.0 _returnvalue))))
        (`KismetArrayLibrary.Array_Add` (`self.Building_Wall2`) _returnvalue_4))
      (:`then_3`
        (bind _returnvalue_5 (`AddComponent|NODE_AddStaticMeshComponent-8` :`RelativeTransform` (`KismetMathLibrary.MakeTransform` (`KismetMathLibrary.MakeVector` 0.0 (`self.wall3Offset`) _returnvalue))))
        (`KismetArrayLibrary.Array_Add` (`self.Building_Wall3`) _returnvalue_5))
      (:`then_4`
        (bind _returnvalue_6 (`AddComponent|NODE_AddStaticMeshComponent-9` :`RelativeTransform` (`KismetMathLibrary.MakeTransform` (`KismetMathLibrary.MakeVector` (`self.wall4Offset`) 0.0 _returnvalue))))
        (`KismetArrayLibrary.Array_Add` (`self.Building_Wall4`) _returnvalue_6)))))