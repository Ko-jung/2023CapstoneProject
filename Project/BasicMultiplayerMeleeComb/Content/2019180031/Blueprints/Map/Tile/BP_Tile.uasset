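; Hexagonal map actor that builds the tile arena and collapses it in stages.
; The construction script lays three section-tagged rings of mesh components around a centre using trigonometry and interpolation.
; BeginPlay spawns random buildings, taller toward the centre, and floating tiles, mapping them to tiles in TilesActor.
; Collapse functions either re-centre on a random neighbour and destroy tiles outside a radius, or drop one random tile, adding geometry collections.
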(event `self.ReceiveBeginPlay`
  (`self.Initial Settiongs`))

(fn `CalculateRelativeLocation`
  (params (AngleCount :type Integer) (`Distance(Section)` :type Integer))
  (returns (RelativeLocation :type "Vector Structure"))
  (bind _returnvalue (* (`KismetMathLibrary.Conv_IntToDouble` `Distance(Section)`) (`self.offset`)))
  (bind _returnvalue_2 (+ (* AngleCount 60) 30.0))
  (return (`KismetMathLibrary.MakeVector` (* _returnvalue (`KismetMathLibrary.DegSin` _returnvalue_2)) (* _returnvalue (`KismetMathLibrary.DegCos` _returnvalue_2)))))

(fn `CollapseLevel1And2`
  (params (`Collapse Value` :type "Float (double-precision)"))
  (locals (`Middle Candidate` :type "Array of StaticMeshComponent Object Reference") (MiddleTileRelativeLocation :type "Vector Structure" :default (0.0 0.0 0.0)) (FirstCollapseDistance :type "Float (double-precision)" :default 2.5) (SpawnLocation :type "Vector Structure") (TargetDestroyTile :type "StaticMeshComponent Object Reference") (InvalidDataCount :type Integer))
  (`KismetSystemLibrary.PrintString` (`KismetTextLibrary.Conv_TextToString` (`|FormatText` "시작은 {n}/{b}개" (`KismetArrayLibrary.Array_Length` (`self.Tiles`)) (`BlueprintMapLibrary.Map_Length` (`self.Tile's Actor`)))))
  ;[1 1 1] 중간 타일 설정
  (for _array_element (`self.Tiles`)
    (`/Engine/EditorBlueprintResources/StandardMacros.IsValid` _array_element
      (:`Is Valid`
        (if (`KismetMathLibrary.InRange_FloatFloat` (`KismetMathLibrary.VSize` (- (`SceneComponent.RelativeLocation` _array_element) (`SceneComponent.RelativeLocation` (`self.CurrentMiddleTile`)))) (* (`self.offset`) 0.5) (* (`self.offset`) 1.5))
          (`KismetArrayLibrary.Array_Add` (`local.Middle Candidate`) _array_element)))))
  (bind _output_get (set `self.CurrentMiddleTile` (`KismetArrayLibrary.Array_Random` (`local.Middle Candidate`))))
  (`PrimitiveComponent.SetMaterial` _output_get 0 "/AnimationSharing/AnimSharingRed.AnimSharingRed")
  (`|ExecutionSequence`
    (:`then_0`
      ;[1 1 1] 중간 타일 및 허용 범위 외 모든 타일 붕괴
      (for _array_element_2 (`self.Tiles`)
        (bind _output_get_2 (set `local.TargetDestroyTile` _array_element_2))
        (bind _relativelocation (`SceneComponent.RelativeLocation` _output_get_2))
        (set `local.SpawnLocation` _relativelocation)
        (if (> (`KismetMathLibrary.VSize` (- _relativelocation (`SceneComponent.RelativeLocation` (`self.CurrentMiddleTile`)))) (* (`self.offset`) `Collapse Value`))
          (`GameplayStatics.SpawnEmitterAtLocation` "/Game/StarterContent/Particles/P_Explosion.P_Explosion" _relativelocation (struct) (10.0 10.0 10.0))
          (message `/Game/2019180031/BlueprintInterface/BPI_Collapse.DoCollapse` (`BlueprintMapLibrary.Map_Find` (`self.Tile's Actor`) (`local.TargetDestroyTile`)))
          (`BlueprintMapLibrary.Map_Remove` (`self.Tile's Actor`) (`local.TargetDestroyTile`))
          (`ActorComponent.K2_DestroyComponent` (`local.TargetDestroyTile`))
          (`AddComponent|NODE_AddGeometryCollectionComponent-3` :`RelativeTransform` (`KismetMathLibrary.MakeTransform` (`local.SpawnLocation`)))))
      ;[1 1 1] 배열 속 Invalid 데이터 제거
      (set `local.InvalidDataCount` 1)
      (while (> (`local.InvalidDataCount`) 0)
        (set `local.InvalidDataCount` 0)
        (for (_array_element_3 _array_index) (`self.Tiles`)
          (`/Engine/EditorBlueprintResources/StandardMacros.IsValid` _array_element_3
            (:`Is Not Valid`
              (`/Engine/EditorBlueprintResources/StandardMacros.IncrementInt` (`local.InvalidDataCount`)
                (:`  `
                  (`KismetArrayLibrary.Array_Remove` (`self.Tiles`) _array_index)
                  (break))))))))))

(fn `CollapseLevel3`
  (locals (`Target Tile` :type "StaticMeshComponent Object Reference") (InvalidDataCount :type Integer))
  (bind _target_tile (`local.Target Tile`))
  (set `local.Target Tile` (`KismetArrayLibrary.Array_Random` (`self.Tiles`)))
  (message `/Game/2019180031/BlueprintInterface/BPI_Collapse.DoCollapse` (`BlueprintMapLibrary.Map_Find` (`self.Tile's Actor`) (`local.Target Tile`)))
  (`BlueprintMapLibrary.Map_Remove` (`self.Tile's Actor`) (`local.Target Tile`))
  (`AddComponent|NODE_AddGeometryCollectionComponent-2` :`RelativeTransform` (`KismetMathLibrary.MakeTransform` (`SceneComponent.RelativeLocation` _target_tile)))
  (`ActorComponent.K2_DestroyComponent` _target_tile)
  ;[1 1 1] 배열 속 Invalid 데이터 제거
  (set `local.InvalidDataCount` 1)
  (while (> (`local.InvalidDataCount`) 0)
    (set `local.InvalidDataCount` 0)
    (for (_array_element _array_index) (`self.Tiles`)
      (`/Engine/EditorBlueprintResources/StandardMacros.IsValid` _array_element
        (:`Is Not Valid`
          (`/Engine/EditorBlueprintResources/StandardMacros.IncrementInt` (`local.InvalidDataCount`)
            (:`  `
              (`KismetArrayLibrary.Array_Remove` (`self.Tiles`) _array_index)
              (break))))))))

(fn `Initial Settiongs`
  (bind _currentmiddletile (`self.CurrentMiddleTile`))
  (`|ExecutionSequence`
    (:`then_0`
      (`self.Spawn Buildings And Floating Tiles` 8 "Section1" 3 4 (0.0 0.0 -3000.0)))
    (:`then_1`
      (`self.Spawn Buildings And Floating Tiles` 4 "Section2" 7 2 (0.0 0.0 -5000.0)))
    (:`then_2`
      (`self.Spawn Buildings And Floating Tiles` 2 "Section3" 11 1 (0.0 0.0 -7000.0)))
    (:`then_3`
      (bind _returnvalue (`|SpawnActorFromClass` "/Game/2019180031/Blueprints/Map/Building/BP_Building.BP_Building_C" (`KismetMathLibrary.MakeTransform` (`SceneComponent.RelativeLocation` _currentmiddletile)) "Undefined" "MultiplyWithRoot" null 15 null))
      (`BlueprintMapLibrary.Map_Add` (`self.Tile's Actor`) _currentmiddletile _returnvalue))))

(fn `Spawn Buildings And Floating Tiles`
  (params (`Spawn Count` :type Integer) (`Tile Tag` :type Name) (Floor :type Integer) (FloatingTileCount :type Integer) (`Movement Offset` :type "Vector Structure"))
  (locals (UsedTile :type "Array of StaticMeshComponent Object Reference") (SectionTiles :type "Array of StaticMeshComponent Object Reference") (TargetTile :type "StaticMeshComponent Object Reference"))
  (bind _returnvalue (`KismetArrayLibrary.Array_Length` (`local.UsedTile`)))
  (`|ExecutionSequence`
    (:`then_0`
      ;[1 1 1] 구역 타일 배열 구하기
      (for _array_element (`self.Tiles`)
        (`/Engine/EditorBlueprintResources/StandardMacros.IsValid` _array_element
          (:`Is Valid`
            (if (`ActorComponent.ComponentHasTag` _array_element `Tile Tag`)
              (`KismetArrayLibrary.Array_Add` (`local.SectionTiles`) _array_element))))))
    (:`then_1`
      ;[1 1 1] 빌딩 배치
      (while (< (`KismetArrayLibrary.Array_Length` (`local.UsedTile`)) `Spawn Count`)
        (bind _output_get (set `local.TargetTile` (`KismetArrayLibrary.Array_Random` (`local.SectionTiles`))))
        (while (not (`KismetArrayLibrary.Array_Contains` (`local.UsedTile`) _output_get))
          (`KismetArrayLibrary.Array_Add` (`local.UsedTile`) _output_get)
          (`KismetArrayLibrary.Array_RemoveItem` (`local.SectionTiles`) _output_get)
          (bind _returnvalue_2 (`|SpawnActorFromClass` "/Game/2019180031/Blueprints/Map/Building/BP_Building.BP_Building_C" (`KismetMathLibrary.MakeTransform` (`SceneComponent.RelativeLocation` _output_get)) "Undefined" "MultiplyWithRoot" null Floor null))
          (`BlueprintMapLibrary.Map_Add` (`self.Tile's Actor`) _output_get _returnvalue_2))))
    (:`then_2`
      ;[1 1 1] 부유 타일 배치
      (`KismetSystemLibrary.LogString` (`KismetStringLibrary.Conv_IntToString` _returnvalue))
      (while (< _returnvalue (+ `Spawn Count` FloatingTileCount))
        (bind _output_get_2 (set `local.TargetTile` (`KismetArrayLibrary.Array_Random` (`local.SectionTiles`))))
        (while (not (`KismetArrayLibrary.Array_Contains` (`local.UsedTile`) _output_get_2))
          (`KismetArrayLibrary.Array_Add` (`local.UsedTile`) _output_get_2)
          (bind _returnvalue_3 (`|SpawnActorFromClass` "/Game/2019180031/Blueprints/Map/FloatingTile/BP_FloatingTile.BP_FloatingTile_C" (`KismetMathLibrary.MakeTransform` (`SceneComponent.RelativeLocation` _output_get_2)) "Undefined" "MultiplyWithRoot" null `Movement Offset` null))
          (`BlueprintMapLibrary.Map_Add` (`self.Tile's Actor`) _output_get_2 _returnvalue_3))))))

(fn `UserConstructionScript`
  (locals (CurrentDistance :type Integer) (Temp :type Integer))
  (bind _currentdistance (`local.CurrentDistance`))
  (`|ExecutionSequence`
    (:`then_0`
      ;[1 1 1] 중앙 육각 타일 배치
      (bind _returnvalue (`AddComponent|NODE_AddStaticMeshComponent-4`))
      (bind _output_get (set `self.CurrentMiddleTile` _returnvalue))
      (`KismetArrayLibrary.Array_Add` (`ActorComponent.ComponentTags` _output_get) "Middle")
      (`KismetArrayLibrary.Array_Add` (`self.Tiles`) _output_get))
    (:`then_1`
      (for _index (range 6)
        (for _index_2 (range 1 4)
          (set `local.CurrentDistance` _index_2)
          (`|ExecutionSequence`
            (:`then_0`
              (bind _returnvalue_2 (`AddComponent|NODE_AddStaticMeshComponent-5` :`RelativeTransform` (`KismetMathLibrary.MakeTransform` (`self.CalculateRelativeLocation` _index (`local.CurrentDistance`))))) ; 각 60도 방면 static mesh
              (switch `int` (`local.CurrentDistance`)
                (:`1`
                  (bind _componenttags (`ActorComponent.ComponentTags` _returnvalue_2))
                  (`KismetArrayLibrary.Array_Add` _componenttags "Section3"))
                (:`2`
                  (`KismetArrayLibrary.Array_Add` _componenttags "Section2"))
                (:`3`
                  (`KismetArrayLibrary.Array_Add` _componenttags "Section1")))
              (`KismetArrayLibrary.Array_Add` (`self.Tiles`) _returnvalue_2))
            (:`then_1`
              (for _index_3 (range 2 (+ _currentdistance 1))
                (bind _relativelocation (`self.CalculateRelativeLocation` (+ _index 1) (`local.CurrentDistance`)))
                (bind _returnvalue_3 (`AddComponent|NODE_AddStaticMeshComponent-6` :`RelativeTransform` (`KismetMathLibrary.MakeTransform` (+ (* (/ (- (`self.CalculateRelativeLocation` _index (`local.CurrentDistance`)) _relativelocation) (`KismetMathLibrary.Conv_IntToDouble` _currentdistance)) (`KismetMathLibrary.Conv_IntToDouble` (+ _index_3 -1))) _relativelocation)))) ; 각 60도 방면 static mesh
                (switch `int` (`local.CurrentDistance`)
                  (:`1`
                    (bind _componenttags_2 (`ActorComponent.ComponentTags` _returnvalue_3))
                    (`KismetArrayLibrary.Array_Add` _componenttags_2 "Section3"))
                  (:`2`
                    (`KismetArrayLibrary.Array_Add` _componenttags_2 "Section2"))
                  (:`3`
                    (`KismetArrayLibrary.Array_Add` _componenttags_2 "Section1")))
                (`KismetArrayLibrary.Array_Add` (`self.Tiles`) _returnvalue_3)))))))))