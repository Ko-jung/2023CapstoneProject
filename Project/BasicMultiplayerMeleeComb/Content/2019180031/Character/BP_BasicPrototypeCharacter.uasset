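; Prototype player character with Enhanced Input movement, look and jump, plus damage reactions.
; BeginPlay adds the input mapping context and clamps camera pitch, while AnyDamage forwards to HealthComponent.
; DoStiffness scales the damaged montage's play rate by the inverse of stiffness time.
; DoDown switches to Flying, plays a knockdown montage with Motion Warping floating and landing targets along the given direction, then switches to Falling on blend out.
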(event `self.ReceiveBeginPlay`
  ;[1 1 1] Begin Play
  (bind _asplayer_controller (cast `PlayerController` (`self.GetController`)))
  (`EnhancedInputSubsystemInterface.AddMappingContext` (pcsubsystem `EnhancedInputLocalPlayerSubsystem` _asplayer_controller) "/Game/DeleteLater_ThirdPerson/Input/IMC_Default.IMC_Default" 0 (struct))
  (`self.SetCameraYawPitchAngle`))

(event `EnhancedInput|/Game/DeleteLater_ThirdPerson/Input/Actions/IA_Jump`
  (params (ActionValue :type Boolean) (ElapsedSeconds :type "Float (double-precision)") (TriggeredSeconds :type "Float (double-precision)") (InputAction :type "InputAction Object Reference" :default "/Game/DeleteLater_ThirdPerson/Input/Actions/IA_Jump.IA_Jump"))
  ;[1 1 1] IA_Jump
  (:`Started`
    (`self.Jump`))
  (:`Completed`
    (`self.StopJumping`)))

(event `EnhancedInput|/Game/DeleteLater_ThirdPerson/Input/Actions/IA_Move`
  (params (ActionValue :type "Vector2D Structure") (ElapsedSeconds :type "Float (double-precision)") (TriggeredSeconds :type "Float (double-precision)") (InputAction :type "InputAction Object Reference" :default "/Game/DeleteLater_ThirdPerson/Input/Actions/IA_Move.IA_Move"))
  ;[1 1 1] IA_Move
  (:`Triggered`
    (`|ExecutionSequence`
      (:`then_0`
        (`self.AddMovementInput` (`self.GetActorForwardVector`) ActionValue_Y) ; x축(전방) 이동
      )
      (:`then_1`
        (`self.AddMovementInput` (`self.GetActorRightVector`) ActionValue_X) ; y축(오른쪽)  이동
      ))))

(event `EnhancedInput|/Game/DeleteLater_ThirdPerson/Input/Actions/IA_Look`
  (params (ActionValue :type "Vector2D Structure") (ElapsedSeconds :type "Float (double-precision)") (TriggeredSeconds :type "Float (double-precision)") (InputAction :type "InputAction Object Reference" :default "/Game/DeleteLater_ThirdPerson/Input/Actions/IA_Look.IA_Look"))
  ;[1 1 1] IA_Look
  (:`Triggered`
    (`|ExecutionSequence`
      (:`then_0`
        (`self.AddControllerYawInput` ActionValue_X))
      (:`then_1`
        (`self.AddControllerPitchInput` ActionValue_Y)))))

(event `/Game/2019180031/BlueprintInterface/BPI_CanstiffnessAndDown.Do Stiffness`
  (params (StiffnessTime :type "Float (double-precision)"))
  (if (not (== StiffnessTime 0.0))
    (`|PlayMontage` (`self.Mesh`) "/Game/BMMCSystem/Animations/Combat/Montages/AM_Damaged.AM_Damaged" (/ 1.0 StiffnessTime))))

(event `self.ReceiveAnyDamage`
  (params (Damage :type "Float (single-precision)") (DamageType :type "DamageType Object Reference") (InstigatedBy :type "Controller Object Reference") (DamageCauser :type "Actor Object Reference"))
  (`/Game/2019180031/Components/HealthComponent/HealthComponent.AnyDamage` (`self.HealthComponent`) Damage))

(event `/Game/2019180031/BlueprintInterface/BPI_CanstiffnessAndDown.Do Down`
  (params (DownDirection :type "Vector Structure"))
  (bind _returnvalue (`self.K2_GetActorLocation`))
  (bind _motionwarping (`self.MotionWarping`))
  (`CharacterMovementComponent.SetMovementMode` (`self.CharacterMovement`) "MOVE_Flying" 0)
  (`|PlayMontage` (`self.Mesh`) "/Game/2019180031/Character/PrototypeAnimation/Damaged/AM_KnockedDown.AM_KnockedDown"
    (:`then`
      (`MotionWarpingComponent.AddOrUpdateWarpTargetFromLocationAndRotation` :`self` _motionwarping :`WarpTargetName` "FloatingPosition" :`TargetLocation` (+ _returnvalue (* DownDirection 50.0) (0.0 0.0 100.0)))
      (`MotionWarpingComponent.AddOrUpdateWarpTargetFromLocationAndRotation` :`self` _motionwarping :`WarpTargetName` "LandingPosition" :`TargetLocation` (+ _returnvalue (* DownDirection 100.0) (0.0 0.0 -100.0))))
    (:`OnBlendOut`
      (`CharacterMovementComponent.SetMovementMode` (`self.CharacterMovement`) "MOVE_Falling" 0))))

(fn `SetCameraYawPitchAngle`
  (bind _returnvalue (`GameplayStatics.GetPlayerCameraManager` 0))
  (set `PlayerCameraManager.ViewPitchMax` 60.0 _returnvalue)
  (set `PlayerCameraManager.ViewPitchMin` -50.0 _returnvalue))

(fn `UserConstructionScript`)