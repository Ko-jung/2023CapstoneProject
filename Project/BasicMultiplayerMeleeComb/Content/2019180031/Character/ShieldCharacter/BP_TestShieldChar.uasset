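; BP_TestShieldChar is a test player character with basic move, look and jump controls; it holds no shield logic.
; On BeginPlay it adds IMC_Default to the player controller's Enhanced Input subsystem.
; IA_Move drives movement along the forward and right vectors of the full control rotation, pitch included, and IA_Look feeds controller yaw and pitch.
; IA_Jump calls Jump, while StopJumping is left unconnected.
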(event `self.ReceiveBeginPlay`
  (bind `_as플레이어_컨트롤러` (cast `PlayerController` (`self.GetController`)))
  (`EnhancedInputSubsystemInterface.AddMappingContext` (pcsubsystem `EnhancedInputLocalPlayerSubsystem` `_as플레이어_컨트롤러`) "/Game/DeleteLater_ThirdPerson/Input/IMC_Default.IMC_Default" 0 (struct)))

(event `EnhancedInput|/Game/DeleteLater_ThirdPerson/Input/Actions/IA_Jump`
  (params (ActionValue :type Boolean) (ElapsedSeconds :type "Float (double-precision)") (TriggeredSeconds :type "Float (double-precision)") (InputAction :type "InputAction Object Reference" :default "/Game/DeleteLater_ThirdPerson/Input/Actions/IA_Jump.IA_Jump"))
  ;[1 1 1] IA_Jump
  (:`Triggered`
    (`self.Jump`)))

(event `EnhancedInput|/Game/DeleteLater_ThirdPerson/Input/Actions/IA_Move`
  (params (ActionValue :type "Vector2D Structure") (ElapsedSeconds :type "Float (double-precision)") (TriggeredSeconds :type "Float (double-precision)") (InputAction :type "InputAction Object Reference" :default "/Game/DeleteLater_ThirdPerson/Input/Actions/IA_Move.IA_Move"))
  (bind _returnvalue (`self.GetControlRotation`))
  ;[1 1 1] IA_Move
  (:`Triggered`
    (`|ExecutionSequence`
      (:`then_0`
        (`self.AddMovementInput` (`KismetMathLibrary.GetForwardVector` _returnvalue) ActionValue_Y) ; x축(전방) 이동
      )
      (:`then_1`
        (`self.AddMovementInput` (`KismetMathLibrary.GetRightVector` _returnvalue) ActionValue_X) ; y축(오른쪽)  이동
      ))))

(event `EnhancedInput|/Game/DeleteLater_ThirdPerson/Input/Actions/IA_Look`
  (params (ActionValue :type "Vector2D Structure") (ElapsedSeconds :type "Float (double-precision)") (TriggeredSeconds :type "Float (double-precision)") (InputAction :type "InputAction Object Reference" :default "/Game/DeleteLater_ThirdPerson/Input/Actions/IA_Look.IA_Look"))
  ;[1 1 1] IA_Look
  (:`Triggered`
    (`|ExecutionSequence`
      (:`then_0`
        (`self.AddControllerYawInput` ActionValue_X))
      (:`then_1`
        (`self.AddControllerPitchInput` ActionValue_Y)))))

(fn `UserConstructionScript`)