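; BP_PrototypeGameMode is the prototype game mode that runs a match countdown timer, started at BeginPlay with a hardcoded duration.
; FlowGameTimer loops through a Delay, pushing the remaining Timespan to each BP_BasicPrototypeCharacter's Player_GameTimerComponent for UI display, then subtracting the tick interval.
; The loop re-finds all characters each pass, runs at a fixed interval rather than on Tick, and has no stop at zero.
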(event `self.ReceiveBeginPlay`
  (`self.SetGameTimer` true 120.0))

(event `SetGameTimer`
  (params (TurnOnGameTime :type Boolean) (GameTimer :type "Float (double-precision)"))
  ;[1 1 1] 게임 타이머 시스템, 프로토타입에선 클라에서 작동 및 하드코딩 되어있음
  (set `self.TurnOnGameTime` TurnOnGameTime)
  (set `self.GameTimeSpan` (`KismetMathLibrary.FromSeconds` GameTimer))
  (`self.FlowGameTimer`))

(event `FlowGameTimer`
  ;[1 1 1] 게임 타이머 시스템, 프로토타입에선 클라에서 작동 및 하드코딩 되어있음
  (if (`self.TurnOnGameTime`)
    (bind _outactors (`GameplayStatics.GetAllActorsOfClass` "/Game/2019180031/Character/BP_BasicPrototypeCharacter.BP_BasicPrototypeCharacter_C"))
    (for _array_element _outactors
      (bind _returnvalue (`self.GetComponentByClass` _array_element "/Game/2019180031/Components/GameTimerComponent/Player_GameTimerComponent.Player_GameTimerComponent_C"))
      (`/Engine/EditorBlueprintResources/StandardMacros.IsValid` _returnvalue
        (:`Is Valid`
          (`/Game/2019180031/Components/GameTimerComponent/Player_GameTimerComponent.SetGameTimeUI` _returnvalue (`self.GameTimeSpan`)))))
    (`KismetSystemLibrary.Delay` (`self.GameTimerTickTime`))
    (set `self.GameTimeSpan` (- (`self.GameTimeSpan`) (`KismetMathLibrary.FromSeconds` (`self.GameTimerTickTime`))))
    (`self.FlowGameTimer`)))

(event `self.ReceiveTick`
  (params (DeltaSeconds :type "Float (single-precision)"))
  ;[1 1 1] 게임 타이머 시스템, 프로토타입에선 클라에서 작동 및 하드코딩 되어있음
)

(fn `UserConstructionScript`)