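; Jetpack character Blueprint that holds a fuel value and provides helper functions for fuel and velocity.
; GetJetPackFuel returns the current JetPackFuel value.
; ClampToMaxWalkSpeed caps a given velocity at the CharacterMovement MaxWalkSpeed by rescaling its normalized direction, and passes slower velocities through unchanged.
; The construction script is empty, and no graph here applies thrust or changes fuel.
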(fn `Clamp To Max Walk Speed`
  (params (`Now Velocity` :type "Vector Structure"))
  (returns (`Out Velocity` :type "Vector Structure"))
  (bind _maxwalkspeed (`CharacterMovementComponent.MaxWalkSpeed` (`self.CharacterMovement`)))
  (if (> (`KismetMathLibrary.VSize` `Now Velocity`) _maxwalkspeed)
    (return (* (`KismetMathLibrary.Normal` `Now Velocity`) _maxwalkspeed))
    (else
      (return `Now Velocity`))))

(fn `GetJetPackFuel`
  (returns (NewParam :type "Float (double-precision)"))
  (return (`self.JetPackFuel`)))

(fn `UserConstructionScript`)