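; BP_NavLink_AIJump is a smart nav link that makes AI characters jump to the link's destination when they reach it.
; On reaching the link, it stops the AI controller's movement and solves a custom-arc launch velocity toward the destination.
; It launches the character with that velocity, overriding XY and Z, and rotates it to face the horizontal launch direction.
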(event `self.ReceiveSmartLinkReached`
  (params (Agent :type "Actor Object Reference") (Destination :type "Vector Structure (by ref)"))
  (`/Engine/EditorBlueprintResources/StandardMacros.IsValid` Agent
    (:`Is Valid`
      (bind _ascharacter (cast `Character` Agent))
      (`Controller.StopMovement` (`AIBlueprintHelperLibrary.GetAIController` _ascharacter))
      (bind _outlaunchvelocity (`GameplayStatics.SuggestProjectileVelocity_CustomArc` (`self.K2_GetActorLocation` _ascharacter) Destination 0.0 0.35))
      (`Character.LaunchCharacter` _ascharacter _outlaunchvelocity true true)
      (`self.K2_SetActorRotation` _ascharacter (`KismetMathLibrary.Conv_VectorToRotator` (`KismetMathLibrary.MakeVector` (.x _outlaunchvelocity) (.y _outlaunchvelocity))) false))))

(fn `UserConstructionScript`)