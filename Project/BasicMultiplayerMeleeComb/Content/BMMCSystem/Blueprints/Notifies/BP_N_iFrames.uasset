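; Animation notify state that grants invincibility frames to the animated character for the notify window.
; On begin it fetches the owner's combat component through an interface message and sets its invincible state to true.
; On end it sends the same message with false, so the i-frame span matches the notify's placement in the animation.
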(fn `Received_NotifyBegin`
  (params (MeshComp :type "SkeletalMeshComponent Object Reference") (Animation :type "AnimSequenceBase Object Reference") (TotalDuration :type "Float (double-precision)"))
  (returns (ReturnValue :type Boolean))
  (bind _returnvalue (`ActorComponent.GetOwner` MeshComp))
  (`/Engine/EditorBlueprintResources/StandardMacros.IsValid` _returnvalue
    (:`Is Valid`
      (bind _component (message `/Game/BMMCSystem/Blueprints/Interfaces/BPI_Characters.GetCombatComp` _returnvalue))
      (message `/Game/BMMCSystem/Blueprints/Interfaces/BPI_Components_Combat.I_UpdateInvincibleState` _component true)
      (return true))))

(fn `Received_NotifyEnd`
  (params (MeshComp :type "SkeletalMeshComponent Object Reference") (Animation :type "AnimSequenceBase Object Reference"))
  (returns (ReturnValue :type Boolean))
  (bind _returnvalue (`ActorComponent.GetOwner` MeshComp))
  (`/Engine/EditorBlueprintResources/StandardMacros.IsValid` _returnvalue
    (:`Is Valid`
      (bind _component (message `/Game/BMMCSystem/Blueprints/Interfaces/BPI_Characters.GetCombatComp` _returnvalue))
      (message `/Game/BMMCSystem/Blueprints/Interfaces/BPI_Components_Combat.I_UpdateInvincibleState` _component false)
      (return true))))