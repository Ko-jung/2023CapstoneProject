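; BP_WeaponsBase is the base weapon actor, pairing a skeletal mesh with a weapons component.
; When ConstructWeapon is set, construction pulls the mesh from DT_Weapons by WeaponName and BeginPlay initializes the component as a pickable weapon; the component's OnEquipped event updates the name.
; Getters expose component, mesh, name, trace-ignore actors and aim, which uses the owning Character's shoot direction or falls back to the actor's forward vector.
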(event `self.ReceiveBeginPlay`
  (if (`self.ConstructWeapon`)
    (message `/Game/BMMCSystem/Blueprints/Interfaces/ActorComponents/BPI_Components_Weapons.I Init Pickable Weapon` (`self.BPC_Weapons`) (`self.WeaponName`))))

(event `self.BPC_Weapons.OnEquipped`
  (params (Name :type Name))
  (set `self.WeaponName` Name))

(fn `GetIgnoreActorsForShootingTrace`
  (returns (Actors :type "Array of Actor Object Reference"))
  (return (`|MakeArray` self (`self.GetOwner`) :!type "Actor Object Reference")))

(fn `GetProjectileComponent`
  (returns (Comp :type "ActorComponent Object Reference"))
  (return null))

(fn `GetWeaponAimDirection`
  (returns (Direction :type "Vector Structure") (Location :type "Vector Structure"))
  (bind _returnvalue (`self.GetOwner`))
  (`/Engine/EditorBlueprintResources/StandardMacros.IsValid` _returnvalue
    (:`Is Valid`
      (bind _ascharacter (cast `Character` _returnvalue)
        (:`then`
          (bind (_direction _location) (`/Game/BMMCSystem/Blueprints/Utilities/BFL_ComponentUtilities.GetShootDirection` _ascharacter))
          (return _direction _location))
        (:`CastFailed`
          _)))
    (:`Is Not Valid`
      _))
  (return (`self.GetActorForwardVector`) (`self.K2_GetActorLocation`)))

(fn `GetWeaponComponent`
  (returns (Component :type "ActorComponent Object Reference"))
  (return (`self.BPC_Weapons`)))

(fn `GetWeaponMesh`
  (returns (Mesh :type "SkeletalMeshComponent Object Reference"))
  (return (`self.SkeletalMesh`)))

(fn `GetWeaponName`
  (returns (Name :type Name))
  (return (`self.WeaponName`)))

(fn `SetMeshFromDataTable`
  (`/Engine/EditorBlueprintResources/StandardMacros.IsValid` (`self.BPC_Weapons`)
    (:`Is Valid`
      (if (`self.ConstructWeapon`)
        (bind _returnvalue (`|GetDataTableRow` "/Game/BMMCSystem/Blueprints/DataTables/DT_Weapons.DT_Weapons" (`self.WeaponName`))
          (:`then`
            (`SkinnedMeshComponent.SetSkinnedAssetAndUpdate` (`self.SkeletalMesh`) (`.Mesh_5_E5EB27FB4390E2F7B95F589D86B70262` (break `/Game/BMMCSystem/Blueprints/Structures/S_WeaponConstruction` _returnvalue)) true)))))))

(fn `UserConstructionScript`
  (`self.SetMeshFromDataTable`))