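; BP_WeaponsBase_Ranged is the base Blueprint for ranged weapons in the BMMC system.
; Shoot and reload interface calls are forwarded as messages to its BPC_ProjectSpawner component, with reload passing the weapon's owner.
; The spawner's fired event plays a fire montage on the owner, and its ammo-changed event refreshes the owner's ranged UI.
; A getter exposes the spawner component, while the equipped and reloaded events are empty.
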(event `self.ReceiveBeginPlay`
  (`parent.ReceiveBeginPlay`))

(event `/Game/BMMCSystem/Blueprints/Interfaces/BPI_Weapons.I_RangedWeapon_Shoot`
  (message `/Game/BMMCSystem/Blueprints/Interfaces/ActorComponents/BPI_Components_Projectiles.I_Shoot` (`self.BPC_ProjectSpawner`)))

(event `/Game/BMMCSystem/Blueprints/Interfaces/BPI_Weapons.I_RangedWeaponReload`
  (message `/Game/BMMCSystem/Blueprints/Interfaces/ActorComponents/BPI_Components_Projectiles.I_Reload` (`self.BPC_ProjectSpawner`) (`self.GetOwner`) 1 true))

(event `self.BPC_Weapons.OnEquipped`
  (params (Name :type Name)))

(event `self.BPC_ProjectSpawner.OnFired`
  (`/Game/BMMCSystem/Blueprints/Components/BPC_ProjectileSpawner.PlayFireMontage` (`self.BPC_ProjectSpawner`) (`self.GetOwner`)))

(event `self.BPC_ProjectSpawner.OnAmmoChanged`
  (`/Game/BMMCSystem/Blueprints/Utilities/BFL_ComponentUtilities.Update Owner Ranged UI` (`self.GetOwner`)))

(event `self.BPC_ProjectSpawner.OnReloaded`)

(fn `GetProjectileComponent`
  (returns (Comp :type "ActorComponent Object Reference"))
  (return (`self.BPC_ProjectSpawner`)))

(fn `UserConstructionScript`
  (`parent.UserConstructionScript`))