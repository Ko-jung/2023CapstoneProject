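; Main game mode that spawns skill actors and selected characters for the match.
; SpawnSkillActor switches on the skill type to spawn boomerang, mine, shield, tornado or electric actors, passing team and, where needed, caster and aim data.
; SpawnCharactersUsingSelectInfo spawns a given character class at a location, stores it in an array and prints the class name.
; Tick only calls the parent, and BeginPlay is unused.
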(event `self.SpawnSkillActor`
  (params (SkillActor :type "ESkillActor Enum" :default "BP_NULL") (SpawnLocation :type "Vector Structure") (ForwardVec :type "Vector Structure") (Spawner :type "SkyscraperCharacter Object Reference") (Team :type Name))
  (switch `ESkillActor` SkillActor
    (:`BP_BoomerangGrab`
      (`|SpawnActorFromClass` "/Game/2019180016/Blueprint/SkillBP/Boomerang_Grab.Boomerang_Grab_C" (`KismetMathLibrary.MakeTransform` SpawnLocation) "Undefined" "MultiplyWithRoot" null SpawnLocation ForwardVec Spawner Team null))
    (:`BP_BoomerangCenter`
      (`|SpawnActorFromClass` "/Game/2019180016/Blueprint/SkillBP/Boomerang_GrabCenter.Boomerang_GrabCenter_C" (`KismetMathLibrary.MakeTransform` SpawnLocation) "Undefined" "MultiplyWithRoot" null ForwardVec Spawner Team null))
    (:`BP_DetectorMine`
      (`|SpawnActorFromClass` "/Game/2019180016/Blueprint/SkillBP/BP_DetectorMine.BP_DetectorMine_C" (`KismetMathLibrary.MakeTransform` SpawnLocation) "Undefined" "MultiplyWithRoot" null Team null))
    (:`BP_ShieldSphere`
      (`|SpawnActorFromClass` "/Game/2019180016/Blueprint/SkillBP/BP_ShieldSphere.BP_ShieldSphere_C" (`KismetMathLibrary.MakeTransform` SpawnLocation) "Undefined" "MultiplyWithRoot" null Team null))
    (:`BP_ShieldSphereThrow`
      (`|SpawnActorFromClass` "/Game/2019180016/Blueprint/SkillBP/BP_ShieldSphereThrow.BP_ShieldSphereThrow_C" (`KismetMathLibrary.MakeTransform` SpawnLocation) "Undefined" "MultiplyWithRoot" null Spawner Team null))
    (:`BP_WindTornado`
      (`|SpawnActorFromClass` "/Game/2019180016/Blueprint/SkillBP/BP_WindTornado.BP_WindTornado_C" (`KismetMathLibrary.MakeTransform` SpawnLocation) "Undefined" "MultiplyWithRoot" null Team null))
    (:`BP_ElectSphereBoom`
      (`|SpawnActorFromClass` "/Game/2019180016/Blueprint/SkillBP/Elect_SphereBoom.Elect_SphereBoom_C" (`KismetMathLibrary.MakeTransform` SpawnLocation) "Undefined" "MultiplyWithRoot" null Spawner Team null))
    (:`BP_ElectTrap`
      (`|SpawnActorFromClass` "/Game/2019180016/Blueprint/SkillBP/Elect_Trab.Elect_Trab_C" (`KismetMathLibrary.MakeTransform` SpawnLocation) "Undefined" "MultiplyWithRoot" null Team null))))

(event `self.SpawnCharactersUsingSelectInfo`
  (params (Class :type "SkyscraperCharacter Class Reference") (location :type "Vector Structure"))
  (bind _returnvalue (`|SpawnActorFromClass` Class (`KismetMathLibrary.MakeTransform` location) "Undefined" "MultiplyWithRoot" null null))
  (`KismetArrayLibrary.Array_Add` (`self.NewVar`) _returnvalue)
  (`KismetSystemLibrary.PrintString` (`KismetSystemLibrary.GetClassDisplayName` Class)))

(event `self.ReceiveTick`
  (params (DeltaSeconds :type "Float (single-precision)"))
  (`parent.ReceiveTick` DeltaSeconds))

(fn `UserConstructionScript`)