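; BP_NonCppController is a Blueprint player controller that drives first- or third-person style movement and look through Enhanced Input.
; On BeginPlay it adds the IMC_Default mapping context.
; IA_Move feeds movement input to the controlled pawn along its root component's forward (X) and right (Y) vectors.
; IA_Look feeds the controller's yaw (X) and pitch (Y) input directly.
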(event `self.ReceiveBeginPlay`
  (`EnhancedInputSubsystemInterface.AddMappingContext` (subsystem `EnhancedInputLocalPlayerSubsystem`) "/Game/DeleteLater_ThirdPerson/Input/IMC_Default.IMC_Default" 0 (struct)))

(event `EnhancedInput|/Game/DeleteLater_ThirdPerson/Input/Actions/IA_Move`
  (params (ActionValue :type "Vector2D Structure") (ElapsedSeconds :type "Float (double-precision)") (TriggeredSeconds :type "Float (double-precision)") (InputAction :type "InputAction Object Reference" :default "/Game/DeleteLater_ThirdPerson/Input/Actions/IA_Move.IA_Move"))
  (bind _returnvalue (`self.K2_GetPawn`))
  (bind _rootcomponent (`Actor.RootComponent` _returnvalue))
  (:`Triggered`
    (`Pawn.AddMovementInput` _returnvalue (`SceneComponent.GetForwardVector` _rootcomponent) ActionValue_X false)
    (`Pawn.AddMovementInput` _returnvalue (`SceneComponent.GetRightVector` _rootcomponent) ActionValue_Y false)))

(event `EnhancedInput|/Game/DeleteLater_ThirdPerson/Input/Actions/IA_Look`
  (params (ActionValue :type "Vector2D Structure") (ElapsedSeconds :type "Float (double-precision)") (TriggeredSeconds :type "Float (double-precision)") (InputAction :type "InputAction Object Reference" :default "/Game/DeleteLater_ThirdPerson/Input/Actions/IA_Look.IA_Look"))
  (:`Triggered`
    (`self.AddPitchInput` ActionValue_Y)
    (`self.AddYawInput` ActionValue_X)))

(fn `UserConstructionScript`)