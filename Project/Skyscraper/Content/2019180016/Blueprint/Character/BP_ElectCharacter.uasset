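; Electric character Blueprint that casts two skills from key presses: a sphere boom on Z and a trap on Q.
; Each key calls an OnServer event that forwards to an OnClient event to spawn the actor, passing the first actor tag as team.
; The sphere boom spawns at the character with it as caster, while the flattened trap spawns ahead and is lobbed by impulse.
; An authority-switched copy of the trap spawn is left unconnected.
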(event `Key|Z`
  (params (Key :type "Key Structure"))
  (:`Pressed`
    (`self.Spawn Elect Sphere Boom On Server` (`self.K2_GetActorLocation`) self (`|GetArrayItem` (`self.Tags`)))))

(event `Spawn Elect Sphere Boom On Server`
  (params (`Spawn Transform Location` :type "Vector Structure") (SkillCaster :type "Character Object Reference") (WhoSpawnTeam :type Name))
  (`self.Spawn Elect Sphere Boom On Client` `Spawn Transform Location` SkillCaster WhoSpawnTeam))

(event `Key|Q`
  (params (Key :type "Key Structure"))
  (:`Pressed`
    (`self.Spawn Elect Trab On Server` (+ (`self.K2_GetActorLocation`) (* (`self.GetActorForwardVector`) 100.0)) (`|GetArrayItem` (`self.Tags`)))))

(event `Spawn Elect Sphere Boom On Client`
  (params (`Spawn Transform Location` :type "Vector Structure") (SkillCaster :type "Character Object Reference") (WhoSpawnTeam :type Name))
  (`|SpawnActorFromClass` "/Game/2019180016/Blueprint/SkillBP/Elect_SphereBoom.Elect_SphereBoom_C" (`KismetMathLibrary.MakeTransform` `Spawn Transform Location`) "Undefined" "MultiplyWithRoot" null SkillCaster WhoSpawnTeam null))

(event `Spawn Elect Trab On Server`
  (params (`Spawn Transform Location` :type "Vector Structure") (WhoSpawnTeam :type Name))
  (`self.Spawn Elect Trab On Client` `Spawn Transform Location` WhoSpawnTeam))

(event `Spawn Elect Trab On Client`
  (params (`Spawn Transform Location` :type "Vector Structure") (WhoSpawnTeam :type Name))
  (bind _returnvalue (`|SpawnActorFromClass` "/Game/2019180016/Blueprint/SkillBP/Elect_Trab.Elect_Trab_C" (`KismetMathLibrary.MakeTransform` `Spawn Transform Location` (struct) (1.0 1.0 0.2)) "Undefined" "OverrideRootScale" null WhoSpawnTeam null))
  (`PrimitiveComponent.AddImpulse` (`/Game/2019180016/Blueprint/SkillBP/Elect_Trab.StaticMesh` _returnvalue) (* (+ (`self.GetActorForwardVector`) (0.0 0.0 1.0)) 500.0) "None" true)
  (`KismetSystemLibrary.PrintString` "ElectGrabSpawning at character"))

(fn `UserConstructionScript`
  (`parent.UserConstructionScript`))