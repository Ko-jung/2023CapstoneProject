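; Playable assassin character Blueprint whose Q skill grants timed stealth.
; Q plays skill montages on the body and boost meshes, sends the montage status, then enables stealth and calls BuffUsingSkill on completion.
; StealthOnOff swaps both meshes between materials cached at BeginPlay and preset opacity materials.
; Tick counts down the stealth timer with debug prints, playing the boost montage's End section on expiry and restoring visibility when it completes.
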(event `self.ReceiveBeginPlay`
  (for _array_element (`MeshComponent.GetMaterials` (`self.Mesh`))
    (`KismetArrayLibrary.Array_Add` (`self.Material`) _array_element))
  (set `self.BoostMaterial` (`PrimitiveComponent.GetMaterial` (`self.BoostMesh`) 0)))

(event `self.ReceiveTick`
  (params (DeltaSeconds :type "Float (single-precision)"))
  (if (`self.IsStealth`)
    (bind _output_get (set `self.StealthTimer` (- (`self.StealthTimer`) DeltaSeconds)))
    (`KismetSystemLibrary.PrintString` (`KismetStringLibrary.Conv_DoubleToString` _output_get) true true (struct :`G` 0.66 :`B` 1.0 :`A` 1.0) 0.01)
    (if (<= _output_get 0.0)
      (`|PlayMontage` (`self.BoostMesh`) "/Game/2019180016/Montage/Assasin/AM_Assasin_Boost_Skill1.AM_Assasin_Boost_Skill1" 1.0 0.0 "End"
        (:`OnCompleted`
          (`self.StealthOnOff` false)
          (`KismetSystemLibrary.PrintString` "StealthOff"))))))

(event `Key|Q`
  (params (Key :type "Key Structure"))
  (:`Pressed`
    (`|PlayMontage` (`self.Mesh`) "/Game/2019180016/Montage/Assasin/AM_Assasin_Skill1.AM_Assasin_Skill1"
      (:`then`
        (`|PlayMontage` (`self.BoostMesh`) "/Game/2019180016/Montage/Assasin/AM_Assasin_Boost_Skill1.AM_Assasin_Boost_Skill1"
          (:`then`
            (`self.SendAnimMontageStatus` "ECAM_CommonSkill"))))
      (:`OnCompleted`
        (`self.StealthOnOff` true)))))

(fn `StealthOnOff`
  (params (On :type Boolean))
  (bind _boostmesh (`self.BoostMesh`))
  (if On
    (set `self.IsStealth` true)
    (set `self.StealthTimer` 10.0)
    (`self.BuffUsingSkill`)
    (`PrimitiveComponent.SetMaterial` _boostmesh 0 "/Game/2019180016/Blueprint/Material/Assasin/Opercity_Material_boost.Opercity_Material_boost")
    (for (_array_element _array_index) (`self.OpacityMaterial`)
      (`PrimitiveComponent.SetMaterial` (`self.Mesh`) _array_index _array_element))
    (else
      (set `self.IsStealth` false)
      (set `self.StealthTimer` 0.0)
      (`PrimitiveComponent.SetMaterial` _boostmesh 0 (`self.BoostMaterial`))
      (for (_array_element_2 _array_index_2) (`self.Material`)
        (`PrimitiveComponent.SetMaterial` (`self.Mesh`) _array_index_2 _array_element_2)))))

(fn `UserConstructionScript`)