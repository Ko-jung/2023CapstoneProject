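; Playable boomerang character with a common skill on Q and a special skill on Z, each throwing a different boomerang actor.
; Key presses play paired body and BoostMesh montages and send montage status.
; ActiveSkill hides a held boomerang, spawns its team-tagged projectile and sends a spawn packet, though the special's packet carries zero vectors.
; CatchBoomerang1 plays the common skill's End section; PlaySkillMontage replays Start montages without sending.
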(event `Key|Z`
  (params (Key :type "Key Structure"))
  (:`Pressed`
    (`|PlayMontage` (`self.Mesh`) "/Game/2019180016/Montage/Boomerang/AM_Boomerang_Skill2.AM_Boomerang_Skill2" 1.0 0.0 "Start"
      (:`then`
        (`|PlayMontage` (`self.BoostMesh`) "/Game/2019180016/Montage/Boomerang/AM_Boomerang_Boost_Skill2.AM_Boomerang_Boost_Skill2" 1.0 0.0 "Start"
          (:`then`
            (`self.SendAnimMontageStatus` "ECAM_SpecialSkill")))))))

(event `self.ReceiveBeginPlay`
  (`parent.ReceiveBeginPlay`))

(event `Key|Q`
  (params (Key :type "Key Structure"))
  (:`Pressed`
    (`|PlayMontage` (`self.Mesh`) "/Game/2019180016/Montage/Boomerang/AM_Boomerang_Skill1.AM_Boomerang_Skill1" 1.0 0.0 "Start"
      (:`then`
        (`|PlayMontage` (`self.BoostMesh`) "/Game/2019180016/Montage/Boomerang/AM_Boomerang_Boost_Skill1.AM_Boomerang_Boost_Skill1" 1.0 0.0 "Start"
          (:`then`
            (`self.SendAnimMontageStatus` "ECAM_CommonSkill")))))))

(event `self.SpawnBoomerangActor`
  (params (IsSpecialSkill :type Boolean))
  (if IsSpecialSkill
    _))

(event `self.ActiveSkill`
  (params (IsSpecialSkill :type Boolean))
  (if IsSpecialSkill
    (`self.SpawnBoomerang2`)
    (else
      (`self.SpawnBoomerang1`) ; Temp
      (`KismetSystemLibrary.PrintString` (`KismetStringLibrary.Concat_StrStr` (`KismetSystemLibrary.GetDisplayName` self) "Spawn Common Skill")))))

(event `CatchBoomerang1`
  (`|PlayMontage` (`self.Mesh`) "/Game/2019180016/Montage/Boomerang/AM_Boomerang_Skill1.AM_Boomerang_Skill1" 1.0 0.0 "End"
    (:`then`
      (`|PlayMontage` (`self.BoostMesh`) "/Game/2019180016/Montage/Boomerang/AM_Boomerang_Boost_Skill1.AM_Boomerang_Boost_Skill1" 1.0 0.0 "End"))))

(event `self.PlaySkillMontage`
  (params (IsSpecialSkill :type Boolean))
  (if IsSpecialSkill
    (`|PlayMontage` (`self.Mesh`) "/Game/2019180016/Montage/Boomerang/AM_Boomerang_Skill2.AM_Boomerang_Skill2" 1.0 0.0 "Start"
      (:`then`
        (`|PlayMontage` (`self.BoostMesh`) "/Game/2019180016/Montage/Boomerang/AM_Boomerang_Boost_Skill2.AM_Boomerang_Boost_Skill2" 1.0 0.0 "Start")))
    (else
      (`|PlayMontage` (`self.Mesh`) "/Game/2019180016/Montage/Boomerang/AM_Boomerang_Skill1.AM_Boomerang_Skill1" 1.0 0.0 "Start"
        (:`then`
          (`|PlayMontage` (`self.BoostMesh`) "/Game/2019180016/Montage/Boomerang/AM_Boomerang_Boost_Skill1.AM_Boomerang_Boost_Skill1" 1.0 0.0 "Start"))))))

(fn `SpawnBoomerang1`
  (bind _returnvalue (`self.K2_GetActorLocation`))
  (bind _returnvalue_2 (* (`self.GetActorForwardVector`) 1000.0))
  (`SceneComponent.SetVisibility` (`self.Boomerang_L`) false false)
  (`|SpawnActorFromClass` "/Game/2019180016/Blueprint/SkillBP/Boomerang_Grab.Boomerang_Grab_C" (`KismetMathLibrary.MakeTransform` _returnvalue) "Undefined" "MultiplyWithRoot" null _returnvalue _returnvalue_2 self (`|GetArrayItem` (`self.Tags`)) null)
  (`self.SendSkillActorSpawnPacket` "BP_BoomerangGrab" _returnvalue _returnvalue_2))

(fn `SpawnBoomerang2`
  (`SceneComponent.SetVisibility` (`self.Boomerang_R`) false false)
  (`|SpawnActorFromClass` "/Game/2019180016/Blueprint/SkillBP/Boomerang_GrabCenter.Boomerang_GrabCenter_C" (`KismetMathLibrary.MakeTransform` (`self.K2_GetActorLocation`)) "Undefined" "MultiplyWithRoot" null (`self.GetActorForwardVector`) self (`|GetArrayItem` (`self.Tags`)) null)
  (`self.SendSkillActorSpawnPacket` "BP_BoomerangGrab"))

(fn `UserConstructionScript`)