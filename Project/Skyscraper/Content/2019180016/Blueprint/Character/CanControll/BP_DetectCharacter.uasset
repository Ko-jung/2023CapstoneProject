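; BP_DetectCharacter is a controllable character that previews and places detector mines tagged with its team, taken from its first actor tag.
; Q toggles a preview mine, which Tick moves to the follow camera's forward trace hit.
; If that misses, a downward trace from a point ahead along the camera's horizontal direction finds the surface.
; Left click spawns a mine there with IsSetting enabled and destroys the preview.
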(event `Key|Q`
  (params (Key :type "Key Structure"))
  (:`Pressed`
    (if (`self.ViewDectorMine`)
      (set `self.ViewDectorMine` false)
      (`self.K2_DestroyActor` (`self.DetectorMine`))
      (else
        (set `self.ViewDectorMine` true)
        (bind _returnvalue (`|SpawnActorFromClass` "/Game/2019180016/Blueprint/SkillBP/BP_DetectorMine.BP_DetectorMine_C" (`KismetMathLibrary.MakeTransform` (0.0 0.0 0.0) (struct) (5.0 5.0 5.0)) "Undefined" "MultiplyWithRoot" null (`|GetArrayItem` (`self.Tags`)) null))
        (set `self.DetectorMine` _returnvalue)
        (`KismetSystemLibrary.PrintString` "Spawn mine")))))

(event `self.ReceiveTick`
  (params (DeltaSeconds :type "Float (single-precision)"))
  (bind _followcamera (`self.FollowCamera`))
  (bind _followcamera_2 (`self.FollowCamera`))
  (bind (_returnvalue_x _returnvalue_y) (`KismetMathLibrary.BreakVector` (`SceneComponent.GetForwardVector` _followcamera_2)))
  (bind _returnvalue (`SceneComponent.K2_GetComponentLocation` _followcamera))
  (bind _returnvalue_2 (+ (`SceneComponent.K2_GetComponentLocation` _followcamera_2) (* (`KismetMathLibrary.MakeVector` _returnvalue_x _returnvalue_y) 1000.0)))
  (`parent.ReceiveTick` DeltaSeconds)
  (if (`self.ViewDectorMine`)
    (bind (_outhit _returnvalue_3) (`KismetSystemLibrary.LineTraceSingle` _returnvalue (+ _returnvalue (* (`SceneComponent.GetForwardVector` _followcamera) 1000.0)) "TraceTypeQuery1"))
    (if _returnvalue_3
      (`self.K2_SetActorLocation` (`self.DetectorMine`) (`.Location` (`GameplayStatics.BreakHitResult` _outhit)) false false)
      (else
        (bind (_outhit_2 _returnvalue_4) (`KismetSystemLibrary.LineTraceSingle` _returnvalue_2 (- _returnvalue_2 (0.0 0.0 1000.0)) "TraceTypeQuery1"))
        (if _returnvalue_4
          (`self.K2_SetActorLocation` (`self.DetectorMine`) (`.Location` (`GameplayStatics.BreakHitResult` _outhit_2)) false false))))))

(event `Key|LeftMouseButton`
  (params (Key :type "Key Structure"))
  (bind _detectormine (`self.DetectorMine`))
  (:`Pressed`
    (if (`self.ViewDectorMine`)
      (bind _returnvalue (`|SpawnActorFromClass` "/Game/2019180016/Blueprint/SkillBP/BP_DetectorMine.BP_DetectorMine_C" (`KismetMathLibrary.MakeTransform` (`self.K2_GetActorLocation` _detectormine)) "Undefined" "MultiplyWithRoot" null (`|GetArrayItem` (`self.Tags`)) null))
      (set `/Game/2019180016/Blueprint/SkillBP/BP_DetectorMine.IsSetting` true _returnvalue)
      (`self.K2_DestroyActor` _detectormine)
      (set `self.ViewDectorMine` false))))

(fn `UserConstructionScript`)