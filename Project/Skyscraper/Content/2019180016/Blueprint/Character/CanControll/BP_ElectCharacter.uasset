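; Playable electric character with two skills: a thrown trap as the common skill and a sphere boom as the special.
; Q, Z or PlaySkillMontage play the skill montages and send their status over the network.
; ActiveSkill sends a spawn packet for the trap, which SkillActorSpawnUsingPacket spawns and launches by impulse, but spawns the boom directly at the character.
; Tick replays the stun hit montage every frame while IsUnableAct is set.
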(event `Test`
  (`SkeletalMeshComponent.SetUpdateClothInEditor` (`self.Mesh`) true))

(event `self.ReceiveBeginPlay`
  (`parent.ReceiveBeginPlay`))

(event `self.ReceiveTick`
  (params (DeltaSeconds :type "Float (single-precision)"))
  (if (`self.IsUnableAct`)
    (`|PlayMontage` (`self.Mesh`) "/Game/2019180031/MainGame/Animation/Electric/Combat/Damaged/AM_Electric_Hit.AM_Electric_Hit" 1.0 0.16 "Stun_Bwd")))

(event `Key|Q`
  (params (Key :type "Key Structure"))
  (:`Pressed`
    (`|PlayMontage` (`self.Mesh`) "/Game/2019180016/Montage/Electric/AM_Electric_Skill1.AM_Electric_Skill1" :!label _label
      (:`then`
        (`self.SendAnimMontageStatus` "ECAM_CommonSkill")))))

(event `self.ActiveSkill`
  (params (IsSpecialSkill :type Boolean))
  (if IsSpecialSkill
    (`self.SpawnBoom`)
    (else
      (`self.SendSkillActorSpawnPacket` self "BP_ElectTrap" (+ (`SceneComponent.GetSocketLocation` (`self.Mesh`) "Bip001-L-Hand") (0.0 0.0 5.0)) (`self.GetActorForwardVector`)))))

(event `self.PlaySkillMontage`
  (params (IsSpecialSkill :type Boolean) (SectionNum :type Byte))
  (if IsSpecialSkill
    (`|PlayMontage` (`self.Mesh`) "/Game/2019180016/Montage/Electric/AM_Electric_Skill2.AM_Electric_Skill2" :!label _label_2
      (:`then`
        (`self.SendAnimMontageStatus` "ECAM_SpecialSkill")))
    (else
      (goto _label))))

(event `Key|Z`
  (params (Key :type "Key Structure"))
  (:`Pressed`
    (goto _label_2)))

(fn `SkillActorSpawnUsingPacket`
  (params (IsSpecialSkill :type Boolean) (SpawnLocation :type "Vector Structure") (ForwardVector :type "Vector Structure"))
  (returns (NewActor :type "Actor Object Reference"))
  (if (not IsSpecialSkill)
    (bind _skillactor (`self.SpawnTrap` SpawnLocation ForwardVector))
    (return _skillactor)))

(fn `SpawnBoom`
  (`|SpawnActorFromClass` "/Game/2019180016/Blueprint/SkillBP/Elect_SphereBoom.Elect_SphereBoom_C" (`KismetMathLibrary.MakeTransform` (`self.K2_GetActorLocation`)) "Undefined" "MultiplyWithRoot" null self (`|GetArrayItem` (`self.Tags`)) null))

(fn `SpawnTrap`
  (params (Location :type "Vector Structure") (Forward :type "Vector Structure"))
  (returns (SkillActor :type "Actor Object Reference"))
  (bind _returnvalue (`|SpawnActorFromClass` "/Game/2019180016/Blueprint/SkillBP/Elect_Trab.Elect_Trab_C" (`KismetMathLibrary.MakeTransform` Location) "Undefined" "OverrideRootScale" null (`|GetArrayItem` (`self.Tags`)) null))
  (`PrimitiveComponent.AddImpulse` (`/Game/2019180016/Blueprint/SkillBP/Elect_Trab.StaticMesh` _returnvalue) (* (+ Forward (0.0 0.0 1.0)) 500.0) "None" true)
  (`KismetSystemLibrary.PrintString` "ElectGrabSpawning at character")
  (return _returnvalue))

(fn `UserConstructionScript`)