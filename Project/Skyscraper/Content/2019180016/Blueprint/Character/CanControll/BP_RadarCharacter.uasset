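; Playable Radar character Blueprint with two skills: a thrown detector mine (Q) and an EMP (Z).
; Each key plays its montage and sends the animation status; ActiveSkill then either spawns the EMP directly or sends a mine spawn packet from the left hand.
; SkillActorSpawnUsingPacket spawns the mine with an impulse, and both skill actors take their team from the first actor tag.
; An older camera-trace mine placement preview remains unwired.
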(event `self.ReceiveTick`
  (params (DeltaSeconds :type "Float (single-precision)"))
  (`parent.ReceiveTick` DeltaSeconds))

(event `self.SetCustomDepth`
  (params (On :type Boolean))
  (`PrimitiveComponent.SetRenderCustomDepth` (`self.Mesh`) On))

(event `Key|LeftMouseButton`
  (params (Key :type "Key Structure")))

(event `self.PlaySkillMontage`
  (params (IsSpecialSkill :type Boolean) (SectionNum :type Byte))
  (if IsSpecialSkill
    (`|PlayMontage` (`self.Mesh`) "/Game/2019180016/Montage/Radar/AM_Radar_Skill2.AM_Radar_Skill2" :!label _label
      (:`then`
        (`self.SendAnimMontageStatus` "ECAM_SpecialSkill")))
    (else
      (`|PlayMontage` (`self.Mesh`) "/Game/2019180016/Montage/Radar/AM_Radar_Skill1.AM_Radar_Skill1" :!label _label_2
        (:`then`
          (`self.SendAnimMontageStatus` "ECAM_CommonSkill"))))))

(event `Key|Q`
  (params (Key :type "Key Structure"))
  (:`Pressed`
    (goto _label_2)))

(event `Key|Z`
  (params (Key :type "Key Structure"))
  (:`Pressed`
    (goto _label)))

(event `self.ActiveSkill`
  (params (IsSpecialSkill :type Boolean))
  (if IsSpecialSkill
    (`self.ActivateEMP`)
    (else
      (`self.SendSkillActorSpawnPacket` self "BP_DetectorMine" (+ (`SceneComponent.GetSocketLocation` (`self.Mesh`) "Bip001-L-Hand") (0.0 0.0 5.0)) (`self.GetActorForwardVector`)))))

(fn `ActivateEMP`
  (`|SpawnActorFromClass` "/Game/2019180016/Blueprint/SkillBP/BP_RadarEMP.BP_RadarEMP_C" (`KismetMathLibrary.MakeTransform` (`self.K2_GetActorLocation`)) "Undefined" "MultiplyWithRoot" null self (`|GetArrayItem` (`self.Tags`)) null))

(fn `SkillActorSpawnUsingPacket`
  (params (IsSpecialSkill :type Boolean) (SpawnLocation :type "Vector Structure") (ForwardVector :type "Vector Structure"))
  (returns (NewActor :type "Actor Object Reference"))
  (if (not IsSpecialSkill)
    (bind _actor (`self.SpawnRadar` SpawnLocation ForwardVector))
    (return _actor)))

(fn `SpawnRadar`
  (params (Location :type "Vector Structure") (Forward :type "Vector Structure"))
  (returns (Actor :type "Actor Object Reference"))
  (bind _returnvalue (`|SpawnActorFromClass` "/Game/2019180016/Blueprint/SkillBP/BP_DetectorMine.BP_DetectorMine_C" (`KismetMathLibrary.MakeTransform` Location) "Undefined" "MultiplyWithRoot" self (`|GetArrayItem` (`self.Tags`)) null))
  (`PrimitiveComponent.AddImpulse` (`/Game/2019180016/Blueprint/SkillBP/BP_DetectorMine.StaticMesh` _returnvalue) (* (+ Forward (0.0 0.0 1.0)) 500.0) "None" true)
  (return _returnvalue))

(fn `UserConstructionScript`)