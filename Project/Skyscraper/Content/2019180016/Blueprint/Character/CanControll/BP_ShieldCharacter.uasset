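; Playable shield character with a toggled shield skill and a special shield-sphere skill.
; Q and Z play paired body and boost-mesh montages and send montage status; PlaySkillMontage plays them from an event call.
; ActiveSkill spawns an attached BP_Shield or a team-tagged BP_ShieldSphere; the thrown-sphere code is unconnected.
; Toggling Q off destroys the shield, saving its health for the next spawn.
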(event `self.ReceiveBeginPlay`)

(event `self.SetCustomDepth`
  (params (On :type Boolean))
  (`PrimitiveComponent.SetRenderCustomDepth` (`self.Mesh`) On))

(event `self.ReceiveTick`
  (params (DeltaSeconds :type "Float (single-precision)"))
  (`parent.ReceiveTick` DeltaSeconds))

(event `self.ActiveSkill`
  (params (IsSpecialSkill :type Boolean))
  (if IsSpecialSkill
    (`self.ThrowShieldBomb`)
    (else
      (`self.ShowShield` true))))

(event `Key|Q`
  (params (Key :type "Key Structure"))
  (:`Pressed`
    (`/Engine/EditorBlueprintResources/StandardMacros.FlipFlop`
      (:`A`
        (`|PlayMontage` (`self.Mesh`) "/Game/2019180016/Montage/Shield/AM_Shield_Skill1.AM_Shield_Skill1" 1.0 0.0 "Start"
          (:`then`
            (`|PlayMontage` (`self.BoostMesh`) "/Game/2019180016/Montage/Shield/AM_Shield_Boost_Skill1.AM_Shield_Boost_Skill1" 1.0 0.0 "Start"
              (:`then`
                (`self.SendAnimMontageStatus` "ECAM_CommonSkill"))))))
      (:`B`
        (`|PlayMontage` (`self.Mesh`) "/Game/2019180016/Montage/Shield/AM_Shield_Skill1.AM_Shield_Skill1" 1.0 0.0 "End"
          (:`then`
            (`|PlayMontage` (`self.BoostMesh`) "/Game/2019180016/Montage/Shield/AM_Shield_Boost_Skill1.AM_Shield_Boost_Skill1" 1.0 0.0 "End"
              (:`then`
                (`self.SendAnimMontageStatus` "ECAM_CommonSkill" 1)
                (`self.ShowShield` false)))))))))

(event `Key|Z`
  (params (Key :type "Key Structure"))
  (:`Pressed`
    (`|PlayMontage` (`self.Mesh`) "/Game/2019180016/Montage/Shield/AM_Shield_Skill2.AM_Shield_Skill2" 1.0 0.0 "Start" :!label _label
      (:`then`
        (`|PlayMontage` (`self.BoostMesh`) "/Game/2019180016/Montage/Shield/AM_Shield_Boost_Skill2.AM_Shield_Boost_Skill2"
          (:`then`
            (`self.SendAnimMontageStatus` "ECAM_SpecialSkill")))))))

(event `self.PlaySkillMontage`
  (params (IsSpecialSkill :type Boolean) (SectionNum :type Byte))
  (if IsSpecialSkill
    (goto _label)
    (elif (== SectionNum 0)
      (`|PlayMontage` (`self.Mesh`) "/Game/2019180016/Montage/Shield/AM_Shield_Skill1.AM_Shield_Skill1" 1.0 0.0 "Start"
        (:`then`
          (`|PlayMontage` (`self.BoostMesh`) "/Game/2019180016/Montage/Shield/AM_Shield_Boost_Skill1.AM_Shield_Boost_Skill1" 1.0 0.0 "Start")))
      (else
        (`|PlayMontage` (`self.Mesh`) "/Game/2019180016/Montage/Shield/AM_Shield_Skill1.AM_Shield_Skill1" 1.0 0.0 "End"
          (:`then`
            (`|PlayMontage` (`self.BoostMesh`) "/Game/2019180016/Montage/Shield/AM_Shield_Boost_Skill1.AM_Shield_Boost_Skill1" 1.0 0.0 "End"
              (:`then`
                (`self.ShowShield` false)))))))))

(fn `ShowShield`
  (params (IsShowing :type Boolean))
  (bind _shieldactor (`self.ShieldActor`))
  (if IsShowing
    (bind _returnvalue (`|SpawnActorFromClass` "/Game/2019180016/Blueprint/SkillBP/BP_Shield.BP_Shield_C" (`KismetMathLibrary.MakeTransform` (`SceneComponent.RelativeLocation` (`self.ShieldLocate`))) "Undefined" "MultiplyWithRoot" null (`self.ShieldHealth`) null))
    (`self.K2_AttachToActor` _returnvalue self "None" "KeepRelative" "KeepRelative" "KeepRelative" true)
    (set `self.ShieldActor` _returnvalue)
    (`KismetSystemLibrary.PrintString` "Showing Shield")
    (else
      (set `self.ShieldHealth` (`/Game/2019180016/Blueprint/SkillBP/BP_Shield.Health` _shieldactor))
      (`self.K2_DetachFromActor` _shieldactor "KeepRelative" "KeepRelative" "KeepRelative")
      (`self.K2_DestroyActor` _shieldactor)
      (`KismetSystemLibrary.PrintString` "Hiding Shield"))))

(fn `ThrowShieldBomb`
  (bind _returnvalue (`|SpawnActorFromClass` "/Game/2019180016/Blueprint/SkillBP/BP_ShieldSphere.BP_ShieldSphere_C" (`KismetMathLibrary.MakeTransform` (0.0 0.0 0.0)) "Undefined" "OverrideRootScale" null (`|GetArrayItem` (`self.Tags`)) null))
  (`self.K2_AttachToActor` _returnvalue self "None" "KeepRelative" "KeepRelative" "KeepRelative" true))

(fn `UserConstructionScript`)