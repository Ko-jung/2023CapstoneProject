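; Playable Wind character with a common wind-blast skill and a special tornado skill.
; Q, Z or PlaySkillMontage play paired body and boost-mesh montages and send their status, while ActiveSkill separately applies the effects.
; ShootWind recoils the character, at half power unless falling, and sphere-traces forward to launch characters whose first tag (team) differs.
; SpawnTornado spawns a team-tagged tornado where a camera line trace hits.
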(event `self.SetCustomDepth`
  (params (On :type Boolean))
  (`PrimitiveComponent.SetRenderCustomDepth` (`self.Mesh`) On)
  (`PrimitiveComponent.SetRenderCustomDepth` (`self.BoostMesh`) On))

(event `self.ReceiveTick`
  (params (DeltaSeconds :type "Float (single-precision)"))
  (`parent.ReceiveTick` DeltaSeconds))

(event `Key|Q`
  (params (Key :type "Key Structure"))
  (:`Pressed`
    (`|PlayMontage` (`self.Mesh`) "/Game/2019180016/Montage/Wind/AM_Wind_Skill1.AM_Wind_Skill1" :!label _label
      (:`then`
        (`|PlayMontage` (`self.BoostMesh`) "/Game/2019180016/Montage/Wind/AM_Wind_Boost_Skill1.AM_Wind_Boost_Skill1"
          (:`then`
            (`self.SendAnimMontageStatus` "ECAM_CommonSkill")))))))

(event `self.PlaySkillMontage`
  (params (IsSpecialSkill :type Boolean) (SectionNum :type Byte))
  (`KismetSystemLibrary.PrintString` "Wind Play Skill Montage Called")
  (if IsSpecialSkill
    (`|PlayMontage` (`self.Mesh`) "/Game/2019180016/Montage/Wind/AM_Wind_Skill2.AM_Wind_Skill2" :!label _label_2
      (:`then`
        (`|PlayMontage` (`self.BoostMesh`) "/Game/2019180016/Montage/Wind/AM_Wind_Boost_Skill2.AM_Wind_Boost_Skill2"
          (:`then`
            (`self.SendAnimMontageStatus` "ECAM_SpecialSkill")))))
    (else
      (goto _label))))

(event `self.ActiveSkill`
  (params (IsSpecialSkill :type Boolean))
  (if IsSpecialSkill
    (`self.SpawnTornado`)
    (else
      (`self.ShootWind`))))

(event `Key|Z`
  (params (Key :type "Key Structure"))
  (:`Pressed`
    (goto _label_2)))

(fn `ShootWind`
  (bind _returnvalue (`self.K2_GetActorLocation`))
  (bind _returnvalue_2 (`self.GetActorForwardVector` (`self.GetController`)))
  (`|ExecutionSequence`
    (:`then_0`
      (if (`NavMovementComponent.IsFalling` (`self.CharacterMovement`))
        (`self.LaunchCharacter` (* _returnvalue_2 (`self.LaunchPower`) -1.0) true true)
        (else
          (`self.LaunchCharacter` (* _returnvalue_2 (/ (`self.LaunchPower`) 2.0) -1.0) true true))))
    (:`then_1`
      (bind _outhits (`KismetSystemLibrary.SphereTraceMulti` :`Start` _returnvalue :`End` (+ _returnvalue (* (`self.GetActorForwardVector` (`self.GetController`)) 1000.0)) :`Radius` 150.0 :`TraceChannel` "TraceTypeQuery3" :`DrawDebugType` "ForDuration"))
      (for _array_element _outhits
        (bind (_bblockinghit _binitialoverlap _time _distance _location _impactpoint _normal _impactnormal _physmat _hitactor) (`GameplayStatics.BreakHitResult` _array_element))
        (`KismetSystemLibrary.PrintString` (`KismetStringLibrary.Concat_StrStr` (`KismetSystemLibrary.GetDisplayName` _hitactor) " AAAAA"))
        (bind _asskyscraper_character (cast `SkyscraperCharacter` _hitactor))
        (`KismetSystemLibrary.PrintString` "BBBB")
        (if (!= (`|GetArrayItem` (`self.Tags`)) (`|GetArrayItem` (`Actor.Tags` _hitactor)))
          (`KismetSystemLibrary.PrintString` "CCCC")
          (`self.LaunchCharacter` _asskyscraper_character (* (`self.GetActorForwardVector` (`self.GetController`)) 1000.0) true true)
          (`KismetSystemLibrary.PrintString` (`KismetStringLibrary.Concat_StrStr` (`KismetSystemLibrary.GetDisplayName` _asskyscraper_character) " Launched!")))))))

(fn `SpawnTornado`
  (bind _followcamera (`self.FollowCamera`))
  (bind _returnvalue (`SceneComponent.K2_GetComponentLocation` _followcamera))
  (bind (_outhit _returnvalue_2) (`KismetSystemLibrary.LineTraceSingle` _returnvalue (+ _returnvalue (* (`SceneComponent.GetForwardVector` _followcamera) 1000.0)) "TraceTypeQuery1"))
  (if _returnvalue_2
    (`|SpawnActorFromClass` "/Game/2019180016/Blueprint/SkillBP/BP_WindTornado.BP_WindTornado_C" (`KismetMathLibrary.MakeTransform` (`.Location` (`GameplayStatics.BreakHitResult` _outhit))) "Undefined" "MultiplyWithRoot" null (`|GetArrayItem` (`self.Tags`)) null)
    (`KismetSystemLibrary.PrintString` "Spawn Tornado")))

(fn `UserConstructionScript`)