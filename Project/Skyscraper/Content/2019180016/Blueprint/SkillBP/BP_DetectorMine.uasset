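; Detector mine skill actor: a radar pod that periodically scans for non-allied SkyscraperCharacters.
; The pod falls under physics until it drops below its spawn height or overlaps a non-character, then freezes, switches to its active mesh and animates vertically.
; Tick drives a delayed, expanding sphere pulse that reports each new target through MainGameMode.SendDetecting, or enables custom depth without that game mode.
; The detected list clears after each pulse.
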(event `self.ReceiveBeginPlay`
  (bind (_returnvalue_x _returnvalue_y _returnvalue_z) (`KismetMathLibrary.BreakVector` (`SceneComponent.K2_GetComponentLocation` (`self.StaticMesh`))))
  (`parent.ReceiveBeginPlay`)
  (`self.SphereVisiable` false)
  (`PrimitiveComponent.SetSimulatePhysics` (`self.StaticMesh`) true)
  (`PrimitiveComponent.SetCollisionEnabled` (`self.StaticMesh`) "QueryAndPhysics")
  (set `self.SpawnZLocation` (- _returnvalue_z 5.0)))

(event `self.ReceiveTick`
  (params (DeltaSeconds :type "Float (single-precision)"))
  (bind (_returnvalue_x _returnvalue_y _returnvalue_z) (`KismetMathLibrary.BreakVector` (`SceneComponent.K2_GetComponentLocation` (`self.StaticMesh`))))
  (`|ExecutionSequence`
    (:`then_0`
      (if (and (< _returnvalue_z (`self.SpawnZLocation`)) (not (`self.IsSetting`)))
        (`self.SetIsSettingTrue`)
        (`KismetSystemLibrary.PrintString` "Falling Stop")))
    (:`then_1`
      (if (`self.IsSetting`)
        (`|ExecutionSequence`
          (:`then_0`
            (`KismetSystemLibrary.Delay` 7.0)
            (`self.SphereVisiable` true)
            (bind (_direction _newtrack_0) (`Timeline|BoomSphere` :!label _label)
              (:`Update`
                (`SceneComponent.SetWorldScale3D` (`self.Sphere`) (`KismetMathLibrary.Conv_DoubleToVector` (`KismetMathLibrary.Lerp` 0.25 10.0 _newtrack_0))))
              (:`Finished`
                (`|ExecutionSequence`
                  (:`then_0`
                    (`self.SphereVisiable` false)
                    (`KismetArrayLibrary.Array_Clear` (`self.OverlappedCharacter`)))
                  (:`then_1`
                    (goto _label :!via `SetNewTime`))))))
          (:`then_1`
            (bind (_direction_2 _newtrack_0_2) (`Timeline|Timeline` :!label _label_2)
              (:`Update`
                (`SceneComponent.K2_SetWorldLocation` (`self.StaticMesh`) (+ (`self.SettingLocation`) (`KismetMathLibrary.MakeVector` 0.0 0.0 (`KismetMathLibrary.Lerp` 0.0 40.0 _newtrack_0_2))) false false))
              (:`Finished`
                (`|ExecutionSequence`
                  (:`then_0`
                    (goto _label_2 :!via `SetNewTime`)))))))))))

(event `self.SphereCollision.OnComponentBeginOverlap`
  (params (OverlappedComponent :type "PrimitiveComponent Object Reference") (OtherActor :type "Actor Object Reference") (OtherComp :type "PrimitiveComponent Object Reference") (OtherBodyIndex :type Integer) (bFromSweep :type Boolean) (SweepResult :type "HitResult Structure (by ref)"))
  (if (== (`KismetArrayLibrary.Array_Find` (`self.OverlappedCharacter`) OtherActor) -1)
    (bind _asskyscraper_character (cast `SkyscraperCharacter` OtherActor))
    (if (not (`self.IsAllience?` _asskyscraper_character))
      (bind _asmain_game_mode (cast `MainGameMode` (`GameplayStatics.GetGameMode`))
        (:`then`
          (`KismetSystemLibrary.PrintString` (`KismetSystemLibrary.GetDisplayName` _asskyscraper_character))
          (`MainGameMode.SendDetecting` _asmain_game_mode (`self.GetOwner`) _asskyscraper_character)
          (`KismetArrayLibrary.Array_Add` (`self.OverlappedCharacter`) _asskyscraper_character))
        (:`CastFailed`
          (`PrimitiveComponent.SetRenderCustomDepth` (`Character.Mesh` _asskyscraper_character) true))))))

(event `self.SettingCollision.OnComponentBeginOverlap`
  (params (OverlappedComponent :type "PrimitiveComponent Object Reference") (OtherActor :type "Actor Object Reference") (OtherComp :type "PrimitiveComponent Object Reference") (OtherBodyIndex :type Integer) (bFromSweep :type Boolean) (SweepResult :type "HitResult Structure (by ref)"))
  (cast `Character` OtherActor
    (:`CastFailed`
      (if (and (!= (`self.Sphere`) OtherComp) (!= (`self.SphereCollision`) OtherComp))
        (`self.SetIsSettingTrue`)
        (`KismetSystemLibrary.PrintString` "CollisionStop")))))

(event `self.StaticMesh.OnComponentHit`
  (params (HitComponent :type "PrimitiveComponent Object Reference") (OtherActor :type "Actor Object Reference") (OtherComp :type "PrimitiveComponent Object Reference") (NormalImpulse :type "Vector Structure") (Hit :type "HitResult Structure (by ref)")))

(fn `SetIsSettingTrue`
  (`PrimitiveComponent.SetSimulatePhysics` (`self.StaticMesh`) false)
  (`StaticMeshComponent.SetStaticMesh` (`self.StaticMesh`) "/Game/2016180023/character/5_radar/radar_skill_radar_pod_on.radar_skill_radar_pod_on")
  (set `self.IsSetting` true)
  (`PrimitiveComponent.SetCollisionEnabled` (`self.StaticMesh`) "NoCollision")
  (set `self.SettingLocation` (`SceneComponent.K2_GetComponentLocation` (`self.StaticMesh`))))

(fn `SphereVisiable`
  (params (`IsVisible?` :type Boolean))
  (bind _spherecollision (`self.SphereCollision`))
  (bind _sphere (`self.Sphere`))
  (if `IsVisible?`
    (`SceneComponent.SetVisibility` _sphere true false)
    (`PrimitiveComponent.SetCollisionEnabled` _spherecollision "QueryOnly")
    (`SceneComponent.SetVisibility` _spherecollision true false)
    (else
      (`SceneComponent.SetVisibility` _sphere false false)
      (`PrimitiveComponent.SetCollisionEnabled` _spherecollision "NoCollision")
      (`SceneComponent.SetVisibility` _spherecollision false false))))

(fn `UserConstructionScript`)