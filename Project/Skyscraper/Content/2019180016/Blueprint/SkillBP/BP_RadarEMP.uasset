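; BP_RadarEMP is a skill actor that emits an expanding EMP pulse against SkyscraperCharacter actors.
; On BeginPlay a timeline scales the actor up, growing its Sphere outward.
; Each character the Sphere overlaps is recorded to prevent repeat hits, then has SubtractFuelHalf called and lock-on temporarily disabled, with no alliance check.
; A debug-drawn multi-sphere trace also runs at start, but its alliance check leads to no action.
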(event `self.ReceiveBeginPlay`
  (bind _returnvalue (`self.K2_GetActorLocation`))
  (`parent.ReceiveBeginPlay`)
  (`|ExecutionSequence`
    (:`then_0`
      (bind (_outhits _returnvalue_2) (`KismetSystemLibrary.SphereTraceMulti` :`Start` _returnvalue :`End` _returnvalue :`Radius` 6000.0 :`TraceChannel` "TraceTypeQuery1" :`DrawDebugType` "ForDuration"))
      (if _returnvalue_2
        (for _array_element _outhits
          (bind _asskyscraper_character (cast `SkyscraperCharacter` (`.HitActor` (`GameplayStatics.BreakHitResult` _array_element))))
          (if (`self.IsAllience?` _asskyscraper_character)
            _))))
    (:`then_1`
      (bind (_direction _newtrack_0) (`Timeline|Timeline`)
        (:`Update`
          (`self.SetActorScale3D` (* (60.0 60.0 60.0) _newtrack_0)))))))

(event `self.ReceiveTick`
  (params (DeltaSeconds :type "Float (single-precision)")))

(event `self.Sphere.OnComponentBeginOverlap`
  (params (OverlappedComponent :type "PrimitiveComponent Object Reference") (OtherActor :type "Actor Object Reference") (OtherComp :type "PrimitiveComponent Object Reference") (OtherBodyIndex :type Integer) (bFromSweep :type Boolean) (SweepResult :type "HitResult Structure (by ref)"))
  (if (== (`KismetArrayLibrary.Array_Find` (`self.OverlappedCharacter`) OtherActor) -1)
    (`KismetArrayLibrary.Array_Add` (`self.OverlappedCharacter`) OtherActor)
    (bind _asskyscraper_character (cast `SkyscraperCharacter` OtherActor))
    (`SkyscraperCharacter.SubtractFuelHalf` _asskyscraper_character)
    (`SkyscraperCharacter.DoDisableLockOn` _asskyscraper_character 10.0)))

(fn `UserConstructionScript`)