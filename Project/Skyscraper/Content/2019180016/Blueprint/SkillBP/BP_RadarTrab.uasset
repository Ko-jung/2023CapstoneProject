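; Radar trap skill actor that falls under physics, sticks where it hits a non-character, then hunts characters.
; Once attached, Tick sphere-traces around it for a non-allied Character to target.
; It moves toward that target by swept steps whenever the Visibility line trace between them hits nothing.
; Hitting any Character while attached spawns an explosion, launches the character upward and destroys the trap.
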(event `self.ReceiveBeginPlay`
  (`parent.ReceiveBeginPlay`)
  (set `self.IsAttach` false)
  (`PrimitiveComponent.SetSimulatePhysics` (`self.StaticMesh`) true))

(event `self.ReceiveTick`
  (params (DeltaSeconds :type "Float (single-precision)"))
  (bind _returnvalue (`self.K2_GetActorLocation`))
  (bind _returnvalue_2 (`self.K2_GetActorLocation`))
  (bind _returnvalue_3 (`self.K2_GetActorLocation` (`self.ToTarget`)))
  (if (`self.IsAttach`)
    (`/Engine/EditorBlueprintResources/StandardMacros.IsValid` (`self.ToTarget`)
      (:`Is Valid`
        (bind (_outhit _returnvalue_4) (`KismetSystemLibrary.LineTraceSingle` _returnvalue_2 _returnvalue_3 "TraceTypeQuery1"))
        (if _returnvalue_4
          (`KismetSystemLibrary.PrintString` "Yesy")
          (else
            (`SceneComponent.K2_AddRelativeLocation` (`self.StaticMesh`) (* (`KismetMathLibrary.Normal` (- _returnvalue_3 _returnvalue_2)) 10.0) true true)
            (`KismetSystemLibrary.PrintString` "No"))))
      (:`Is Not Valid`
        (bind (_outhit_2 _returnvalue_5) (`KismetSystemLibrary.SphereTraceSingle` :`Start` _returnvalue :`End` _returnvalue :`Radius` 1000.0 :`TraceChannel` "TraceTypeQuery3" :`DrawDebugType` "ForOneFrame"))
        (if _returnvalue_5
          (bind _ascharacter (cast `Character` (`.HitActor` (`GameplayStatics.BreakHitResult` _outhit_2))))
          (if (not (`self.IsAllience?` _ascharacter))
            (set `self.ToTarget` _ascharacter)))))))

(event `self.StaticMesh.OnComponentHit`
  (params (HitComponent :type "PrimitiveComponent Object Reference") (OtherActor :type "Actor Object Reference") (OtherComp :type "PrimitiveComponent Object Reference") (NormalImpulse :type "Vector Structure") (Hit :type "HitResult Structure (by ref)"))
  (bind _ascharacter (cast `Character` OtherActor)
    (:`then`
      (if (`self.IsAttach`)
        (`GameplayStatics.SpawnEmitterAtLocation` "/Game/StarterContent/Particles/P_Explosion.P_Explosion" (`self.K2_GetActorLocation`))
        (`Character.LaunchCharacter` _ascharacter (0.0 0.0 1000.0) false false)
        (`self.K2_DestroyActor`)))
    (:`CastFailed`
      (set `self.IsAttach` true)
      (`PrimitiveComponent.SetSimulatePhysics` (`self.StaticMesh`) false)
      (`self.K2_SetActorRotation` (struct :`Pitch` 90.0 :`Roll` 90.0))
      (`self.K2_SetActorLocation` (+ (`.Location` (`GameplayStatics.BreakHitResult` Hit)) (* (`self.GetActorUpVector`) 5.0)))
      (`KismetSystemLibrary.PrintString` "Attach"))))

(fn `UserConstructionScript`)