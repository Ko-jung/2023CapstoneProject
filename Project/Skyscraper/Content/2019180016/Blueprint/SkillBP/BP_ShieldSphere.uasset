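; BP_ShieldSphere is a timed shield skill actor that calls SkillInteract on Skyscraper characters near it.
; A looping quarter-second timer runs a sphere trace, diffing current and previous overlap sets to notify only new entrants.
; Characters leaving early get no call; those in the last set are called again on destruction.
; Overlap events are empty, and the alliance check sits in unreachable code, so allies are not filtered.
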(event `self.ReceiveBeginPlay`
  (`parent.ReceiveBeginPlay`)
  (`self.SetLifeSpan` (`self.Timer`))
  (`KismetSystemLibrary.K2_SetTimer` null "CollisionCheck" 0.25 true))

(event `self.ReceiveTick`
  (params (DeltaSeconds :type "Float (single-precision)")))

(event `self.SphereCollision.OnComponentBeginOverlap`
  (params (OverlappedComponent :type "PrimitiveComponent Object Reference") (OtherActor :type "Actor Object Reference") (OtherComp :type "PrimitiveComponent Object Reference") (OtherBodyIndex :type Integer) (bFromSweep :type Boolean) (SweepResult :type "HitResult Structure (by ref)")))

(event `self.SphereCollision.OnComponentEndOverlap`
  (params (OverlappedComponent :type "PrimitiveComponent Object Reference") (OtherActor :type "Actor Object Reference") (OtherComp :type "PrimitiveComponent Object Reference") (OtherBodyIndex :type Integer)))

(event `self.ReceiveDestroyed`
  (bind _result (`BlueprintSetLibrary.Set_ToArray` (`self.PrevOverlapped`)))
  (for _array_element _result
    (`SkyscraperCharacter.SkillInteract` _array_element "BP_ShieldSphere" 0.0)
    (`KismetSystemLibrary.PrintString` (`KismetStringLibrary.Concat_StrStr` (`KismetSystemLibrary.GetDisplayName` _array_element) "Delete"))))

(fn `CollisionCheck`
  (bind _returnvalue (`self.K2_GetActorLocation`))
  (bind _curroverlapped (`self.CurrOverlapped`))
  (`|ExecutionSequence`
    (:`then_0`
      (bind _outhits (`KismetSystemLibrary.SphereTraceMulti` _returnvalue _returnvalue 300.0 "TraceTypeQuery1"))
      (for _array_element _outhits
        (bind _asskyscraper_character (cast `SkyscraperCharacter` (`.HitActor` (`GameplayStatics.BreakHitResult` _array_element))))
        (`BlueprintSetLibrary.Set_Add` (`self.CurrOverlapped`) _asskyscraper_character)))
    (:`then_1`
      (bind _result (`BlueprintSetLibrary.Set_ToArray` (`self.CurrOverlapped`)))
      (for _array_element_2 _result
        (if (not (`BlueprintSetLibrary.Set_Contains` (`self.PrevOverlapped`) _array_element_2))
          (`SkyscraperCharacter.SkillInteract` _array_element_2 "BP_ShieldSphere" 0.0)
          (`KismetSystemLibrary.PrintString` (`KismetStringLibrary.Concat_StrStr` (`KismetSystemLibrary.GetDisplayName` _array_element_2) "Begin Overlap"))))
      (set `self.PrevOverlapped` _curroverlapped)
      (`BlueprintSetLibrary.Set_Clear` _curroverlapped))))

(fn `UserConstructionScript`)