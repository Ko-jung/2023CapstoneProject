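; BP_ShieldSphereThrow is a thrown skill projectile that deploys a BP_ShieldSphere where it lands.
; On BeginPlay it launches its Sphere with a velocity-change impulse along the spawning character's forward vector plus up.
; Hitting anything other than a Character passes the impact location and team (first actor tag) through server-then-client events.
; The client event spawns the shield, prints debug locations and destroys the projectile.
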(event `self.ReceiveBeginPlay`
  (`parent.ReceiveBeginPlay`)
  (`PrimitiveComponent.AddImpulse` (`self.Sphere`) (* (+ (`self.GetActorForwardVector` (`self.SpawnChar`)) (0.0 0.0 1.0)) 500.0) "None" true))

(event `self.Sphere.OnComponentHit`
  (params (HitComponent :type "PrimitiveComponent Object Reference") (OtherActor :type "Actor Object Reference") (OtherComp :type "PrimitiveComponent Object Reference") (NormalImpulse :type "Vector Structure") (Hit :type "HitResult Structure (by ref)"))
  (cast `Character` OtherActor
    (:`CastFailed`
      (`self.Spawn Shield Sphere On Server` (`SceneComponent.K2_GetComponentLocation` (`self.Sphere`)) (`|GetArrayItem` (`self.Tags`))))))

(event `Spawn Shield Sphere On Server`
  (params (`Spawn Transform Location` :type "Vector Structure") (WhoSpawnTeam :type Name))
  (`self.Spawn Shield Sphere On Client` `Spawn Transform Location` WhoSpawnTeam))

(event `Spawn Shield Sphere On Client`
  (params (`Spawn Transform Location` :type "Vector Structure") (WhoSpawnTeam :type Name))
  (`|SpawnActorFromClass` "/Game/2019180016/Blueprint/SkillBP/BP_ShieldSphere.BP_ShieldSphere_C" (`KismetMathLibrary.MakeTransform` `Spawn Transform Location`) "Undefined" "MultiplyWithRoot" null WhoSpawnTeam null)
  (`KismetSystemLibrary.PrintString` (`KismetStringLibrary.Concat_StrStr` "SpawnChar Location: " (`KismetStringLibrary.Conv_VectorToString` (`self.K2_GetActorLocation` (`self.SpawnChar`)))))
  (`KismetSystemLibrary.PrintString` (`KismetStringLibrary.Concat_StrStr` "Throw Location: " (`KismetStringLibrary.Conv_VectorToString` (`self.K2_GetActorLocation`))))
  (`self.K2_DestroyActor`))

(fn `UserConstructionScript`)