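; Grab variant of a thrown boomerang skill projectile that seizes a non-allied character and drags it along.
; A timeline moves the spinning boomerang out from its start location, then Tick homes it back toward an offset on the thrower.
; An overlapped enemy is teleported to the boomerang's location every frame.
; On return, separate spheres trigger the thrower's catch once and destroy the boomerang; timer-based fallbacks are left unfinished or disconnected.
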(event `self.ReceiveBeginPlay`
  (`parent.ReceiveBeginPlay`)
  (set `RotatingMovementComponent.RotationRate` (`KismetMathLibrary.MakeRotator` 0.0 0.0 720.0) (`self.RotatingMovement`))
  (`|ExecutionSequence`
    (:`then_0`
      (bind (_direction _newtrack_1) (`Timeline|Timeline` :!via `SetNewTime` :!label _label)
        (:`Update`
          (`self.K2_SetActorLocation` (+ (`self.StartLocation`) (* (`self.EndLocation`) _newtrack_1))))
        (:`Finished`
          (set `self.IsBackTracking` true))))
    (:`then_1`
      (goto _label))))

(event `self.Sphere.OnComponentBeginOverlap`
  (params (OverlappedComponent :type "PrimitiveComponent Object Reference") (OtherActor :type "Actor Object Reference") (OtherComp :type "PrimitiveComponent Object Reference") (OtherBodyIndex :type Integer) (bFromSweep :type Boolean) (SweepResult :type "HitResult Structure (by ref)"))
  (bind _ascharacter (cast `Character` OtherActor))
  (if (not (`self.IsAllience?` _ascharacter))
    (set `self.GrabbedCharacter` _ascharacter)
    (set `self.IsGrabbing` true)))

(event `self.DestroySphere.OnComponentBeginOverlap`
  (params (OverlappedComponent :type "PrimitiveComponent Object Reference") (OtherActor :type "Actor Object Reference") (OtherComp :type "PrimitiveComponent Object Reference") (OtherBodyIndex :type Integer) (bFromSweep :type Boolean) (SweepResult :type "HitResult Structure (by ref)"))
  (if (and (== OtherActor (`self.ThrowChar`)) (`self.IsBackTracking`))
    (`self.K2_DestroyActor`)))

(event `self.CatchMotionSphere.OnComponentBeginOverlap`
  (params (OverlappedComponent :type "PrimitiveComponent Object Reference") (OtherActor :type "Actor Object Reference") (OtherComp :type "PrimitiveComponent Object Reference") (OtherBodyIndex :type Integer) (bFromSweep :type Boolean) (SweepResult :type "HitResult Structure (by ref)"))
  (if (and (not (`self.IsSendingCatch`)) (and (== OtherActor (`self.ThrowChar`)) (`self.IsBackTracking`)))
    (bind _asbp_boomerang_character (cast `/Game/2019180016/Blueprint/Character/CanControll/BP_BoomerangCharacter` (`self.ThrowChar`)))
    (`/Game/2019180016/Blueprint/Character/CanControll/BP_BoomerangCharacter.CatchBoomerang1` _asbp_boomerang_character)
    (set `self.IsSendingCatch` true)))

(event `self.ReceiveTick`
  (params (DeltaSeconds :type "Float (single-precision)"))
  (bind _returnvalue (`self.K2_GetActorLocation`))
  (`|ExecutionSequence`
    (:`then_0`
      (if (`self.IsBackTracking`)
        (`self.K2_SetActorLocation` (+ _returnvalue (* (`KismetMathLibrary.Normal` (- (+ (`self.K2_GetActorLocation` (`self.ThrowChar`)) (0.0 -50.0 95.0)) _returnvalue)) (* DeltaSeconds 1000.0))))))
    (:`then_1`
      (if (`self.IsGrabbing`)
        (`self.K2_SetActorLocation` (`self.GrabbedCharacter`) (`self.K2_GetActorLocation`) false false)))
    (:`then_2`
      (`self.AddTimer` DeltaSeconds)
      (`|ExecutionSequence`
        (:`then_0`
          (if (and (> (`self.Timer`) 1.5) (not (`self.IsSendingCatch`)))
            _))))))

(fn `AddTimer`
  (params (DeltaTime :type "Float (double-precision)"))
  (set `self.Timer` (+ (`self.Timer`) DeltaTime)))

(fn `UserConstructionScript`)