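; Boomerang skill projectile that drags characters along and stuns them on returning to its thrower.
; It spins along a Timeline-driven outward path, spawning Elect_Trab at the computed end point, then homes back every Tick.
; Skyscraper characters leaving CollisionSphere, except the thrower, are snapped to it each frame; CatchSphere triggers the catch, DestroySphere stuns them and destroys it.
; Older chain-target and pull-to-center logic remains unconnected.
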(event `self.ReceiveBeginPlay`
  (`parent.ReceiveBeginPlay`)
  (set `RotatingMovementComponent.RotationRate` (`KismetMathLibrary.MakeRotator` 0.0 0.0 720.0) (`self.RotatingMovement`))
  (set `self.StartLocation` (`self.K2_GetActorLocation`))
  (bind _output_get (set `self.EndLocation` (+ (* (`self.TargetVector`) 1000.0) (`self.StartLocation`))))
  (`|SpawnActorFromClass` "/Game/2019180016/Blueprint/SkillBP/Elect_Trab.Elect_Trab_C" (`KismetMathLibrary.MakeTransform` _output_get) "Undefined" "MultiplyWithRoot" null "None" null)
  (`|ExecutionSequence`
    (:`then_0`
      (bind (_direction _newtrack_1) (`Timeline|Timeline` :!via `SetNewTime` :!label _label)
        (:`Update`
          (`self.K2_SetActorLocation` (+ (`self.StartLocation`) (* (`self.EndLocation`) _newtrack_1))))
        (:`Finished`
          (set `self.IsBackTracking` true))))
    (:`then_1`
      (goto _label))))

(event `self.CollisionSphere.OnComponentBeginOverlap`
  (params (OverlappedComponent :type "PrimitiveComponent Object Reference") (OtherActor :type "Actor Object Reference") (OtherComp :type "PrimitiveComponent Object Reference") (OtherBodyIndex :type Integer) (bFromSweep :type Boolean) (SweepResult :type "HitResult Structure (by ref)")))

(event `self.CatchSphere.OnComponentBeginOverlap`
  (params (OverlappedComponent :type "PrimitiveComponent Object Reference") (OtherActor :type "Actor Object Reference") (OtherComp :type "PrimitiveComponent Object Reference") (OtherBodyIndex :type Integer) (bFromSweep :type Boolean) (SweepResult :type "HitResult Structure (by ref)"))
  (bind _throwcharacter (`self.ThrowCharacter`))
  (if (and (== OtherActor _throwcharacter) (`self.IsBackTracking`))
    (bind _asbp_boomerang_character (cast `/Game/2019180016/Blueprint/Character/CanControll/BP_BoomerangCharacter` _throwcharacter))
    (`/Game/2019180016/Blueprint/Character/CanControll/BP_BoomerangCharacter.CatchBoomerang2` _asbp_boomerang_character)))

(event `self.ReceiveTick`
  (params (DeltaSeconds :type "Float (single-precision)"))
  (bind _returnvalue (`self.K2_GetActorLocation`))
  (`|ExecutionSequence`
    (:`then_0`
      (if (`self.IsBackTracking`)
        (`self.K2_SetActorLocation` (+ _returnvalue (* (`KismetMathLibrary.Normal` (- (`self.K2_GetActorLocation` (`self.ThrowCharacter`)) _returnvalue)) (* DeltaSeconds 1000.0))))))
    (:`then_1`
      (bind _result (`BlueprintSetLibrary.Set_ToArray` (`self.OverlappedCharacters`)))
      (for _array_element _result
        (`self.K2_SetActorLocation` _array_element (`self.K2_GetActorLocation`) false false)))))

(event `self.DestroySphere.OnComponentBeginOverlap`
  (params (OverlappedComponent :type "PrimitiveComponent Object Reference") (OtherActor :type "Actor Object Reference") (OtherComp :type "PrimitiveComponent Object Reference") (OtherBodyIndex :type Integer) (bFromSweep :type Boolean) (SweepResult :type "HitResult Structure (by ref)"))
  (if (and (== OtherActor (`self.ThrowCharacter`)) (`self.IsBackTracking`))
    (bind _result (`BlueprintSetLibrary.Set_ToArray` (`self.OverlappedCharacters`)))
    (for _array_element _result
      (`SkyscraperCharacter.ApplyStun` _array_element 3.0))
    (`self.K2_DestroyActor`)))

(event `self.CollisionSphere.OnComponentEndOverlap`
  (params (OverlappedComponent :type "PrimitiveComponent Object Reference") (OtherActor :type "Actor Object Reference") (OtherComp :type "PrimitiveComponent Object Reference") (OtherBodyIndex :type Integer))
  (if (not (== OtherActor (`self.ThrowCharacter`)))
    (bind _asskyscraper_character (cast `SkyscraperCharacter` OtherActor))
    (if (not (`BlueprintSetLibrary.Set_Contains` (`self.OverlappedCharacters`) _asskyscraper_character))
      (`BlueprintSetLibrary.Set_Add` (`self.OverlappedCharacters`) _asskyscraper_character))))

(fn `Char Add to Array`
  (params (FindCharacter :type "Character Object Reference (by ref)") (BlockedCharArray :type "Array of Character Object Reference (by ref)"))
  (returns (AddDone :type Boolean))
  (if (== (`KismetArrayLibrary.Array_Find` BlockedCharArray FindCharacter) -1)
    (`KismetArrayLibrary.Array_Add` BlockedCharArray FindCharacter)
    (`KismetSystemLibrary.PrintString` (`KismetStringLibrary.Concat_StrStr` (`KismetSystemLibrary.GetDisplayName` FindCharacter) "Is Append!"))
    (return true)
    (else
      (return false))))

(fn `Get Center Location To Grab And Set Location Array`
  (returns (CenterLocation :type "Vector Structure"))
  (bind _blockcharacterarray (`self.BlockCharacterArray`))
  (for _array_element _blockcharacterarray
    (bind _returnvalue (`self.K2_GetActorLocation` _array_element))
    (set `self.GrabSumLocation` (+ _returnvalue (`self.GrabSumLocation`)))
    (`KismetArrayLibrary.Array_Add` (`self.BlockCharacterLocationArray`) _returnvalue))
  (bind _output_get (set `self.GrabToCenterLocation` (/ (`self.GrabSumLocation`) (`KismetArrayLibrary.Array_Length` _blockcharacterarray))))
  (return _output_get))

(fn `PrintAllCharacterArray`
  (bind _blockcharacterarray (`self.BlockCharacterArray`))
  (for _index (range (`KismetArrayLibrary.Array_Length` _blockcharacterarray))
    (`KismetSystemLibrary.PrintString` (`KismetSystemLibrary.GetDisplayName` (`|GetArrayItem` _blockcharacterarray _index)))))

(fn `UserConstructionScript`)