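; Electric sphere burst skill that slows non-allied SkyscraperCharacters caught in its expanding blast.
; On BeginPlay it spawns a Niagara effect, disables the caster's input and scales itself up through a timeline, then restores input and destroys itself.
; BoomCollision overlaps apply the timed speed debuff as the actor grows.
; A sphere trace also checks hit characters for alliance but acts on none of them.
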(event `self.ReceiveBeginPlay`
  (bind _returnvalue (`self.K2_GetActorLocation`))
  (bind _skillcaster (`self.SkillCaster`))
  (`parent.ReceiveBeginPlay`)
  (`NiagaraFunctionLibrary.SpawnSystemAtLocation` "/Game/2016180023/fx/electric_2/NS_elec_02.NS_elec_02" (`self.K2_GetActorLocation`))
  (`self.DisableInput` _skillcaster (`GameplayStatics.GetPlayerController` 0))
  (bind (_outhits _returnvalue_2) (`KismetSystemLibrary.SphereTraceMulti` _returnvalue _returnvalue 1000.0 "TraceTypeQuery3"))
  (`|ExecutionSequence`
    (:`then_0`
      (if _returnvalue_2
        (for _array_element _outhits
          (bind _asskyscraper_character (cast `SkyscraperCharacter` (`.HitActor` (`GameplayStatics.BreakHitResult` _array_element))))
          (if (`self.IsAllience?` _asskyscraper_character)
            _))))
    (:`then_1`
      (bind (_direction _newtrack_0) (`Timeline|Timeline` :!label _label)
        (:`Update`
          (`self.SetActorScale3D` (* (20.0 20.0 20.0) _newtrack_0)))
        (:`Finished`
          (`self.EnableInput` _skillcaster (`GameplayStatics.GetPlayerController` 0))
          (`|ExecutionSequence`
            (:`then_0`
              (goto _label :!via `SetNewTime`))
            (:`then_1`
              (`self.K2_DestroyActor`))))))))

(event `self.BoomCollision.OnComponentBeginOverlap`
  (params (OverlappedComponent :type "PrimitiveComponent Object Reference") (OtherActor :type "Actor Object Reference") (OtherComp :type "PrimitiveComponent Object Reference") (OtherBodyIndex :type Integer) (bFromSweep :type Boolean) (SweepResult :type "HitResult Structure (by ref)"))
  (bind _asskyscraper_character (cast `SkyscraperCharacter` OtherActor))
  (if (not (`self.IsAllience?` _asskyscraper_character))
    (`SkyscraperCharacter.SetSpeedBuffValue` _asskyscraper_character 0.7 7.0)))

(fn `UserConstructionScript`)