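; Base item actor that a player picks up or uses by holding an interaction until a required time is reached.
; Sphere overlap gives each player character a key-prompt widget, tracked in a map and removed on exit or EndPlay.
; Repeated ItemInteraction calls from one actor at a time fill a gauge; Tick, enabled only meanwhile, resets it after a brief lapse.
; Completion calls DoItemEffectFunc, which here prints a placeholder message and destroys the item.
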(event `self.ReceiveEndPlay`
  (params (EndPlayReason :type "EEndPlayReason Enum" :default "Destroyed"))
  ;[1 1 1] 완료
  (bind _keys (`BlueprintMapLibrary.Map_Keys` (`self.PlayerAndWidgetMap`)))
  (for _array_element _keys
    (`self.RemoveWidget` _array_element)))

(event `self.Sphere.OnComponentBeginOverlap`
  (params (OverlappedComponent :type "PrimitiveComponent Object Reference") (OtherActor :type "Actor Object Reference") (OtherComp :type "PrimitiveComponent Object Reference") (OtherBodyIndex :type Integer) (bFromSweep :type Boolean) (SweepResult :type "HitResult Structure (by ref)"))
  (bind _asskyscraper_character (cast `SkyscraperCharacter` OtherActor))
  (bind _asplayer_controller (cast `PlayerController` (`Pawn.GetController` _asskyscraper_character)))
  (bind _returnvalue (`|CreateWidget` "/Game/2019180031/MainGame/Widget/ItemInteraction/WBP_PressItemKey.WBP_PressItemKey_C" _asplayer_controller))
  (`UserWidget.AddToViewport` _returnvalue 0)
  (`BlueprintMapLibrary.Map_Add` (`self.PlayerAndWidgetMap`) _asskyscraper_character _returnvalue))

(event `self.Sphere.OnComponentEndOverlap`
  (params (OverlappedComponent :type "PrimitiveComponent Object Reference") (OtherActor :type "Actor Object Reference") (OtherComp :type "PrimitiveComponent Object Reference") (OtherBodyIndex :type Integer))
  (`self.RemoveWidget` OtherActor))

(event `RemoveWidget`
  (params (Actor :type "Actor Object Reference (by ref)"))
  (bind (_value _returnvalue) (`BlueprintMapLibrary.Map_Find` (`self.PlayerAndWidgetMap`) Actor))
  (if _returnvalue
    (`Widget.RemoveFromParent` _value)
    (`BlueprintMapLibrary.Map_Remove` (`self.PlayerAndWidgetMap`))))

(event `self.ReceiveTick`
  (params (DeltaSeconds :type "Float (single-precision)"))
  (if (> (- (`GameplayStatics.GetTimeSeconds`) (`self.LastInteractionTime`)) 0.5)
    (set `self.CurrentInteractionTime` 0.0)
    (`SceneComponent.SetHiddenInGame` (`self.Widget`) true false)
    (`self.SetActorTickEnabled` false)
    (set `self.CurrentInteractionActor` null)
    (`self.SetWidgetPercent`)))

(event `/Game/2019180031/Blueprints/Item/BPI_InteractionItem.Item Interaction`
  (params (InteractionActor :type "Actor Object Reference"))
  (bind _currentinteractionactor (`self.CurrentInteractionActor`)
    (:`then`
      (if (== _currentinteractionactor InteractionActor)
        (set `self.CurrentInteractionTime` (+ (`self.CurrentInteractionTime`) (`GameplayStatics.GetWorldDeltaSeconds`)))
        (set `self.LastInteractionTime` (`GameplayStatics.GetTimeSeconds`))
        (`self.SetWidgetPercent`)
        (if (>= (`self.CurrentInteractionTime`) (`self.RequirdTime`))
          (`self.DoItemEffectFunc`))))
    (:`else`
      (set `self.CurrentInteractionActor` InteractionActor)
      (`self.SetActorTickEnabled` true)
      (set `self.LastInteractionTime` (`GameplayStatics.GetTimeSeconds`))
      (bind _aswbp_interaction_gauge (cast `/Game/2019180031/MainGame/Widget/ItemInteraction/WBP_InteractionGauge` (`WidgetComponent.GetWidget` (`self.Widget`))))
      (`UserWidget.SetColorAndOpacity` _aswbp_interaction_gauge (struct :`R` 1.0 :`G` 1.0 :`B` 1.0 :`A` 1.0))
      (`SceneComponent.SetHiddenInGame` (`self.Widget`) false false))))

(event `SetWidgetPercent`
  (bind _aswbp_interaction_gauge (cast `/Game/2019180031/MainGame/Widget/ItemInteraction/WBP_InteractionGauge` (`WidgetComponent.GetWidget` (`self.Widget`))))
  (`/Game/2019180031/MainGame/Widget/ItemInteraction/WBP_InteractionGauge.Set Interaction Percent` _aswbp_interaction_gauge (`KismetMathLibrary.SafeDivide` (`self.CurrentInteractionTime`) (`self.RequirdTime`))))

(fn `DoItemEffectFunc`
  (`KismetSystemLibrary.PrintString` "아이템 효과 발생")
  (`self.K2_DestroyActor`))

(fn `UserConstructionScript`)