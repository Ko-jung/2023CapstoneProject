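; Multi-floor building actor that can collapse into physics debris using Chaos geometry collections.
; The construction script stacks a static mesh floor and four offset walls per level, storing each in an array.
; DoCollapse runs CollapseBuilding from level zero, swapping each piece up to CurrentFloor for a geometry collection at the same relative location.
; Swapped floors get an upward velocity and walls random spin, then CurrentFloor drops below the collapse start.
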(event `self.ReceiveBeginPlay`
  (set `self.CurrentFloor` (`self.Floor`)) ; 0~n-1층임
)

(event `/Game/2019180031/BlueprintInterface/BPI_Collapse.DoCollapse`
  (`self.CollapseBuilding` 0))

(fn `CollapseBuilding`
  (params (`Collapse Start Floor` :type Integer))
  (for _index (range `Collapse Start Floor` (+ (`self.CurrentFloor`) 1))
    (`|ExecutionSequence`
      (:`then_0`
        (`self.SwapStaticToGeometry` (`|GetArrayItem` (`self.Building_Floor`) _index) "/Game/2019180031/Blueprints/Map/Building/GeometryComp/GeoComp_Floor.GeoComp_Floor"))
      (:`then_1`
        (`self.SwapStaticToGeometry` (`|GetArrayItem` (`self.Building_Wall1`) _index) "/Game/2019180031/Blueprints/Map/Building/GeometryComp/GeoComp_wall1.GeoComp_wall1"))
      (:`then_2`
        (`self.SwapStaticToGeometry` (`|GetArrayItem` (`self.Building_Wall2`) _index) "/Game/2019180031/Blueprints/Map/Building/GeometryComp/GeoComp_wall2.GeoComp_wall2"))
      (:`then_3`
        (`self.SwapStaticToGeometry` (`|GetArrayItem` (`self.Building_Wall3`) _index) "/Game/2019180031/Blueprints/Map/Building/GeometryComp/GeoComp_wall3.GeoComp_wall3"))
      (:`then_4`
        (`self.SwapStaticToGeometry` (`|GetArrayItem` (`self.Building_Wall4`) _index) "/Game/2019180031/Blueprints/Map/Building/GeometryComp/GeoComp_wall4.GeoComp_wall4"))))
  (set `self.CurrentFloor` (- `Collapse Start Floor` 1)))

(fn `SwapStaticToGeometry`
  (params (Target :type "StaticMeshComponent Object Reference") (RestCollectionIn :type "GeometryCollection Object Reference"))
  (locals (RelativeLocation :type "Vector Structure"))
  (bind _returnvalue (`KismetMathLibrary.RandomFloat`))
  (bind _returnvalue_2 (`KismetMathLibrary.RandomFloat`))
  (bind _returnvalue_3 (`KismetMathLibrary.RandomFloat`))
  (bind _returnvalue_4 (`KismetMathLibrary.RandomFloat`))
  (set `local.RelativeLocation` (`SceneComponent.RelativeLocation` Target))
  (`ActorComponent.K2_DestroyComponent` Target)
  (`|ExecutionSequence`
    (:`then_0`
      (if (== RestCollectionIn "/Game/2019180031/Blueprints/Map/Building/GeometryComp/GeoComp_Floor.GeoComp_Floor")
        (bind _returnvalue_5 (`AddComponent|NODE_AddGeometryCollectionComponent-11` :`RelativeTransform` (`KismetMathLibrary.MakeTransform` (`local.RelativeLocation`))))
        (`GeometryCollectionComponent.ApplyLinearVelocity` _returnvalue_5 0 (0.0 0.0 100.0))))
    (:`then_1`
      (if (== RestCollectionIn "/Game/2019180031/Blueprints/Map/Building/GeometryComp/GeoComp_wall1.GeoComp_wall1")
        (bind _returnvalue_6 (`AddComponent|NODE_AddGeometryCollectionComponent-12` :`RelativeTransform` (`KismetMathLibrary.MakeTransform` (`local.RelativeLocation`))))
        (`GeometryCollectionComponent.ApplyAngularVelocity` _returnvalue_6 0 (`KismetMathLibrary.MakeVector` _returnvalue _returnvalue _returnvalue))))
    (:`then_2`
      (if (== RestCollectionIn "/Game/2019180031/Blueprints/Map/Building/GeometryComp/GeoComp_wall2.GeoComp_wall2")
        (bind _returnvalue_7 (`AddComponent|NODE_AddGeometryCollectionComponent-13` :`RelativeTransform` (`KismetMathLibrary.MakeTransform` (`local.RelativeLocation`))))
        (`GeometryCollectionComponent.ApplyAngularVelocity` _returnvalue_7 0 (`KismetMathLibrary.MakeVector` _returnvalue_4 _returnvalue_4 _returnvalue_4))))
    (:`then_3`
      (if (== RestCollectionIn "/Game/2019180031/Blueprints/Map/Building/GeometryComp/GeoComp_wall3.GeoComp_wall3")
        (bind _returnvalue_8 (`AddComponent|NODE_AddGeometryCollectionComponent-14` :`RelativeTransform` (`KismetMathLibrary.MakeTransform` (`local.RelativeLocation`))))
        (`GeometryCollectionComponent.ApplyAngularVelocity` _returnvalue_8 0 (`KismetMathLibrary.MakeVector` _returnvalue_3 _returnvalue_3 _returnvalue_3))))
    (:`then_4`
      (if (== RestCollectionIn "/Game/2019180031/Blueprints/Map/Building/GeometryComp/GeoComp_wall4.GeoComp_wall4")
        (bind _returnvalue_9 (`AddComponent|NODE_AddGeometryCollectionComponent-15` :`RelativeTransform` (`KismetMathLibrary.MakeTransform` (`local.RelativeLocation`))))
        (`GeometryCollectionComponent.ApplyAngularVelocity` _returnvalue_9 0 (`KismetMathLibrary.MakeVector` _returnvalue_2 _returnvalue_2 _returnvalue_2))))))

(fn `UserConstructionScript`
  (locals (ChaosObjectType :type "EObjectStateTypeEnum Enum" :default "Chaos_Object_Static"))
  ;[1 1 1] test-1
  (for _index (range (+ (`self.Floor`) 1))
    (`|ExecutionSequence`
      (:`then_0`
        (bind _returnvalue (* _index (`self.FloorDistance`)))
        (bind _returnvalue_2 (`AddComponent|NODE_AddStaticMeshComponent-5` :`RelativeTransform` (`KismetMathLibrary.MakeTransform` (`KismetMathLibrary.MakeVector` 0.0 0.0 (- _returnvalue 500.0)))))
        (`KismetArrayLibrary.Array_Add` (`self.Building_Floor`) _returnvalue_2))
      (:`then_1`
        (bind _returnvalue_3 (`AddComponent|NODE_AddStaticMeshComponent-6` :`RelativeTransform` (`KismetMathLibrary.MakeTransform` (`KismetMathLibrary.MakeVector` 0.0 (`self.Wall1Offset`) _returnvalue))))
        (`KismetArrayLibrary.Array_Add` (`self.Building_Wall1`) _returnvalue_3))
      (:`then_2`
        (bind _returnvalue_4 (`AddComponent|NODE_AddStaticMeshComponent-7` :`RelativeTransform` (`KismetMathLibrary.MakeTransform` (`KismetMathLibrary.MakeVector` (`self.wall2Offset`) 0.0 _returnvalue))))
        (`KismetArrayLibrary.Array_Add` (`self.Building_Wall2`) _returnvalue_4))
      (:`then_3`
        (bind _returnvalue_5 (`AddComponent|NODE_AddStaticMeshComponent-8` :`RelativeTransform` (`KismetMathLibrary.MakeTransform` (`KismetMathLibrary.MakeVector` 0.0 (`self.wall3Offset`) _returnvalue))))
        (`KismetArrayLibrary.Array_Add` (`self.Building_Wall3`) _returnvalue_5))
      (:`then_4`
        (bind _returnvalue_6 (`AddComponent|NODE_AddStaticMeshComponent-9` :`RelativeTransform` (`KismetMathLibrary.MakeTransform` (`KismetMathLibrary.MakeVector` (`self.wall4Offset`) 0.0 _returnvalue))))
        (`KismetArrayLibrary.Array_Add` (`self.Building_Wall4`) _returnvalue_6)))))