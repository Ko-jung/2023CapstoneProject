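; BP_FloatingTile is a map tile actor that drifts back and forth and can collapse into a fractured version.
; On BeginPlay it drops 200 units and picks a random speed, then sets its endpoints using MovementOffset.
; Tick eases it toward the current target with VInterpTo, swapping targets when within 50 units.
; DoCollapse stops ticking, hides and disables the static mesh, then spawns a Geometry Collection component in its place.
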(event `self.ReceiveBeginPlay`
  (bind _returnvalue (`self.K2_GetActorLocation`))
  (set `self.Speed` (`KismetMathLibrary.RandomFloatInRange` 0.5 0.7))
  (`self.K2_SetActorLocation` (- (`self.K2_GetActorLocation`) (0.0 0.0 200.0)))
  (set `self.Init Start Location` _returnvalue)
  (bind _output_get (set `self.Init End Location` (+ _returnvalue (`self.Movement Offset`))))
  (set `self.Target Location` _output_get)
  (set `self.Move To End?` true))

(event `self.ReceiveTick`
  (params (DeltaSeconds :type "Float (single-precision)"))
  (`self.K2_SetActorLocation` (`KismetMathLibrary.VInterpTo` (`self.K2_GetActorLocation`) (`self.Target Location`) (`GameplayStatics.GetWorldDeltaSeconds`) (`self.Speed`)))
  (if (< (`KismetMathLibrary.VSize` (- (`self.Target Location`) (`self.K2_GetActorLocation`))) 50.0)
    (if (`self.Move To End?`)
      (set `self.Target Location` (`self.Init Start Location`))
      (else
        (set `self.Target Location` (`self.Init End Location`))))
    (set `self.Move To End?` (not (`self.Move To End?`)))))

(event `/Game/2019180031/BlueprintInterface/BPI_Collapse.DoCollapse`
  (bind _staticmesh (`self.StaticMesh`))
  (`self.SetActorTickEnabled` false)
  (`SceneComponent.SetHiddenInGame` _staticmesh true false)
  (`PrimitiveComponent.SetSimulatePhysics` _staticmesh false)
  (`PrimitiveComponent.SetCollisionEnabled` _staticmesh "NoCollision")
  (`AddComponent|NODE_AddGeometryCollectionComponent-0` :`RelativeTransform` (`KismetMathLibrary.MakeTransform` (0.0 0.0 0.0) (struct) (0.9 0.9 0.9))))

(fn `UserConstructionScript`)