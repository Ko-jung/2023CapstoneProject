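; Base player character prototype with Enhanced Input move and look, a keyboard-layout widget and camera pitch limits.
; Components handle the gameplay: health takes damage, the weapon system takes stiffness and knockdown, the jetpack hears landings, and overlapped items apply effects.
; Montages relay through server then client events, with a greatsword blend-out callback.
; Respawn spawns a replacement at Team1 respawn points, copies weapon selections, transfers possession and destroys itself.
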(event `self.ReceiveBeginPlay`
  ;[1 1 1] Begin Play
  (bind _asplayer_controller (cast `PlayerController` (`self.GetController`)))
  (`EnhancedInputSubsystemInterface.AddMappingContext` (pcsubsystem `EnhancedInputLocalPlayerSubsystem` _asplayer_controller) "/Game/DeleteLater_ThirdPerson/Input/IMC_Default.IMC_Default" 0 (struct))
  (`self.SetCameraYawPitchAngle`)
  (cast `PlayerController` (`self.GetController`))
  (`|AddComponentByClass` "/Game/2019180031/Components/GameTimerComponent/Player_GameTimerComponent.Player_GameTimerComponent_C")
  (bind _returnvalue (`|CreateWidget` "/Game/2019180031/WidgetUI/WBP_KeyboardLayOut.WBP_KeyboardLayOut_C"))
  (`UserWidget.AddToViewport` _returnvalue 0))

(event `EnhancedInput|/Game/DeleteLater_ThirdPerson/Input/Actions/IA_Jump`
  (params (ActionValue :type Boolean) (ElapsedSeconds :type "Float (double-precision)") (TriggeredSeconds :type "Float (double-precision)") (InputAction :type "InputAction Object Reference" :default "/Game/DeleteLater_ThirdPerson/Input/Actions/IA_Jump.IA_Jump"))
  ;[1 1 1] IA_Jump
)

(event `EnhancedInput|/Game/DeleteLater_ThirdPerson/Input/Actions/IA_Move`
  (params (ActionValue :type "Vector2D Structure") (ElapsedSeconds :type "Float (double-precision)") (TriggeredSeconds :type "Float (double-precision)") (InputAction :type "InputAction Object Reference" :default "/Game/DeleteLater_ThirdPerson/Input/Actions/IA_Move.IA_Move"))
  ;[1 1 1] IA_Move
  (:`Triggered`
    (`|ExecutionSequence`
      (:`then_0`
        (`self.AddMovementInput` (`self.GetActorForwardVector`) ActionValue_X) ; x축(전방) 이동
      )
      (:`then_1`
        (`self.AddMovementInput` (`self.GetActorRightVector`) ActionValue_Y) ; y축(오른쪽)  이동
      ))))

(event `EnhancedInput|/Game/DeleteLater_ThirdPerson/Input/Actions/IA_Look`
  (params (ActionValue :type "Vector2D Structure") (ElapsedSeconds :type "Float (double-precision)") (TriggeredSeconds :type "Float (double-precision)") (InputAction :type "InputAction Object Reference" :default "/Game/DeleteLater_ThirdPerson/Input/Actions/IA_Look.IA_Look"))
  ;[1 1 1] IA_Look
  (:`Triggered`
    (`|ExecutionSequence`
      (:`then_0`
        (`self.AddControllerYawInput` ActionValue_X))
      (:`then_1`
        (`self.AddControllerPitchInput` ActionValue_Y)))))

(event `self.OnLanded`
  (params (Hit :type "HitResult Structure (by ref)"))
  (`/Game/2019180031/Components/JetpackComponent.OnLandJetPack` (`self.JetpackComponent`))
  (set `MovementComponent.Velocity` (0.0 0.0 0.0) (`self.CharacterMovement`)))

(event `self.CapsuleComponent.OnComponentBeginOverlap`
  (params (OverlappedComponent :type "PrimitiveComponent Object Reference") (OtherActor :type "Actor Object Reference") (OtherComp :type "PrimitiveComponent Object Reference") (OtherBodyIndex :type Integer) (bFromSweep :type Boolean) (SweepResult :type "HitResult Structure (by ref)"))
  (message `/Game/2019180031/BlueprintInterface/BPI_Item.DoItemEffect` OverlappedComponent self))

(event `/Game/2019180031/BlueprintInterface/BPI_CanstiffnessAndDown.Do Stiffness`
  (params (StiffnessTime :type "Float (double-precision)"))
  ;[1 1 1] Stiffness
  (`/Game/2019180031/Components/CombatSystemComponent/BP_CombatSystemComponent.Stiffness` (`self.WeaponSystemComponent`) StiffnessTime))

(event `self.ReceiveAnyDamage`
  (params (Damage :type "Float (single-precision)") (DamageType :type "DamageType Object Reference") (InstigatedBy :type "Controller Object Reference") (DamageCauser :type "Actor Object Reference"))
  ;[1 1 1] Any Damage
  (`/Game/2019180031/Components/HealthComponent/HealthComponent.Any Damage` (`self.HealthComponent`) Damage))

(event `/Game/2019180031/BlueprintInterface/BPI_CanstiffnessAndDown.Do Down`
  (params (DownDirection :type "Vector Structure"))
  ;[1 1 1] Down
  (`/Game/2019180031/Components/CombatSystemComponent/BP_CombatSystemComponent.Down` (`self.WeaponSystemComponent`) DownDirection))

(event `MyPlayMontage`
  (params (MontageToPlay :type "AnimMontage Object Reference") (PlayRate :type "Float (single-precision)"))
  (`self.MyPlayMontage On Server` MontageToPlay PlayRate))

(event `MyPlayMontageForGreatSword`
  (params (MontageToPlay :type "AnimMontage Object Reference") (PlayRate :type "Float (single-precision)"))
  (`self.MyPlayMontageForGreatSword On Server` MontageToPlay PlayRate))

(event `MyPlayMontage On Server`
  (params (MontageToPlay :type "AnimMontage Object Reference") (PlayRate :type "Float (single-precision)"))
  (`self.MyPlayMontage On Client` MontageToPlay PlayRate))

(event `MyPlayMontageForGreatSword On Server`
  (params (MontageToPlay :type "AnimMontage Object Reference") (PlayRate :type "Float (single-precision)"))
  (`self.MyPlayMontageForGreatSword On Client` MontageToPlay PlayRate))

(event `MyPlayMontage On Client`
  (params (MontageToPlay :type "AnimMontage Object Reference") (PlayRate :type "Float (single-precision)"))
  (`|PlayMontage` (`self.Mesh`) MontageToPlay PlayRate))

(event `MyPlayMontageForGreatSword On Client`
  (params (MontageToPlay :type "AnimMontage Object Reference") (PlayRate :type "Float (single-precision)"))
  (`|PlayMontage` (`self.Mesh`) MontageToPlay PlayRate
    (:`OnBlendOut`
      (`/Game/2019180031/Components/CombatSystemComponent/BP_CombatSystemComponent.GreatSword_OnBlendOut` (`self.WeaponSystemComponent`)))))

(fn `GetPlayerController`
  (returns (`Player Controller` :type "PlayerController Object Reference"))
  (bind _asplayer_controller (cast `PlayerController` (`self.GetController`)))
  (return _asplayer_controller))

(fn `RespawnCharacter`
  (bind _player_controller (`self.GetPlayerController`))
  (bind _player_controller_2 (`self.GetPlayerController`))
  (bind _returnvalue (`self.GetComponentByClass` "/Game/2019180031/Components/CombatSystemComponent/RangeAttack/BPMainRangeAttackComponent.BPMainRangeAttackComponent_C"))
  (bind _returnvalue_2 (`self.GetComponentByClass` "/Game/2019180031/Components/CombatSystemComponent/MeleeAtack/MainMeleeAttackComponent.MainMeleeAttackComponent_C"))
  (bind _weaponsystemcomponent (`self.WeaponSystemComponent`))
  (`|ExecutionSequence`
    (:`then_0`
      (`/Engine/EditorBlueprintResources/StandardMacros.IsValid` _returnvalue
        (:`Is Valid`
          (`ActorComponent.K2_DestroyComponent` _returnvalue))))
    (:`then_1`
      (`/Engine/EditorBlueprintResources/StandardMacros.IsValid` _returnvalue_2
        (:`Is Valid`
          (`ActorComponent.K2_DestroyComponent` _returnvalue_2))))
    (:`then_2`
      (`WidgetBlueprintLibrary.SetInputMode_GameOnly` _player_controller_2)
      (set `PlayerController.bShowMouseCursor` false _player_controller_2)
      (bind _outactors (`GameplayStatics.GetAllActorsOfClass` "/Game/2019180031/Blueprints/Respawn/BP_RespawnPosition.BP_RespawnPosition_C"))
      (for _array_element _outactors
        (if (`self.ActorHasTag` _array_element "Team1")
          (bind _returnvalue_3 (`|SpawnActorFromClass` (`GameplayStatics.GetObjectClass` self) (`KismetMathLibrary.MakeTransform` (`self.K2_GetActorLocation` _array_element)) "Undefined" "MultiplyWithRoot" null null))
          (bind _weaponsystemcomponent_2 (`/Game/2019180031/Character/BP_BasicPrototypeCharacter.WeaponSystemComponent` _returnvalue_3))
          (set `/Game/2019180031/Components/CombatSystemComponent/BP_CombatSystemComponent.Selected Melee Weapon` (`/Game/2019180031/Components/CombatSystemComponent/BP_CombatSystemComponent.Selected Melee Weapon` _weaponsystemcomponent) _weaponsystemcomponent_2)
          (set `/Game/2019180031/Components/CombatSystemComponent/BP_CombatSystemComponent.Selected Range Weapon` (`/Game/2019180031/Components/CombatSystemComponent/BP_CombatSystemComponent.Selected Range Weapon` _weaponsystemcomponent) _weaponsystemcomponent_2)
          (`Controller.UnPossess` _player_controller)
          (`Controller.Possess` _player_controller _returnvalue_3))))
    (:`then_3`
      (`self.K2_DestroyActor`))))

(fn `SetCameraYawPitchAngle`
  (bind _returnvalue (`GameplayStatics.GetPlayerCameraManager` 0))
  (set `PlayerCameraManager.ViewPitchMax` 60.0 _returnvalue)
  (set `PlayerCameraManager.ViewPitchMin` -50.0 _returnvalue))

(fn `UserConstructionScript`)