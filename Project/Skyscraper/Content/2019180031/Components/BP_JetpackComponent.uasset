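; Jetpack component for BP_BasicPrototypeCharacter that adds fuel-limited hovering, boosting and gliding, with a WBP_JetPack fuel gauge.
; Jump adds clamped upward velocity and Left Shift raises max speed, both entering zero-gravity Falling and draining fuel; release or empty fuel switches to low-gravity gliding.
; Left Ctrl exits hovering, and OnLandJetPack also refills fuel.
; DodgeJetpack launches horizontally then decelerates in a delay loop; its double-tap callers are unconnected.
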(event `Set Hovering Mode`
  (params (`To Hovering Mode` :type Boolean))
  (bind _returnvalue (`self.GetOwnerCharacterMovement`))
  (bind _returnvalue_2 (`self.GetOwnerCharacterMovement`))
  ;[0 0.09617 1] Hover Mode 바꾸기
  (if `To Hovering Mode`
    (`/Engine/EditorBlueprintResources/StandardMacros.DoOnce` false :!label _label
      (:`Completed`
        (set `/Game/2019180031/Character/BP_BasicPrototypeCharacter.IsHovering` true (`self.GetOwnerCharacter`))
        (set `CharacterMovementComponent.MaxWalkSpeed` (`self.HoveringMaxSpeed`) _returnvalue)
        (set `CharacterMovementComponent.GravityScale` 0.0 _returnvalue)
        (`CharacterMovementComponent.SetMovementMode` _returnvalue "MOVE_Falling" 0)
        (set `CharacterMovementComponent.MaxAcceleration` 50000.0 _returnvalue)))
    (else
      (set `/Game/2019180031/Character/BP_BasicPrototypeCharacter.IsHovering` false (`self.GetOwnerCharacter`))
      (set `CharacterMovementComponent.MaxWalkSpeed` 600.0 _returnvalue_2)
      (set `CharacterMovementComponent.GravityScale` 2.0 _returnvalue_2)
      (goto _label :!via `Reset`))))

(event `self.ReceiveBeginPlay`
  ;[0.2479 0.33 1] Begin Play - Set Widget
  (bind _returnvalue (`|CreateWidget` "/Game/2019180031/WidgetUI/WBP_JetPack.WBP_JetPack_C"))
  (set `self.WBP_Jetpack` _returnvalue)
  (`UserWidget.AddToViewport` _returnvalue 0)
  (set `self.JetPackFuel` (`self.MaxJetpackFuel`)))

(event `To Gliding Speed`
  ;[0 0.218 1] 글라이딩 속도로
  (set `CharacterMovementComponent.GravityScale` 0.5 (`self.GetOwnerCharacterMovement`)))

(event `EnhancedInput|/Game/DeleteLater_ThirdPerson/Input/Actions/IA_LShift`
  (params (ActionValue :type Boolean) (ElapsedSeconds :type "Float (double-precision)") (TriggeredSeconds :type "Float (double-precision)") (InputAction :type "InputAction Object Reference" :default "/Game/DeleteLater_ThirdPerson/Input/Actions/IA_LShift.IA_LShift"))
  (bind _returnvalue (`self.GetOwnerCharacterMovement`))
  ;[0 0.01766 1] LSHIFT - 빠르게 부스터
  (:`Triggered`
    (if (> (`self.JetPackFuel`) 0.0)
      (`self.Set Hovering Mode` true)
      (set `CharacterMovementComponent.MaxWalkSpeed` 1500.0 (`self.GetOwnerCharacterMovement`))
      (`self.Set Fuel` (- (`self.JetPackFuel`) (* (`GameplayStatics.GetWorldDeltaSeconds`) (`self.ShiftGaugePerSec`))))
      (else
        (`self.To Gliding Speed` :!label _label_2)
        (set `CharacterMovementComponent.MaxWalkSpeed` 600.0 _returnvalue)
        (set `MovementComponent.Velocity` (`self.ClampToMaxWalkSpeed` (`MovementComponent.Velocity` _returnvalue)) _returnvalue))))
  (:`Completed`
    (goto _label_2)))

(event `Set Fuel`
  (params (TargetValue :type "Float (double-precision)"))
  ;[0 0.09229 1] 제트팩 Fuel 조정
  (bind _output_get (set `self.JetPackFuel` (`KismetMathLibrary.FMax` TargetValue)))
  (`/Game/2019180031/WidgetUI/WBP_JetPack.Set Gauge Percent` (`self.WBP_Jetpack`) _output_get))

(event `EnhancedInput|/Game/DeleteLater_ThirdPerson/Input/Actions/IA_Jump`
  (params (ActionValue :type Boolean) (ElapsedSeconds :type "Float (double-precision)") (TriggeredSeconds :type "Float (double-precision)") (InputAction :type "InputAction Object Reference" :default "/Game/DeleteLater_ThirdPerson/Input/Actions/IA_Jump.IA_Jump"))
  (bind _returnvalue (`self.GetOwnerCharacterMovement`))
  (bind (_velocity_x _velocity_y _velocity_z) (`KismetMathLibrary.BreakVector` (`MovementComponent.Velocity` _returnvalue)))
  ;[0 0.0568 1] Floating JetPack
  (:`Triggered`
    (if (> (`self.JetPackFuel`) 0.0)
      (`self.Add JetPack Movement` (0.0 0.0 50.0) (`self.HoverGaugePerSec`))
      (goto _label_4 :!via `Reset`)
      (else
        (`self.To Gliding Speed` :!label _label_3)
        (`/Engine/EditorBlueprintResources/StandardMacros.DoOnce` false :!label _label_4
          (:`Completed`
            (set `MovementComponent.Velocity` (`KismetMathLibrary.MakeVector` _velocity_x _velocity_y (* _velocity_z 0.1)) _returnvalue))))))
  (:`Completed`
    (goto _label_3)))

(event `Key|LeftControl`
  (params (Key :type "Key Structure"))
  ;[0 0.1602 1] Left Ctrl - 나중에 Input Action 으로 바꾸기
  (:`Pressed`
    (if true
      (`self.Set Hovering Mode` false))))

(event `Add JetPack Movement`
  (params (AddVelocity :type "Vector Structure") (FuelReduction :type "Float (double-precision)"))
  (bind _returnvalue (`self.GetOwnerCharacterMovement`))
  ;[0 0.2245 1] AddJetPackMovement
  (`self.Set Hovering Mode` true)
  (set `MovementComponent.Velocity` (`self.ClampToMaxWalkSpeed` (+ AddVelocity (`MovementComponent.Velocity` _returnvalue))) _returnvalue)
  (`self.Set Fuel` (- (`self.JetPackFuel`) (* (`GameplayStatics.GetWorldDeltaSeconds`) FuelReduction))))

(event `Dodge Jetpack`
  (params (FwdInput :type "Float (double-precision)") (RightInput :type "Float (double-precision)") (DodgeStartSpeed :type "Float (double-precision)") (Deceleration :type "Float (double-precision)"))
  (bind _returnvalue (`self.GetOwnerCharacterMovement`))
  (bind _returnvalue_2 (`self.GetOwnerCharacterMovement`))
  (bind _returnvalue_3 (`Pawn.GetControlRotation` (`self.GetOwnerCharacter`)))
  (if (> (`self.JetPackFuel`) 0.1)
    (`|ExecutionSequence`
      (:`then_0`
        ;[1 1 1] Dodge - Initial Settings
        (set `CharacterMovementComponent.GravityScale` 0.0 (`self.GetOwnerCharacterMovement`)) ; Initial Settings
        (`Actor.K2_SetActorLocation` (`self.GetOwnerCharacter`) (+ (`Actor.K2_GetActorLocation` (`self.GetOwnerCharacter`)) (0.0 0.0 3.0)) false false)
        (`Character.LaunchCharacter` (`self.GetOwnerCharacter`) (* (`KismetMathLibrary.Normal` (+ (* (`KismetMathLibrary.GetForwardVector` _returnvalue_3) FwdInput) (* (`KismetMathLibrary.GetRightVector` _returnvalue_3) RightInput))) DodgeStartSpeed (1.0 1.0 0.0)) false false)
        (`self.Set Fuel` (- (`self.JetPackFuel`) 0.3)))
      (:`then_1`
        ;[1 1 1] Dodge - Logic (Decelation)
        (`KismetSystemLibrary.Delay` 0.2) ; Logic
        (if (< (`KismetMathLibrary.VSize` (`MovementComponent.Velocity` _returnvalue)) 600.0) :!label _label_5
          (set `CharacterMovementComponent.GravityScale` 1.0 _returnvalue)
          (else
            (`KismetSystemLibrary.Delay` 0.1)
            (set `MovementComponent.Velocity` (* (`MovementComponent.Velocity` _returnvalue_2) Deceleration) _returnvalue_2)
            (goto _label_5)))))))

(fn `ClampToMaxWalkSpeed`
  (params (`Now Velocity` :type "Vector Structure"))
  (returns (OutVelocity :type "Vector Structure"))
  (bind _maxwalkspeed (`CharacterMovementComponent.MaxWalkSpeed` (`self.GetOwnerCharacterMovement`)))
  (if (> (`KismetMathLibrary.VSize` `Now Velocity`) _maxwalkspeed)
    (return (* (`KismetMathLibrary.Normal` `Now Velocity`) _maxwalkspeed))
    (else
      (return `Now Velocity`))))

(fn `GetOwnerCharacter`
  (returns (OwnerCharacter :type "/Game/2019180031/Character/BP_BasicPrototypeCharacter Object Reference"))
  (bind _asbp_basic_prototype_character (cast `/Game/2019180031/Character/BP_BasicPrototypeCharacter` (`self.GetOwner`)))
  (return _asbp_basic_prototype_character))

(fn `GetOwnerCharacterMovement`
  (returns (ReturnValue :type "CharacterMovementComponent Object Reference"))
  (bind _asbp_basic_prototype_character (cast `/Game/2019180031/Character/BP_BasicPrototypeCharacter` (`self.GetOwner`))
    (:`then`
      (return (`Character.CharacterMovement` _asbp_basic_prototype_character)))
    (:`CastFailed`
      (return null))))

(fn `OnLandJetPack`
  (`self.Set Fuel` (`self.MaxJetpackFuel`))
  (`self.Set Hovering Mode` false))