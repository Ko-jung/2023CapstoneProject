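; Combat component for BP_BasicPrototypeCharacter that handles weapon swapping, hold-to-lock-on aiming and a stiffness hit-reaction montage.
; Number keys call SwapWeapon, which removes the current melee or range attack component and adds the chosen class at runtime.
; Lock-on picks the character nearest screen center and interpolates control rotation toward it, faster just after the press.
; Older enum-based weapon-actor switching, combo attack and knockdown logic remains but is mostly disconnected.
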(event `self.ReceiveBeginPlay`
  (bind _playercontroller (`self.GetOwnerPlayerController`))
  ;[0 0.2555 1] BeginPlay
  (`/Engine/EditorBlueprintResources/StandardMacros.IsValid` _playercontroller
    (:`Is Valid`
      (`EnhancedInputSubsystemInterface.AddMappingContext` (pcsubsystem `EnhancedInputLocalPlayerSubsystem` _playercontroller) "/Game/2019180031/MainGame/Core/Input/Combat/IMC_CombatSystem.IMC_CombatSystem" 0 (struct)))))

(event `self.ReceiveEndPlay`
  (params (EndPlayReason :type "EEndPlayReason Enum" :default "Destroyed"))
  (bind _playercontroller (`self.GetOwnerPlayerController`))
  (`/Engine/EditorBlueprintResources/StandardMacros.IsValid` _playercontroller
    (:`Is Valid`
      (`EnhancedInputSubsystemInterface.RemoveMappingContext` (pcsubsystem `EnhancedInputLocalPlayerSubsystem` _playercontroller) "/Game/2019180031/MainGame/Core/Input/Combat/IMC_CombatSystem.IMC_CombatSystem" (struct)))))

(event `Key|One`
  (params (Key :type "Key Structure"))
  (bind _selected_range_weapon (`self.Selected Range Weapon`))
  ;[1 1 1] 무기교체
  (:`Pressed`
    (`self.Swap Weapon` _selected_range_weapon)
    (`KismetSystemLibrary.PrintString` (`KismetTextLibrary.Conv_TextToString` (`|FormatText` "{comp} 무기 교체" (`KismetSystemLibrary.GetClassDisplayName` _selected_range_weapon))))))

(event `Key|Two`
  (params (Key :type "Key Structure"))
  (bind _selected_melee_weapon (`self.Selected Melee Weapon`))
  ;[1 1 1] 무기교체
  (:`Pressed`
    (`self.Swap Weapon` _selected_melee_weapon)
    (`KismetSystemLibrary.PrintString` (`KismetTextLibrary.Conv_TextToString` (`|FormatText` "{comp} 무기 교체" (`KismetSystemLibrary.GetClassDisplayName` _selected_melee_weapon))))))

(event `Key|Three`
  (params (Key :type "Key Structure"))
  ;[1 1 1] 무기교체
  (:`Pressed`
    (`self.Swap Weapon` null)
    (`KismetSystemLibrary.PrintString` "무기 벗기")))

(event `Change Weapon UI`
  (params (EWeaponState :type "/Game/2019180031/Components/CombatSystemComponent/EWeapon Enum (by ref)") (PlayerController :type "PlayerController Object Reference"))
  (bind _weaponui (`self.WeaponUI`))
  ;[0 0.2264 1] Change Weapon UI
  (`/Engine/EditorBlueprintResources/ActorComponentMacros.Switch Has Authority`
    (:`Remote`
      (`|ExecutionSequence`
        (:`then_0`
          (bind _weaponui_2 (`self.WeaponUI`)
            (:`then`
              (`Widget.RemoveFromParent` _weaponui_2)
              (set `self.WeaponUI` null))
            (:`else`)))
        (:`then_1`
          (switch `/Game/2019180031/Components/CombatSystemComponent/EWeapon` EWeaponState
            (:`NewEnumerator0`
              (bind _returnvalue (`|CreateWidget` "/Game/2019180031/WidgetUI/WBP_MainRangeUI.WBP_MainRangeUI_C" PlayerController))
              (set `self.WeaponUI` _returnvalue))
            (:`NewEnumerator1`
              (bind _returnvalue_2 (`|CreateWidget` "/Game/2019180031/WidgetUI/WBP_MainMeleeUI.WBP_MainMeleeUI_C" PlayerController))
              (set `self.WeaponUI` _returnvalue_2)))
          (`/Engine/EditorBlueprintResources/StandardMacros.IsValid` _weaponui
            (:`Is Valid`
              (`UserWidget.AddToViewport` _weaponui 0))))
        (:`then_2`
          (set `self.EWeaponState` EWeaponState))))))

(event `Stiffness`
  (params (StiffnessTime :type "Float (double-precision)"))
  ;[0.001685 1 0] Stiffness
  (if (not (== StiffnessTime 0.0))
    (`|PlayMontage` (`self.GetOwnerMeshComponent`) (`self.AM_Damaged`) (/ 1.0 StiffnessTime))))

(event `Key|Four`
  (params (Key :type "Key Structure"))
  ;[1 1 1] 무기교체
  (:`Pressed`
    (`self.Swap Weapon` "/Game/2019180031/Components/CombatSystemComponent/RangeAttack/RPG-7Component.RPG-7Component_C")
    (`KismetSystemLibrary.PrintString` "RPG-7 무기 교체")))

(event `Key|Five`
  (params (Key :type "Key Structure"))
  ;[1 1 1] 무기교체
  (:`Pressed`
    (`self.Swap Weapon` "/Game/2019180031/Components/CombatSystemComponent/MeleeAtack/KatanaAttackComponent.KatanaAttackComponent_C")
    (`KismetSystemLibrary.PrintString` "카타나 무기 교체")))

(event `Down`
  (params (DownDirection :type "Vector Structure"))
  ;[0.001685 1 0] Down
)

(event `Key|Six`
  (params (Key :type "Key Structure"))
  ;[1 1 1] 무기교체
  (:`Pressed`
    (`self.Swap Weapon` "/Game/2019180031/Components/CombatSystemComponent/RangeAttack/RifleComponent.RifleComponent_C")
    (`KismetSystemLibrary.PrintString` "라이플 무기 교체")))

(event `Key|Seven`
  (params (Key :type "Key Structure"))
  ;[1 1 1] 무기교체
  (:`Pressed`
    (`self.Swap Weapon` "/Game/2019180031/Components/CombatSystemComponent/MeleeAtack/GreatSwordAttackComponent.GreatSwordAttackComponent_C")
    (`KismetSystemLibrary.PrintString` "대검 무기 교체")))

(event `Key|Eight`
  (params (Key :type "Key Structure"))
  ;[1 1 1] 무기교체
  (:`Pressed`
    (`self.Swap Weapon` "/Game/2019180031/Components/CombatSystemComponent/RangeAttack/SMGComponent.SMGComponent_C")
    (`KismetSystemLibrary.PrintString` "기관단총 무기 교체")))

(event `Key|Nine`
  (params (Key :type "Key Structure"))
  ;[1 1 1] 무기교체
  (:`Pressed`
    (`self.Swap Weapon` "/Game/2019180031/Components/CombatSystemComponent/MeleeAtack/DaggerAttackComponent.DaggerAttackComponent_C")
    (`KismetSystemLibrary.PrintString` "단감 무기 교체")))

(event `EnhancedInput|/Game/2019180031/MainGame/Core/Input/Combat/IA_LockOn`
  (params (ActionValue :type Boolean) (ElapsedSeconds :type "Float (double-precision)") (TriggeredSeconds :type "Float (double-precision)") (InputAction :type "InputAction Object Reference" :default "/Game/2019180031/MainGame/Core/Input/Combat/IA_LockOn.IA_LockOn"))
  ;[1 1 1] 우클릭 / IA_LockOn
  (:`Triggered`
    (`self.LockOn`))
  (:`Started`
    (set `self.LockOnStartTime` (`KismetSystemLibrary.GetGameTimeInSeconds`)))
  (:`Completed`
    (set `self.LockOnActor` null)
    (set `self.Close Target Distance` (`self.Init Target Distance`))))

(event `LockOn`
  (bind _playercontroller (`self.GetOwnerPlayerController`))
  (bind _returnvalue (`WidgetLayoutLibrary.GetViewportSize`))
  ;[1 1 1] 락온 / 우클릭 / LockOn
  (set `self.Count Lock on Player` 0)
  (bind _outactors (`GameplayStatics.GetAllActorsOfClass` "/Game/2019180031/Character/BP_BasicPrototypeCharacter.BP_BasicPrototypeCharacter_C")) ; 락온 대상 - BP_BasicProtoCharacter
  (for _array_element _outactors
    (if (!= (`self.GetOwner`) _array_element)
      (bind _returnvalue_2 (`KismetMathLibrary.Distance2D` (`GameplayStatics.ProjectWorldToScreen` (`self.GetOwnerPlayerController`) (`Actor.K2_GetActorLocation` _array_element)) (/ _returnvalue 2.0)))
      (if (< _returnvalue_2 (/ (`KismetMathLibrary.BreakVector2D` _returnvalue) 10.0))
        (`/Engine/EditorBlueprintResources/StandardMacros.IncrementInt` (`self.Count Lock on Player`)
          (:`  `
            (if (< _returnvalue_2 (`self.Close Target Distance`))
              (set `self.LockOnActor` _array_element)
              (set `self.Close Target Distance` _returnvalue_2)))))))
  (`|ExecutionSequence`
    (:`then_0`
      (if (== (`self.Count Lock on Player`) 0)
        (set `self.Close Target Distance` (`self.Init Target Distance`))
        (set `self.LockOnActor` null)))
    (:`then_1`
      (`self.LockOnActor` ; 락온 액터 있을 시 해당 액터로 락온
        (:`then`
          (if (< (- (`KismetSystemLibrary.GetGameTimeInSeconds`) (`self.LockOnStartTime`)) 0.5)
            (set `self.Lock on Speed` 20.0)
            (else
              (set `self.Lock on Speed` 2.0)))
          (`Controller.SetControlRotation` _playercontroller (`KismetMathLibrary.RInterpTo` (`Controller.GetControlRotation` _playercontroller) (`KismetMathLibrary.Conv_VectorToRotator` (- (`Actor.K2_GetActorLocation` (`self.LockOnActor`)) (`SceneComponent.K2_GetComponentLocation` (`self.GetOwnerCameraComponent`)))) (`GameplayStatics.GetWorldDeltaSeconds`) (`self.Lock on Speed`))))
        (:`else`)))))

(event `EnhancedInput|/Game/DeleteLater_ThirdPerson/Input/Actions/IA_RightClick`
  (params (ActionValue :type Boolean) (ElapsedSeconds :type "Float (double-precision)") (TriggeredSeconds :type "Float (double-precision)") (InputAction :type "InputAction Object Reference" :default "/Game/DeleteLater_ThirdPerson/Input/Actions/IA_RightClick.IA_RightClick"))
  ;[0 1 0.09229] 우클릭 - 유실물
)

(event `Key|MouseScrollDown`
  (params (Key :type "Key Structure"))
  ;[1 1 1] Swap Weapon By Wheel - 유실물
)

(event `Key|MouseScrollUp`
  (params (Key :type "Key Structure"))
  ;[1 1 1] Swap Weapon By Wheel - 유실물
)

(event `Spawn Weapon On Server`
  (params (Class :type "Actor Class Reference") (Parent :type "SceneComponent Object Reference") (SocketName :type Name))
  ;[0 0.1266 1] Change Weapon - 유실물
  (bind _returnvalue (`|SpawnActorFromClass` Class (`KismetMathLibrary.MakeTransform` (0.0 0.0 0.0)) "Undefined" "MultiplyWithRoot" null null))
  (`Actor.K2_AttachToComponent` _returnvalue Parent SocketName "KeepRelative" "KeepRelative" "KeepRelative" true)
  (`self.SetWeaponActor` _returnvalue))

(event `SetWeaponActor`
  (params (WeaponActor :type "Actor Object Reference (by ref)"))
  ;[0 0.1266 1] Change Weapon - 유실물
  (`/Engine/EditorBlueprintResources/ActorComponentMacros.Switch Has Authority`
    (:`Authority`
      (set `self.WeaponActor` WeaponActor))))

(event `GreatSword_OnBlendOut`
  ;[0 0.3357 1] 대검 콤보공격 로직 - 유기
  (set `self.LastLeftClickTime` (`GameplayStatics.GetTimeSeconds`)))

(event `Destroy Weapon On Server`
  (params (Actor :type "Actor Object Reference (by ref)"))
  ;[0 0.1266 1] Change Weapon - 유실물
  (`Actor.K2_DestroyActor` Actor))

(event `Key|One`
  (params (Key :type "Key Structure"))
  ;[0 0.2858 1] Swap Weapon - 유실물
)

(event `Change Weapon`
  (params (ChangeTo :type "/Game/2019180031/Components/CombatSystemComponent/EWeapon Enum" :default "NewEnumerator0"))
  ;[0 0.1266 1] Change Weapon - 유실물
  (if (`|EnumInequality` ChangeTo (`self.EWeaponState`))
    (`|ExecutionSequence`
      (:`then_0`
        (bind _weaponactor (`self.WeaponActor`)
          (:`then`
            (`self.Destroy Weapon On Server` _weaponactor))
          (:`else`)))
      (:`then_1`
        (bind _output_get (set `self.EWeaponState` ChangeTo))
        (switch `/Game/2019180031/Components/CombatSystemComponent/EWeapon` _output_get
          (:`NewEnumerator0`
            (`self.Spawn Weapon On Server` "/Game/2019180031/StaticMesh/Weapon_StaticMesh/Rifle/BP_Rifle.BP_Rifle_C" (`self.GetOwnerMeshComponent`) "RifleSocket"))
          (:`NewEnumerator1`
            (`self.Spawn Weapon On Server` "/Game/2019180031/StaticMesh/Weapon_StaticMesh/GreatSword/BP_GreatSword.BP_GreatSword_C" (`self.GetOwnerMeshComponent`) "GreatSwordSocket"))
          (:`NewEnumerator4`
            _))
        (`self.Change Weapon UI` (`self.EWeaponState`) (`self.GetOwnerPlayerController`))))))

(event `Key|Two`
  (params (Key :type "Key Structure"))
  ;[0 0.2858 1] Swap Weapon - 유실물
)

(event `Key|Three`
  (params (Key :type "Key Structure"))
  ;[0 0.2858 1] Swap Weapon - 유실물
)

(fn `GetOwnerCameraComponent`
  (returns (CameraComponent :type "CameraComponent Object Reference"))
  (bind _asbp_basic_prototype_character (cast `/Game/2019180031/Character/BP_BasicPrototypeCharacter` (`self.GetOwner`))
    (:`then`
      (return (`/Game/2019180031/Character/BP_BasicPrototypeCharacter.Camera` _asbp_basic_prototype_character)))
    (:`CastFailed`
      (return null))))

(fn `GetOwnerCharacter`
  (returns (OwnerCharacter :type "/Game/2019180031/Character/BP_BasicPrototypeCharacter Object Reference"))
  (bind _asbp_basic_prototype_character (cast `/Game/2019180031/Character/BP_BasicPrototypeCharacter` (`self.GetOwner`))
    (:`then`
      (return _asbp_basic_prototype_character))
    (:`CastFailed`
      (return null))))

(fn `GetOwnerCharacterMovementComponent`
  (returns (CharacterMovementComponent :type "CharacterMovementComponent Object Reference"))
  (bind _asbp_basic_prototype_character (cast `/Game/2019180031/Character/BP_BasicPrototypeCharacter` (`self.GetOwner`))
    (:`then`
      (return (`Character.CharacterMovement` _asbp_basic_prototype_character)))
    (:`CastFailed`
      (return null))))

(fn `GetOwnerMeshComponent`
  (returns (OwnerMeshComponent :type "SkeletalMeshComponent Object Reference"))
  (bind _asbp_basic_prototype_character (cast `/Game/2019180031/Character/BP_BasicPrototypeCharacter` (`self.GetOwner`))
    (:`then`
      (return (`Character.Mesh` _asbp_basic_prototype_character)))
    (:`CastFailed`
      (return null))))

(fn `GetOwnerMotionWarpingComponent`
  (returns (MotionWarping :type "MotionWarpingComponent Object Reference"))
  (bind _asbp_basic_prototype_character (cast `/Game/2019180031/Character/BP_BasicPrototypeCharacter` (`self.GetOwner`))
    (:`then`
      (return (`/Game/2019180031/Character/BP_BasicPrototypeCharacter.MotionWarping` _asbp_basic_prototype_character)))
    (:`CastFailed`
      (return null))))

(fn `GetOwnerPlayerController`
  (returns (PlayerController :type "PlayerController Object Reference"))
  (bind _asbp_basic_prototype_character (cast `/Game/2019180031/Character/BP_BasicPrototypeCharacter` (`self.GetOwner`))
    (:`then`
      (bind _asplayer_controller (cast `PlayerController` (`Pawn.GetController` _asbp_basic_prototype_character))
        (:`then`
          (return _asplayer_controller))
        (:`CastFailed`
          _)))
    (:`CastFailed`
      _))
  (return null))

(fn `GetOwnerSpringArmComponent`
  (returns (SpringArm :type "SpringArmComponent Object Reference"))
  (bind _asbp_basic_prototype_character (cast `/Game/2019180031/Character/BP_BasicPrototypeCharacter` (`self.GetOwner`))
    (:`then`
      (return (`/Game/2019180031/Character/BP_BasicPrototypeCharacter.SpringArm` _asbp_basic_prototype_character)))
    (:`CastFailed`
      (return null))))

(fn `Swap Weapon`
  (params (Class :type "ActorComponent Class Reference"))
  (`|ExecutionSequence`
    (:`then_0`
      (bind _mainweaponcomponent (`self.MainWeaponComponent`) ; 기존 무기 컴퍼넌트가 존재한다면 삭제
        (:`then`
          (bind _asmain_melee_attack_component (cast `/Game/2019180031/Components/CombatSystemComponent/MeleeAtack/MainMeleeAttackComponent` _mainweaponcomponent)
            (:`then`
              (`/Game/2019180031/Components/CombatSystemComponent/MeleeAtack/MainMeleeAttackComponent.RemoveComponent` _asmain_melee_attack_component)
              (set `self.MainWeaponComponent` null))
            (:`CastFailed`
              (bind _asmain_range_attack_component (cast `/Game/2019180031/Components/CombatSystemComponent/RangeAttack/MainRangeAttackComponent` _mainweaponcomponent))
              (`/Game/2019180031/Components/CombatSystemComponent/RangeAttack/MainRangeAttackComponent.RemoveComponent` _asmain_range_attack_component)
              (set `self.MainWeaponComponent` null))))
        (:`else`)))
    (:`then_1`
      (if (`KismetSystemLibrary.IsValidClass` Class)
        (bind _returnvalue (`|AddComponentByClass` (`self.GetOwner`) Class))
        (set `self.MainWeaponComponent` _returnvalue)))))