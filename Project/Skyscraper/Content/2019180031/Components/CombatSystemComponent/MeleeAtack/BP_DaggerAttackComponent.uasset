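; Dagger melee attack component that gives the owning player dagger attack input and a melee UI.
; On BeginPlay it adds the main melee input mapping context and widget for a valid owner controller, and removes both on EndPlay.
; The attack input calls Attack, while five DaggerAttack functions define hits through CreateAttackArea with progressively larger areas.
; The first four hits apply stiffness, and the fifth knocks down.
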(event `self.ReceiveBeginPlay`
  (bind _playercontroller (`self.GetOwnerPlayerController`))
  (`/Engine/EditorBlueprintResources/StandardMacros.IsValid` _playercontroller
    (:`Is Valid`
      (`EnhancedInputSubsystemInterface.AddMappingContext` (pcsubsystem `EnhancedInputLocalPlayerSubsystem` _playercontroller) "/Game/2019180031/MainGame/Core/Input/Combat/Melee/IMC_MainMeleeInput.IMC_MainMeleeInput" 0 (struct))
      (bind _returnvalue (`|CreateWidget` "/Game/2019180031/WidgetUI/WBP_MainMeleeUI.WBP_MainMeleeUI_C"))
      (`UserWidget.AddToViewport` _returnvalue 0)
      (set `self.MeleeAttackUI` _returnvalue)
      (`KismetSystemLibrary.PrintString` "단검 컴퍼넌트 제작"))))

(event `self.ReceiveEndPlay`
  (params (EndPlayReason :type "EEndPlayReason Enum" :default "Destroyed"))
  (bind _playercontroller (`self.GetOwnerPlayerController`))
  (`parent.ReceiveEndPlay` "Destroyed")
  (`/Engine/EditorBlueprintResources/StandardMacros.IsValid` _playercontroller
    (:`Is Valid`
      (`EnhancedInputSubsystemInterface.RemoveMappingContext` (pcsubsystem `EnhancedInputLocalPlayerSubsystem` _playercontroller) "/Game/2019180031/MainGame/Core/Input/Combat/Melee/IMC_MainMeleeInput.IMC_MainMeleeInput" (struct))
      (`Widget.RemoveFromParent` (`self.MeleeAttackUI`))
      (`KismetSystemLibrary.PrintString` "단검 컴퍼넌트 지워짐"))))

(event `EnhancedInput|/Game/2019180031/MainGame/Core/Input/Combat/Melee/IA_Attack`
  (params (ActionValue :type Boolean) (ElapsedSeconds :type "Float (double-precision)") (TriggeredSeconds :type "Float (double-precision)") (InputAction :type "InputAction Object Reference" :default "/Game/2019180031/MainGame/Core/Input/Combat/Melee/IA_Attack.IA_Attack"))
  (:`Triggered`
    (`self.Attack`)))

(fn `DaggerAttack1`
  (`self.CreateAttackArea` (1.0 20.0 20.0) 0.5 120.0 true))

(fn `DaggerAttack2`
  (`self.CreateAttackArea` (1.0 25.0 25.0) 0.5 120.0 true))

(fn `DaggerAttack3`
  (`self.CreateAttackArea` (1.0 30.0 30.0) 0.5 120.0 true))

(fn `DaggerAttack4`
  (`self.CreateAttackArea` (1.0 35.0 35.0) 0.7 120.0 true))

(fn `DaggerAttack5`
  (`self.CreateAttackArea` (1.0 40.0 40.0) 0.4 120.0 false true))