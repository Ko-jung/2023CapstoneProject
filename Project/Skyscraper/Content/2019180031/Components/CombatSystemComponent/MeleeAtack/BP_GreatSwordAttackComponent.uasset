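; Greatsword attack component that gives a player-controlled owner melee input and UI while it is active.
; On BeginPlay it adds the main melee input mapping context, creates the melee widget and prints a debug equip message.
; IA_Attack calls Attack, whose logic is not defined in this graph.
; EndPlay runs the parent logic, then removes the mapping context and widget and prints a removal message.
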(event `self.ReceiveBeginPlay`
  (bind _playercontroller (`self.GetOwnerPlayerController`))
  (`/Engine/EditorBlueprintResources/StandardMacros.IsValid` _playercontroller
    (:`Is Valid`
      (`EnhancedInputSubsystemInterface.AddMappingContext` (pcsubsystem `EnhancedInputLocalPlayerSubsystem` _playercontroller) "/Game/2019180031/MainGame/Core/Input/Combat/Melee/IMC_MainMeleeInput.IMC_MainMeleeInput" 0 (struct))
      (bind _returnvalue (`|CreateWidget` "/Game/2019180031/WidgetUI/WBP_MainMeleeUI.WBP_MainMeleeUI_C"))
      (`UserWidget.AddToViewport` _returnvalue 0)
      (set `self.MeleeAttackUI` _returnvalue)
      (`KismetSystemLibrary.PrintString` "대검 컴퍼넌트 장착"))))

(event `self.ReceiveEndPlay`
  (params (EndPlayReason :type "EEndPlayReason Enum" :default "Destroyed"))
  (bind _playercontroller (`self.GetOwnerPlayerController`))
  (`parent.ReceiveEndPlay` "Destroyed")
  (`/Engine/EditorBlueprintResources/StandardMacros.IsValid` _playercontroller
    (:`Is Valid`
      (`EnhancedInputSubsystemInterface.RemoveMappingContext` (pcsubsystem `EnhancedInputLocalPlayerSubsystem` _playercontroller) "/Game/2019180031/MainGame/Core/Input/Combat/Melee/IMC_MainMeleeInput.IMC_MainMeleeInput" (struct))
      (`Widget.RemoveFromParent` (`self.MeleeAttackUI`))
      (`KismetSystemLibrary.PrintString` "대검 컴퍼넌트 지워짐"))))

(event `EnhancedInput|/Game/2019180031/MainGame/Core/Input/Combat/Melee/IA_Attack`
  (params (ActionValue :type Boolean) (ElapsedSeconds :type "Float (double-precision)") (TriggeredSeconds :type "Float (double-precision)") (InputAction :type "InputAction Object Reference" :default "/Game/2019180031/MainGame/Core/Input/Combat/Melee/IA_Attack.IA_Attack"))
  (:`Triggered`
    (`self.Attack`)))