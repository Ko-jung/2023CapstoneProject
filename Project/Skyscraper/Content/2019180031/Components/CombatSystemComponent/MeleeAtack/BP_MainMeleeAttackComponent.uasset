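; Base melee attack component for BP_BasicPrototypeCharacter that runs a montage-based combo and deals hit damage.
; Attack steps through ComboAnimMontage, resetting the combo after a half-second gap, and unlocks when the montage blends out.
; A motion warp target scales each attack's forward lunge by held W/S input.
; CreateAttackArea box-traces ahead, applying damage plus optional stiffness and knockdown messages, with debug drawing left on.
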(event `Play Melee Anim Montage`
  (params (MontageToPlay :type "AnimMontage Object Reference") (PlayRate :type "Float (single-precision)"))
  (bind _ownercharacter (`self.GetOwnerCharacter`))
  (bind _animationmovementaxis (`self.AnimationMovementAxis`))
  (bind _returnvalue (`Actor.K2_GetActorLocation` _ownercharacter))
  (bind _returnvalue_2 (+ _returnvalue (* (`Actor.GetActorForwardVector` _ownercharacter) (`self.AnimationMovementDistance`) _animationmovementaxis)))
  ;[1 1 1] 키 입력에 따른 이동 로직
  (set `self.AnimationMovementAxis` 1)
  (`|ExecutionSequence`
    (:`then_0`
      (if (`PlayerController.IsInputKeyDown` (`self.GetOwnerPlayerController`) "W")
        (`/Engine/EditorBlueprintResources/StandardMacros.IncrementInt` (`self.AnimationMovementAxis`))))
    (:`then_1`
      (if (`PlayerController.IsInputKeyDown` (`self.GetOwnerPlayerController`) "S")
        (`/Engine/EditorBlueprintResources/StandardMacros.DecrementInt` (`self.AnimationMovementAxis`))))
    (:`then_2`
      (`KismetSystemLibrary.DrawDebugLine` _returnvalue _returnvalue_2 (struct) 3.0 10.0)
      (`MotionWarpingComponent.AddOrUpdateWarpTargetFromLocation` (`self.GetOwnerMotionWarping`) "MeleeMovement" _returnvalue_2)
      (`KismetSystemLibrary.PrintString` (`KismetStringLibrary.Conv_IntToString` _animationmovementaxis)))
    (:`then_3`
      (`|PlayMontage` (`self.GetOwnerMeshComponent`) MontageToPlay PlayRate
        (:`OnBlendOut`
          (set `self.CanAttack` true)
          (set `self.AttackClickTime` (`GameplayStatics.GetTimeSeconds`)))))))

(fn `Attack`
  (if (`self.CanAttack`)
    (if (not (< (- (`GameplayStatics.GetTimeSeconds`) (`self.AttackClickTime`)) 0.5))
      (set `self.AttackComboCount` 0))
    (`self.PlayAttackAnimMontage`)))

(fn `CreateAttackArea`
  (params (HitSize :type "Vector Structure") (StiffnessTime :type "Float (double-precision)") (BaseDamage :type "Float (single-precision)") (DoStiffness :type Boolean) (DoDown :type Boolean))
  (bind _returnvalue (`self.GetOwner`))
  (bind _returnvalue_2 (`Actor.K2_GetActorLocation` _returnvalue))
  (bind _outhits (`KismetSystemLibrary.BoxTraceMulti` :`Start` _returnvalue_2 :`End` (+ _returnvalue_2 (* (`Actor.GetActorForwardVector` _returnvalue) 150.0)) :`HalfSize` HitSize :`Orientation` (`Actor.K2_GetActorRotation` _returnvalue) :`TraceChannel` "TraceTypeQuery1" :`DrawDebugType` "ForDuration"))
  (for _array_element _outhits
    (`|ExecutionSequence`
      (:`then_0`
        (if DoStiffness
          (bind (_bblockinghit _binitialoverlap _time _distance _location _impactpoint _normal _impactnormal _physmat _hitactor) (`GameplayStatics.BreakHitResult` _array_element))
          (message `/Game/2019180031/BlueprintInterface/BPI_CanstiffnessAndDown.Do Stiffness` _hitactor StiffnessTime)))
      (:`then_1`
        (if DoDown
          (message `/Game/2019180031/BlueprintInterface/BPI_CanstiffnessAndDown.Do Down` _hitactor (`Actor.GetActorForwardVector` (`self.GetOwner`)))))
      (:`then_2`
        (`GameplayStatics.ApplyDamage` _hitactor BaseDamage)))))

(fn `GetOwnerCharacter`
  (returns (OwnerCharacter :type "/Game/2019180031/Character/BP_BasicPrototypeCharacter Object Reference"))
  (bind _asbp_basic_prototype_character (cast `/Game/2019180031/Character/BP_BasicPrototypeCharacter` (`self.GetOwner`))
    (:`then`
      (return _asbp_basic_prototype_character))
    (:`CastFailed`
      (return null))))

(fn `GetOwnerMeshComponent`
  (returns (OwnerMeshComponent :type "SkeletalMeshComponent Object Reference"))
  (bind _asbp_basic_prototype_character (cast `/Game/2019180031/Character/BP_BasicPrototypeCharacter` (`self.GetOwner`))
    (:`then`
      (return (`Character.Mesh` _asbp_basic_prototype_character)))
    (:`CastFailed`
      (return null))))

(fn `GetOwnerMotionWarping`
  (returns (MotionWarping :type "MotionWarpingComponent Object Reference"))
  (return (`/Game/2019180031/Character/BP_BasicPrototypeCharacter.MotionWarping` (`self.GetOwnerCharacter`))))

(fn `GetOwnerPlayerController`
  (returns (PlayerController :type "PlayerController Object Reference"))
  (bind _asbp_basic_prototype_character (cast `/Game/2019180031/Character/BP_BasicPrototypeCharacter` (`self.GetOwner`))
    (:`then`
      (bind _asplayer_controller (cast `PlayerController` (`Pawn.GetController` _asbp_basic_prototype_character))
        (:`then`
          (return _asplayer_controller))
        (:`CastFailed`
          _)))
    (:`CastFailed`
      _))
  (return null))

(fn `PlayAttackAnimMontage`
  (bind _comboanimmontage (`self.ComboAnimMontage`))
  (bind _value (`BlueprintMapLibrary.Map_Find` _comboanimmontage (`self.AttackComboCount`)))
  (`self.Play Melee Anim Montage` _value (/ (`AnimationAsset.GetPlayLength` _value) (`|GetArrayItem` (`self.AnimationSpeed`) (`self.AttackComboCount`))))
  (set `self.AttackComboCount` (mod (+ (`self.AttackComboCount`) 1) (`BlueprintMapLibrary.Map_Length` _comboanimmontage)))
  (set `self.CanAttack` false))

(fn `RemoveComponent`
  (`self.K2_DestroyComponent`))