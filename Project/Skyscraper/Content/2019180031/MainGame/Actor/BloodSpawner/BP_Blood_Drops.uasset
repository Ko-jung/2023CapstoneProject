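; Short-lived blood spray actor that leaves ground decals and wets characters where droplets land.
; Its Niagara effect exports particle positions, which move paired character and ground collision meshes along with the drops.
; Ground hits spawn randomly sized, fading blood decals; character hits trace for the collision UV and pass it to SkyscraperCharacter's LiquidWetComponent.
; Either hit disables that mesh and its index-matched partner.
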(event `self.ReceiveBeginPlay`
  (`NiagaraComponent.SetVariableObject` (`self.NS_Blood_Effect`) "BP_Blood" self)
  (`self.SetLifeSpan` 5.0)
  (for _array_element (`self.CollisionCheckMeshes`)
    (`/Engine/EditorBlueprintResources/StandardMacros.IsValid` _array_element
      (:`Is Valid`
        (add `PrimitiveComponent.OnComponentHit` _array_element (delegate `LiquidCollision_HitEvent`)))))
  (for _array_element_2 (`self.GroundCollisionCheckMeshes`)
    (`/Engine/EditorBlueprintResources/StandardMacros.IsValid` _array_element_2
      (:`Is Valid`
        (add `PrimitiveComponent.OnComponentHit` _array_element_2 (delegate `Ground Component Hit`))))))

(event `Ground Component Hit`
  (params (HitComponent :type "PrimitiveComponent Object Reference") (OtherActor :type "Actor Object Reference") (OtherComp :type "PrimitiveComponent Object Reference") (NormalImpulse :type "Vector Structure") (Hit :type "HitResult Structure (by ref)"))
  (bind (_bblockinghit _binitialoverlap _time _distance _location _impactpoint _normal) (`GameplayStatics.BreakHitResult` Hit))
  (bind _returnvalue (`GameplayStatics.SpawnDecalAtLocation` "/Game/2019180031/MainGame/Material/MF_Blood/M_Blood_Decal.M_Blood_Decal" (`KismetMathLibrary.Conv_DoubleToVector` (`KismetMathLibrary.RandomFloatInRange` 5.0 20.0)) _location (`KismetMathLibrary.Conv_VectorToRotator` (* _normal 1.0))))
  (`DecalComponent.SetFadeOut` _returnvalue 3.0 5.0 true)
  (`PrimitiveComponent.SetSimulatePhysics` HitComponent false)
  (`PrimitiveComponent.SetCollisionEnabled` HitComponent "NoCollision")
  (bind _asstatic_mesh_component (cast `StaticMeshComponent` HitComponent))
  (bind _returnvalue_2 (`KismetArrayLibrary.Array_Find` (`self.GroundCollisionCheckMeshes`) _asstatic_mesh_component))
  (if (!= _returnvalue_2 -1)
    (bind _output (`|GetArrayItem` (`self.CollisionCheckMeshes`) _returnvalue_2))
    (`PrimitiveComponent.SetSimulatePhysics` _output false)
    (`PrimitiveComponent.SetCollisionEnabled` _output "NoCollision")))

(event `LiquidCollision_HitEvent`
  (params (HitComponent :type "PrimitiveComponent Object Reference") (OtherActor :type "Actor Object Reference") (OtherComp :type "PrimitiveComponent Object Reference") (NormalImpulse :type "Vector Structure") (Hit :type "HitResult Structure (by ref)"))
  ;[1 1 1] Liquid Wet Component Hit
  (bind (_outhit _returnvalue) (`KismetSystemLibrary.LineTraceSingleForObjects` :`Start` (`self.K2_GetActorLocation`) :`End` (`.Location` (`GameplayStatics.BreakHitResult` Hit)) :`ObjectTypes` (`|MakeArray` "ObjectTypeQuery7" :!type "EObjectTypeQuery Enum") :`bTraceComplex` true :`DrawTime` 2.0))
  (if _returnvalue
    (bind _asskyscraper_character (cast `SkyscraperCharacter` OtherActor))
    (`LiquidWetComponent.AddHitData` (`SkyscraperCharacter.LiquidWetComponent` _asskyscraper_character) (`GameplayStatics.FindCollisionUV` _outhit) (`KismetMathLibrary.RandomFloatInRange` 4.0 6.0))
    (`PrimitiveComponent.SetSimulatePhysics` HitComponent false)
    (`PrimitiveComponent.SetCollisionEnabled` HitComponent "NoCollision")
    (bind _asstatic_mesh_component (cast `StaticMeshComponent` HitComponent))
    (bind _returnvalue_2 (`KismetArrayLibrary.Array_Find` (`self.CollisionCheckMeshes`) _asstatic_mesh_component))
    (if (!= _returnvalue_2 -1)
      (bind _output (`|GetArrayItem` (`self.GroundCollisionCheckMeshes`) _returnvalue_2))
      (`PrimitiveComponent.SetSimulatePhysics` _output false)
      (`PrimitiveComponent.SetCollisionEnabled` _output "NoCollision"))))

(event `self.ReceiveParticleData`
  (params (Data :type "Array of BasicParticleData Structure (by ref)") (NiagaraSystem :type "NiagaraSystem Object Reference") (SimulationPositionOffset :type "Vector Structure (by ref)"))
  (for (_array_element _array_index) Data
    (bind _output (`|GetArrayItem` (`self.CollisionCheckMeshes`) _array_index))
    (`/Engine/EditorBlueprintResources/StandardMacros.IsValid` _output
      (:`Is Valid`
        (bind _position (break `BasicParticleData` _array_element))
        (`SceneComponent.K2_SetWorldLocation` _output _position false false)
        (`SceneComponent.K2_SetWorldLocation` (`|GetArrayItem` (`self.GroundCollisionCheckMeshes`) _array_index) _position false false)))))

(fn `UserConstructionScript`
  (for _array_element (`|MakeArray` (`self.CollisionCheckMesh`) (`self.CollisionCheckMesh1`) null null null)
    (`KismetArrayLibrary.Array_Add` (`self.CollisionCheckMeshes`) _array_element))
  (for _array_element_2 (`|MakeArray` (`self.CollisionCheckMesh5`) (`self.CollisionCheckMesh6`) null null null)
    (`KismetArrayLibrary.Array_Add` (`self.GroundCollisionCheckMeshes`) _array_element_2)))