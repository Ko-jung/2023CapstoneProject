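; BP_MakeFloatingDamage is a short-lived actor that displays a random damage number as floating Niagara digits.
; On BeginPlay it rolls the number at a randomly offset location and splits it into characters.
; Each digit gets its own FX_FloatingDamage system, shifted along local Y by an accumulating spacing and textured through the user.Digit parameter from a digit texture array.
; The actor destroys itself once all digits are spawned.
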(event `self.ReceiveBeginPlay`
  (set `self.DamageLocationOffset` (* (`KismetMathLibrary.RandomUnitVector`) -50.0))
  (set `self.Damage` (`KismetMathLibrary.RandomIntegerInRange` 100 3000))
  (for _array_element (`KismetStringLibrary.GetCharacterArrayFromString` (`KismetStringLibrary.Conv_IntToString` (`self.Damage`)))
    (bind _returnvalue (`NiagaraFunctionLibrary.SpawnSystemAtLocation` "/Game/2019180031/MainGame/Fbx/Damage/FX_FloatingDamage.FX_FloatingDamage" (+ (`self.K2_GetActorLocation`) (`self.DamageLocationOffset`)) (`self.K2_GetActorRotation`) (0.75 0.75 0.75)))
    (bind _output_get (set `self.FX_FloatingDamage` _returnvalue))
    (`SceneComponent.K2_AddLocalOffset` _output_get (`KismetMathLibrary.MakeVector` 0.0 (`self.TextOffsetY`)) false false)
    (set `self.TextOffsetY` (+ (`self.TextOffsetY`) (* 25.0 0.75)))
    (`NiagaraFunctionLibrary.SetTextureObject` (`self.FX_FloatingDamage`) "user.Digit" (`|GetArrayItem` (`self.DigitTexture`) (`KismetStringLibrary.Conv_StringToInt` _array_element))))
  (`self.K2_DestroyActor`))

(fn `UserConstructionScript`)