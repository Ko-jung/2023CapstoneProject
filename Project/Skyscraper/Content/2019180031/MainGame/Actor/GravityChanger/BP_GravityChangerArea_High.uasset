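; Gravity changer area actor that alters jetpack hovering gravity for SkyscraperCharacters inside its cylinder volume.
; On overlap begin it records the character and adds -1 to the JetpackComponent's hovering gravity scale, then adds 1 back when a recorded character leaves.
; The construction script scales the cylinder by CylinderScale and passes that size and the GravityLow flag to the NSTEST effect, with the flag set again on BeginPlay.
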(event `self.ReceiveBeginPlay`
  (`NiagaraComponent.SetVariableBool` (`self.NS_TEST`) "GravityLow" (`self.GravityLow`)))

(event `self.Cylinder.OnComponentBeginOverlap`
  (params (OverlappedComponent :type "PrimitiveComponent Object Reference") (OtherActor :type "Actor Object Reference") (OtherComp :type "PrimitiveComponent Object Reference") (OtherBodyIndex :type Integer) (bFromSweep :type Boolean) (SweepResult :type "HitResult Structure (by ref)"))
  (bind _asskyscraper_character (cast `SkyscraperCharacter` OtherActor))
  (`KismetArrayLibrary.Array_AddUnique` (`self.AActorArray`) _asskyscraper_character)
  (`JetpackComponent.AddHoveringGravityScale` (`SkyscraperCharacter.JetpackComponent` _asskyscraper_character) -1.0))

(event `self.Cylinder.OnComponentEndOverlap`
  (params (OverlappedComponent :type "PrimitiveComponent Object Reference") (OtherActor :type "Actor Object Reference") (OtherComp :type "PrimitiveComponent Object Reference") (OtherBodyIndex :type Integer))
  (bind _aactorarray (`self.AActorArray`))
  (if (`KismetArrayLibrary.Array_Contains` _aactorarray OtherActor)
    (`KismetArrayLibrary.Array_RemoveItem` _aactorarray OtherActor)
    (bind _asskyscraper_character (cast `SkyscraperCharacter` OtherActor))
    (`JetpackComponent.AddHoveringGravityScale` (`SkyscraperCharacter.JetpackComponent` _asskyscraper_character) 1.0)))

(fn `UserConstructionScript`
  (bind _ns_test (`self.NS_TEST`))
  (`SceneComponent.SetRelativeScale3D` (`self.Cylinder`) (`self.CylinderScale`))
  (`NiagaraComponent.SetVariableVec3` _ns_test "InitialSize" (`self.CylinderScale`))
  (`NiagaraComponent.SetVariableBool` _ns_test "GravityLow" (`self.GravityLow`)))