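; Test actor for instanced static mesh rendering that fills a grid with randomly rotated instances.
; BeginPlay adds the instances to the InstancedStaticMesh component in local space, deriving grid positions from the loop index.
; An unused experiment remains: disconnected nodes create hidden StaticMeshComponents, and a self-repeating delayed event would copy their world transforms onto instances.
; Tick, overlap and the connected construction script do nothing.
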(event `self.ReceiveBeginPlay`
  (for _index (range 101)
    (`InstancedStaticMeshComponent.AddInstance` (`self.InstancedStaticMesh`) (`KismetMathLibrary.MakeTransform` (`KismetMathLibrary.MakeVector` (`KismetMathLibrary.Conv_IntToDouble` (* (/ _index 10) 200)) (`KismetMathLibrary.Conv_IntToDouble` (* (mod _index 10) 200))) (`KismetMathLibrary.RandomRotator` false)) false)))

(event `CustomEvent`
  (for (_array_element _array_index) (`self.NewVar_0`)
    (`InstancedStaticMeshComponent.UpdateInstanceTransform` (`self.InstancedStaticMesh`) _array_index (`SceneComponent.K2_GetComponentToWorld` _array_element) true true false))
  (`KismetSystemLibrary.Delay` 0.05)
  (`self.CustomEvent`))

(event `self.ReceiveTick`
  (params (DeltaSeconds :type "Float (single-precision)")))

(fn `UserConstructionScript`)