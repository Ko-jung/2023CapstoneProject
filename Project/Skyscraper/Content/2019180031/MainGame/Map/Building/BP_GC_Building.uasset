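; Temporary building actor that dissolves its props and structure on timers after spawning, within a fixed lifespan set on BeginPlay.
; The construction script sorts mesh components into an Objects group and a BuildingComponents group.
; Each group gets dynamic dissolve material instances, props after a set delay and the structure timed back from the lifespan's end.
; Self-recalling Delay events step DissolveValue up, then destroy that group's components when complete.
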(event `ChangeDissolveMaterial_Buildings`
  ;[1 1 1] Building Dissolve
  (for _array_element (`self.BuildingComponents`)
    (bind _returnvalue (`PrimitiveComponent.CreateDynamicMaterialInstance` _array_element 0 "/Game/2019180031/MainGame/Material/FurnitureDissolve/BuildingObject/M_Dissolve_Building.M_Dissolve_Building" "None"))
    (`KismetArrayLibrary.Array_Add` (`self.BuildingMaterials`) _returnvalue))
  (`self.SendBuildingDissolve`))

(event `SendBuildingDissolve`
  ;[1 1 1] Building Dissolve
  (set `self.Building_CurrentDissolveTime` (+ (`self.Building_CurrentDissolveTime`) (`self.DissolveTimeOffset`)))
  (for _array_element (`self.BuildingMaterials`)
    (`MaterialInstanceDynamic.SetScalarParameterValue` _array_element "DissolveValue" (/ (`self.Building_CurrentDissolveTime`) (`self.Building_ApplyDissolveTime`))))
  (if (>= (`self.Building_CurrentDissolveTime`) (`self.Building_ApplyDissolveTime`))
    (for _array_element_2 (`self.BuildingComponents`)
      (`ActorComponent.K2_DestroyComponent` _array_element_2))
    (else
      (`KismetSystemLibrary.Delay` (`self.DissolveTimeOffset`))
      (`self.SendBuildingDissolve`))))

(event `self.ReceiveBeginPlay`
  (`self.SetLifeSpan` 30.0)
  (`|ExecutionSequence`
    (:`then_0`
      (`KismetSystemLibrary.Delay` (`self.ObjectDissolveStartTime_Objects`))
      (`self.ChangeDissolveMaterial_Objects`))
    (:`then_1`
      (`KismetSystemLibrary.Delay` (- (- (`self.GetLifeSpan`) (`self.Building_ApplyDissolveTime`)) 5.0))
      (`self.ChangeDissolveMaterial_Buildings`))))

(event `ChangeDissolveMaterial_Objects`
  ;[1 1 1] Object Dissolve
  (for _array_element (`self.Objects`)
    (bind _returnvalue (`PrimitiveComponent.CreateDynamicMaterialInstance` _array_element 0 "/Game/2019180031/MainGame/Material/FurnitureDissolve/BuildingObject/M_Dissolve_BuildingEtc.M_Dissolve_BuildingEtc" "None"))
    (`KismetArrayLibrary.Array_Add` (`self.DissolveMaterials_Objects`) _returnvalue))
  (`self.SendMaterialParameter`))

(event `SendMaterialParameter`
  ;[1 1 1] Object Dissolve
  (set `self.CurrentDissolveTime_Objects` (+ (`self.CurrentDissolveTime_Objects`) (`self.DissolveTimeOffset`)))
  (for _array_element (`self.DissolveMaterials_Objects`)
    (`MaterialInstanceDynamic.SetScalarParameterValue` _array_element "DissolveValue" (/ (`self.CurrentDissolveTime_Objects`) (`self.ApplyDissolveTime`))))
  (if (>= (`self.CurrentDissolveTime_Objects`) (`self.ApplyDissolveTime`))
    (for _array_element_2 (`self.Objects`)
      (`ActorComponent.K2_DestroyComponent` _array_element_2))
    (else
      (`KismetSystemLibrary.Delay` (`self.DissolveTimeOffset`))
      (`self.SendMaterialParameter`))))

(fn `UserConstructionScript`
  (set `self.Objects` (`|MakeArray` (`self.StaticMesh2`) (`self.StaticMesh5`) (`self.StaticMesh1`) (`self.StaticMesh7`) (`self.StaticMesh6`) (`self.StaticMesh8`) (`self.StaticMesh9`) (`self.StaticMesh4`)))
  (set `self.BuildingComponents` (`|MakeArray` (`self.map_4_elevator_door_re_002`) (`self.GC_Map4_AssistFloor`) (`self.map_4_elevator_door_re_001`) (`self.GC_WindowWall`) (`self.GC_WindowWall1`) (`self.GC_WindowWall2`) (`self.GC_Wall`) (`self.GC_Stair_009`) (`self.GC_Stair_009_4`) (`self.GC_Stair_009_3`) (`self.stair_refine_stair013`) (`self.GC_Stair_003`) (`self.stair_refine_stair004`) (`self.GC_Stair_009_2`) (`self.GC_Stair_001`) (`self.stair_refine_stair002`) (`self.stair_refine_stair010`) (`self.stair_refine_stair011`) (`self.stair_refine_stair012`) (`self.stair_refine_stair007`) (`self.GC_Floor_`) :!type "MeshComponent Object Reference")))