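; Stand-in actor for the Assassin's death that plays a forward or backward death animation, then dissolves and destroys itself.
; BeginPlay creates dynamic materials for the body and boost meshes, passing in the capsule's bottom Z.
; After a delay it spawns a Niagara circle and sound, then enables Tick to lower the Erode parameter until destruction.
; The decrement sits inside the body-material loop, so dissolve speed scales with material count.
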(event `self.ReceiveBeginPlay`
  (bind (_returnvalue_x _returnvalue_y _returnvalue_z) (`KismetMathLibrary.BreakVector` (`self.K2_GetActorLocation`)))
  (bind (_returnvalue_x_2 _returnvalue_y_2 _returnvalue_z_2) (`KismetMathLibrary.BreakVector` (`self.K2_GetActorLocation`)))
  (bind _boostmesh (`self.BoostMesh`))
  (if (`self.bIsBwdDeath`)
    (`SkeletalMeshComponent.PlayAnimation` (`self.CharacterMesh`) (`self.BwdDeathAnim`) false)
    (else
      (`SkeletalMeshComponent.PlayAnimation` (`self.CharacterMesh`) (`self.FwdDeathAnim`) false)))
  (set `self.CapsuleComponent` (`self.Capsule`))
  (set `self.Mesh` (`self.CharacterMesh`))
  (`|ExecutionSequence`
    (:`then_0`
      (bind _returnvalue (`PrimitiveComponent.CreateDynamicMaterialInstance` _boostmesh 0 (`PrimitiveComponent.GetMaterial` _boostmesh 0) "None"))
      (bind _output_get (set `self.BoostMaterial` _returnvalue))
      (`MaterialInstanceDynamic.SetScalarParameterValue` _output_get "CharacterPositionZ" (- _returnvalue_z (`CapsuleComponent.CapsuleHalfHeight` (`self.CapsuleComponent`))))
      (for (_array_element _array_index) (`MeshComponent.GetMaterials` (`self.Mesh`))
        (bind _returnvalue_2 (`PrimitiveComponent.CreateDynamicMaterialInstance` (`self.Mesh`) _array_index _array_element "None"))
        (`KismetArrayLibrary.Array_Add` (`self.Materials`) _returnvalue_2)
        (`MaterialInstanceDynamic.SetScalarParameterValue` _returnvalue_2 "CharacterPositionZ" (- _returnvalue_z_2 (`CapsuleComponent.CapsuleHalfHeight` (`self.CapsuleComponent`))))))
    (:`then_1`
      (`KismetSystemLibrary.Delay` 3.0)
      (bind _returnvalue_3 (`NiagaraFunctionLibrary.SpawnSystemAtLocation` "/Game/2019180031/MainGame/Material/TestCharacterMaterial/TechnicalCircle/NS_TechnicalCircle.NS_TechnicalCircle" (- (`self.K2_GetActorLocation`) (`KismetMathLibrary.MakeVector` 0.0 0.0 (`CapsuleComponent.CapsuleHalfHeight` (`self.CapsuleComponent`))))))
      (set `self.NS_TechnicalCircle` _returnvalue_3)
      (`GameplayStatics.PlaySoundAtLocation` "/Game/2016180023/sound/character/사망.사망" (`self.K2_GetActorLocation`) (struct) 0.5 1.0 0.0 null null null null)
      (`KismetSystemLibrary.Delay` 0.6)
      (set `self.StartDissolveValue` 75.0)
      (set `self.StartTick` true))))

(event `self.ReceiveTick`
  (params (DeltaSeconds :type "Float (single-precision)"))
  (if (`self.StartTick`)
    (`MaterialInstanceDynamic.SetScalarParameterValue` (`self.BoostMaterial`) "Erode" (`self.StartDissolveValue`))
    (for _array_element (`self.Materials`)
      (`MaterialInstanceDynamic.SetScalarParameterValue` _array_element "Erode" (`self.StartDissolveValue`))
      (bind _output_get (set `self.StartDissolveValue` (- (`self.StartDissolveValue`) (* DeltaSeconds (`self.DissolveSpeed`)))))
      (if (<= _output_get -100.0)
        (set `self.StartTick` false)
        (`self.K2_DestroyActor`)))))

(fn `TestDissolve`)

(fn `UserConstructionScript`)