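; Child character Blueprint for a liquid wetness showcase that displays its hit-data render target on a plane.
; Shortly after BeginPlay, it destroys its main range component and gives the Plane a dynamic M_LiquidWetData material fed by LiquidWetComponent's RTHitData.
; SetActorAnimation plays either the move or idle sequence as a looping animation directly on the mesh.
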(event `self.ReceiveBeginPlay`
  (`parent.ReceiveBeginPlay`)
  (`KismetSystemLibrary.Delay` 0.2)
  (`self.BeginPlayFunc`))

(event `SetActorAnimation`
  (params (bMoveAnimSequence :type Boolean))
  (if bMoveAnimSequence
    (set `self.PlayingSequence` (`self.MoveSequence`))
    (else
      (set `self.PlayingSequence` (`self.IdelSequence`))))
  (`SkeletalMeshComponent.PlayAnimation` (`self.Mesh`) (`self.PlayingSequence`) true))

(event `self.ReceiveActorBeginOverlap`
  (params (OtherActor :type "Actor Object Reference"))
  (`parent.ReceiveActorBeginOverlap` OtherActor))

(fn `BeginPlayFunc`
  (`ActorComponent.K2_DestroyComponent` (`self.GetComponentByClass` "/Script/Skyscraper.MainRangeComponent"))
  (bind _returnvalue (`PrimitiveComponent.CreateDynamicMaterialInstance` (`self.Plane`) 0 "/Game/2019180031/ShowLiquidWet/M_LiquidWetData.M_LiquidWetData" "None"))
  (`MaterialInstanceDynamic.SetTextureParameterValue` _returnvalue "Texture" (`LiquidWetComponent.RT_HitData` (`self.LiquidWetComponent`))))

(fn `UserConstructionScript`
  (`parent.UserConstructionScript`))