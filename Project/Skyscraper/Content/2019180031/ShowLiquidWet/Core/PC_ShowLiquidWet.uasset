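; Player controller for the ShowLiquidWet demo that sets up its UI and input and toggles mouse cursor access.
; On BeginPlay it adds a WBP_LiquidWet widget to the viewport and registers the IMC_LiquidWet Enhanced Input mapping context.
; IA_Alt Started switches to Game and UI input with a visible cursor, while Canceled, rather than Completed, restores game-only input and hides it.
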(event `self.ReceiveBeginPlay`
  (bind _returnvalue (`|CreateWidget` "/Game/2019180031/ShowLiquidWet/WBP_LiquidWet.WBP_LiquidWet_C"))
  (`UserWidget.AddToViewport` _returnvalue 0)
  (`EnhancedInputSubsystemInterface.AddMappingContext` (subsystem `EnhancedInputLocalPlayerSubsystem`) "/Game/2019180031/ShowLiquidWet/Core/Input/IMC_LiquidWet.IMC_LiquidWet" 0 (struct)))

(event `EnhancedInput|/Game/2019180031/ShowLiquidWet/Core/Input/IA_Alt`
  (params (ActionValue :type Boolean) (ElapsedSeconds :type "Float (double-precision)") (TriggeredSeconds :type "Float (double-precision)") (InputAction :type "InputAction Object Reference" :default "/Game/2019180031/ShowLiquidWet/Core/Input/IA_Alt.IA_Alt"))
  (:`Started`
    (`WidgetBlueprintLibrary.SetInputMode_GameAndUIEx` self null)
    (set `self.bShowMouseCursor` true))
  (:`Canceled`
    (`WidgetBlueprintLibrary.SetInputMode_GameOnly` self)
    (set `self.bShowMouseCursor` false)))

(fn `UserConstructionScript`)