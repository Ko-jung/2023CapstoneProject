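; Test widget component that displays a damage number through WBP_DamageWidget.
; On BeginPlay it counts the digits in Damage with a base-10 logarithm of the absolute value, treating zero as one digit.
; It scales the draw width by that digit count, then passes the value and count to the widget's CreateDamageImage to build the display.
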(event `self.ReceiveBeginPlay`
  (bind _damage (`self.Damage`))
  (if (== _damage 0)
    (set `self.LengthOfDamage` 1)
    (else
      (set `self.LengthOfDamage` (`KismetMathLibrary.FTrunc` (+ (`KismetMathLibrary.Log` (`KismetMathLibrary.Conv_IntToDouble` (`KismetMathLibrary.Abs_Int` _damage)) 10.0) 1.0)))))
  (`self.SetDrawSize` (`KismetMathLibrary.MakeVector2D` (`KismetMathLibrary.Conv_IntToDouble` (* (`self.LengthOfDamage`) 100)) 50.0))
  (bind _aswbp_damage_widget (cast `/Game/2019180031/MainGame/Widget/Damage/WBP_DamageWidget` (`self.GetUserWidgetObject`)))
  (`DamageWidget.CreateDamageImage` _aswbp_damage_widget (`self.Damage`) (`self.LengthOfDamage`)))