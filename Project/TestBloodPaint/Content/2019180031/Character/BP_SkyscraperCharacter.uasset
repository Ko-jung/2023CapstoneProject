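; BP_SkyscraperCharacter is a character Blueprint whose skirt material can be painted with blood at given UV positions.
; On BeginPlay it creates a dynamic instance of the skirt material, assigns it to the character mesh's skirt slot, then initializes BPClothComponent's material settings.
; Getters expose the skirt mesh, slot index and material instance, while Paint forwards hit UV and blood duration to the cloth component.
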(event `self.ReceiveBeginPlay`
  (bind _returnvalue (`KismetMaterialLibrary.CreateDynamicMaterialInstance` (`self.SkirtMatRef`)))
  (set `self.SkirtMatInst` _returnvalue)
  (`PrimitiveComponent.SetMaterial` (`self.Mesh`) (`self.SkirtMaterialValue`) (`self.SkirtMatInst`))
  (`/Game/2019180031/Component/BP_ClothComponent.InitialMaterialSetting` (`self.BP_ClothComponent`)))

(fn `GetSkirtMaterial`
  (returns (SkirtMatInst :type "MaterialInstanceDynamic Object Reference"))
  (return (`self.SkirtMatInst`)))

(fn `GetSkirtMaterialValue`
  (returns (SkirtValue :type Integer))
  (return (`self.SkirtMaterialValue`)))

(fn `GetSkirtMesh`
  (returns (SkirtMesh :type "StaticMesh Object Reference"))
  (return (`self.SkirtMesh`)))

(fn `Paint`
  (params (`Hit UV` :type "Vector2D Structure (by ref)") (`Blood Duration` :type "Float (double-precision) (by ref)"))
  (`/Game/2019180031/Component/BP_ClothComponent.Paint` (`self.BP_ClothComponent`) `Hit UV` `Blood Duration`))

(fn `UserConstructionScript`)