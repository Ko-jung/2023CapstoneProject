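; Character component that shows fading blood hits on the skirt of BP_SkyscraperCharacter.
; BeginPlay attaches a hidden skirt static mesh to SkirtSocket on a custom collision channel.
; Paint stores hit UV and duration, which Tick counts down and removes on expiry.
; RenderBlood packs each hit into RGB slots of a one-pixel-high render target as data for the skirt material, mirrored to BP_TestPlane for testing.
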(event `self.ReceiveBeginPlay`
  (bind _skirtmesh (`self.SkirtMesh`))
  (`|ExecutionSequence`
    (:`then_0`
      (bind _asbp_skyscraper_character (cast `/Game/2019180031/Character/BP_SkyscraperCharacter` (`self.GetOwner`)))
      (bind _returnvalue (`|AddComponentByClass` :`self` _asbp_skyscraper_character :`Class` "/Script/Engine.StaticMeshComponent"))
      (bind _output_get (set `self.SkirtMesh` _returnvalue))
      (`SceneComponent.K2_AttachToComponent` _output_get (`Character.Mesh` _asbp_skyscraper_character) "SkirtSocket" "SnapToTarget" "SnapToTarget" "KeepRelative" true)
      (`StaticMeshComponent.SetStaticMesh` (`self.SkirtMesh`) (`/Game/2019180031/Character/BP_SkyscraperCharacter.GetSkirtMesh` _asbp_skyscraper_character))
      (`PrimitiveComponent.SetCollisionObjectType` _skirtmesh "ECC_GameTraceChannel1")
      (`SceneComponent.SetVisibility` _skirtmesh false false))))

(event `self.ReceiveTick`
  (params (DeltaSeconds :type "Float (single-precision)"))
  (bind _shitdata (`self.SHitData`))
  (for (_array_element _array_index) (`self.SHitData`)
    (bind (_hituv _hitdurationtime) (break `/Game/2019180031/Component/SBloodData` _array_element))
    (bind _returnvalue (`KismetMathLibrary.FMax` (- _hitdurationtime (* (`GameplayStatics.GetWorldDeltaSeconds`) 5.0))))
    (if (<= _returnvalue 0.0)
      (`KismetArrayLibrary.Array_Remove` _shitdata _array_index)
      (`KismetSystemLibrary.PrintString` (`KismetStringLibrary.Conv_IntToString` (`KismetArrayLibrary.Array_Length` _shitdata)))
      (else
        (`KismetArrayLibrary.Array_Set` (`self.SHitData`) _array_index (make `/Game/2019180031/Component/SBloodData` _hituv _returnvalue)))))
  (`self.RenderBlood`))

(fn `InitialMaterialSetting`
  (bind _rt_hitdata (`self.RT_HitData`))
  (bind _asbp_skyscraper_character (cast `/Game/2019180031/Character/BP_SkyscraperCharacter` (`self.GetOwner`)))
  (set `self.Skirt Mat Inst` (`/Game/2019180031/Character/BP_SkyscraperCharacter.GetSkirtMaterial` _asbp_skyscraper_character))
  ;[1 1 1] HitLocation 정보 담아 전송하는 RenderTarget 생성 및 UnWrap Material 파라미터로 적용
  (bind _returnvalue (`KismetRenderingLibrary.CreateRenderTarget2D` (* (`self.MaxHitCount`) (`self.HitDataOffset`)) 1))
  (set `self.RT_HitData` _returnvalue)
  (set `TextureRenderTarget2D.AddressX` "TA_Clamp" _rt_hitdata) ; 이거 해줘야 반대편 외각과 wrap이 안되어서 색상이 온전히 저장됨
  (set `TextureRenderTarget2D.AddressY` "TA_Clamp" _rt_hitdata)
  (`MaterialInstanceDynamic.SetTextureParameterValue` (`self.Skirt Mat Inst`) "Tex" (`self.RT_HitData`))
  (`MaterialInstanceDynamic.SetScalarParameterValue` (`self.Skirt Mat Inst`) "XSize" (`KismetMathLibrary.Conv_IntToDouble` (`self.MaxHitCount`))))

(fn `Paint`
  (params (`Hit UV` :type "Vector2D Structure (by ref)") (`Blood Duration` :type "Float (double-precision) (by ref)"))
  (`KismetArrayLibrary.Array_Add` (`self.SHitData`) (make `/Game/2019180031/Component/SBloodData` `Hit UV` `Blood Duration`))
  (`self.RenderBlood`))

(fn `RenderBlood`
  (bind _rt_hitdata (`self.RT_HitData`))
  (bind _hitdataoffset (`self.HitDataOffset`))
  (`KismetRenderingLibrary.ClearRenderTarget2D` _rt_hitdata)
  (bind (_canvas _size _context) (`KismetRenderingLibrary.BeginDrawCanvasToRenderTarget` _rt_hitdata))
  (for (_array_element _array_index) (`self.SHitData`)
    (bind (_hituv _hitdurationtime) (break `/Game/2019180031/Component/SBloodData` _array_element))
    (`Canvas.K2_DrawTexture` _canvas null (`KismetMathLibrary.MakeVector2D` (`KismetMathLibrary.Conv_IntToDouble` (- (* _array_index _hitdataoffset) (/ _hitdataoffset 2)))) (`KismetMathLibrary.MakeVector2D` (`KismetMathLibrary.Conv_IntToDouble` (`self.HitDataOffset`)) 1.0) (0.0 0.0) (1.0 1.0) (`KismetMathLibrary.MakeColor` (`KismetMathLibrary.BreakVector2D` _hituv) (`.Y` (`KismetMathLibrary.BreakVector2D` _hituv)) (/ _hitdurationtime 50.0)) "BLEND_Translucent" 0.0 (0.5 0.5)))
  (`KismetRenderingLibrary.EndDrawCanvasToRenderTarget` _context)
  (`MaterialInstanceDynamic.SetScalarParameterValue` (`self.Skirt Mat Inst`) "HitCounts" (`KismetMathLibrary.Conv_IntToDouble` (`KismetArrayLibrary.Array_Length` (`self.SHitData`))))
  (`MaterialInstanceDynamic.SetTextureParameterValue` (`self.Skirt Mat Inst`) "Tex" (`self.RT_HitData`))
  ;[1 1 1] Test
  (bind _returnvalue (`KismetMaterialLibrary.CreateDynamicMaterialInstance` "/Game/2019180031/Test/M_TestPlane.M_TestPlane"))
  (`MaterialInstanceDynamic.SetTextureParameterValue` _returnvalue "Tex" (`self.RT_HitData`))
  (bind _returnvalue_2 (`GameplayStatics.GetActorOfClass` "/Game/2019180031/Test/BP_TestPlane.BP_TestPlane_C"))
  (`PrimitiveComponent.SetMaterial` (`/Game/2019180031/Test/BP_TestPlane.Plane` _returnvalue_2) 0 _returnvalue))